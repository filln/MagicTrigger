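; Quest component for the Sevenfold Sphere puzzle, driving a player lift and a sliding rock wall.
; Stepping on the lift sinks it, then a timer compares box and platform tags: all lower platforms must match, but only one upper.
; Success carries the attached, input-locked player to the other level with a half-turn; failure resets that level's boxes.
; Separately, correctly tagged boxes on platforms 4 and 5 slide the wall aside.
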(event `self.ReceiveBeginPlay`
  ;[1 1 1] BeginPlay
  (if (and (`KismetSystemLibrary.IsValid` (`self.PlatformForBox5`)) (`KismetSystemLibrary.IsValid` (`self.PlatformForBox4`)))
    (add `/Game/MagicTrigger/Blueprints/Quests/QuestSevenfoldSphere/BP_PlatformForBox4.Platform4BeginOverlapBox` (`self.PlatformForBox4`) (delegate `Platform4BeginOverlapBox_Event_0`))
    (add `/Game/MagicTrigger/Blueprints/Quests/QuestSevenfoldSphere/BP_PlatformForBox5.Platform5BeginOverlapBox` (`self.PlatformForBox5`) (delegate `Platform5BeginOverlapBox_Event_0`))
    (else
      (`KismetSystemLibrary.PrintString` "platforms is not valid"))))

(event `Platform4BeginOverlapBox`
  ;[1 1 1] Проверка расстановки для сдвига скалы
  (bind _bchecksuccess (`self.CheckRightPlacingsBigWall` (`self.PlatformForBox4`) (`self.PlatformForBox5`)))
  (if _bchecksuccess
    (`self.MoveBigWall`)))

(event `MoveBigWall`
  (bind (_initiallocationdoor_x _initiallocationdoor_y _initiallocationdoor_z) (`KismetMathLibrary.BreakVector` (`/Game/MagicTrigger/Blueprints/Quests/QuestSevenfoldSphere/BP_RockDoor.InitialLocationDoor` (`self.BigWallRef`))))
  ;[0.2222 0.5991 0] Если правильный камень ляжет на платформу для сдвига скалы
  (`KismetSystemLibrary.PrintString` "OpenBigWall")
  (`KismetSystemLibrary.MoveComponentTo` (`/Game/MagicTrigger/Blueprints/Quests/QuestSevenfoldSphere/BP_RockDoor.DoorSphere` (`self.BigWallRef`)) (`KismetMathLibrary.MakeVector` _initiallocationdoor_x (+ _initiallocationdoor_y 70.0) _initiallocationdoor_z) (`SceneComponent.K2_GetComponentRotation` (`/Game/MagicTrigger/Blueprints/Quests/QuestSevenfoldSphere/BP_RockDoor.DoorSphere` (`self.BigWallRef`))) true true 5.0))

(event `Platform4BeginOverlapBox_Event_0`
  ;[1 1 1] BeginPlay
  (`self.Platform4BeginOverlapBox`))

(event `Platform5BeginOverlapBox_Event_0`
  ;[1 1 1] BeginPlay
  (`self.Platform5BeginOverlapBox`))

(event `Platform5BeginOverlapBox`
  ;[1 1 1] Проверка расстановки для сдвига скалы
  (bind _bchecksuccess (`self.CheckRightPlacingsBigWall` (`self.PlatformForBox5`) (`self.PlatformForBox4`)))
  (if _bchecksuccess
    (`self.MoveBigWall`)))

(event `LiftBeginOverlapCharacter`
  (params (CharacterCollision :type "PrimitiveComponent Object Reference"))
  ;[1 1 1] AfterBeginOverlap
  (if (and (== CharacterCollision (`Character.CapsuleComponent` (`GameplayStatics.GetPlayerCharacter` 0))) (not (`self.IsOffOverlapCharacter?`)))
    (`self.BeginOverlapMoveDown`)))

(event `LockIsClosed`
  ;[0.2222 0.5991 0] Если ключ неправильный, переместить все боксы на платформах к начальному положению
  (`KismetSystemLibrary.PrintString` "Closed")
  (if (`self.isLiftDown?`)
    (for _array_element (`self.PlatformsDown`)
      (bind _currentboxref (`/Game/MagicTrigger/Blueprints/Quests/QuestSevenfoldSphere/BP_PlatformForBox_Parent.CurrentBoxRef` _array_element))
      (`/Engine/EditorBlueprintResources/StandardMacros.IsValid` _currentboxref
        (:`Is Valid`
          (`/Game/MagicTrigger/Blueprints/Quests/QuestSevenfoldSphere/BP_BoxForPlatform_Parent.MoveBoxToInitLocation` _currentboxref))))
    (else
      (for _array_element_2 (`self.PlatformsUp`)
        (bind _currentboxref_2 (`/Game/MagicTrigger/Blueprints/Quests/QuestSevenfoldSphere/BP_PlatformForBox_Parent.CurrentBoxRef` _array_element_2))
        (`/Engine/EditorBlueprintResources/StandardMacros.IsValid` _currentboxref_2
          (:`Is Valid`
            (`/Game/MagicTrigger/Blueprints/Quests/QuestSevenfoldSphere/BP_BoxForPlatform_Parent.MoveBoxToInitLocation` _currentboxref_2)))))))

(event `BeginOverlapMoveDown`
  ;[1 1 1] AfterBeginOverlap
  (if (`self.isLiftDown?`)
    (set `self.CurrentLocation` (`self.InitLocation`))
    (else
      (set `self.CurrentLocation` (`self.UpLocation`))))
  (`KismetSystemLibrary.MoveComponentTo` (`Actor.RootComponent` (`self.GetOwner`)) (`KismetMathLibrary.MakeVector` (.x (`self.CurrentLocation`)) (.y (`self.CurrentLocation`)) (- (.z (`self.CurrentLocation`)) (* (.z (`.BoxExtent` (`KismetSystemLibrary.GetComponentBounds` (`self.LiftStaticMesh`)))) 2.0))) (`Actor.K2_GetActorRotation` (`self.GetOwner`)) true true 1.0)
  (`KismetSystemLibrary.K2_SetTimerDelegate` (delegate `CheckKey`) (`self.PauseBeforeCheckKey`)))

(event `CheckKey`
  ;[1 1 1] Проверить расстановку камней на платформах
  (if (`PrimitiveComponent.IsOverlappingComponent` (`self.OverlapBox`) (`Character.CapsuleComponent` (`GameplayStatics.GetPlayerCharacter` 0)))
    (if (`self.isLiftDown?`)
      (bind _islockopen (`self.CheckRightPlacingsDown`))
      (if _islockopen
        (`self.LockIsOpen`)
        (else
          (`self.LockIsClosed`)))
      (else
        (bind _islockopen_2 (`self.CheckRightPlacingsUp`))
        (if _islockopen_2
          (`self.LockIsOpen`)
          (else
            (`self.LockIsClosed`)))))))

(event `LockIsOpen`
  ;[1 1 1] Если ключ правильный
  (`KismetSystemLibrary.PrintString` "Open")
  (if (`self.isLiftDown?`)
    (`self.MoveUp`)
    (else
      (`self.MoveDown`))))

(event `LiftEndOverlapCharacter`
  (params (CharacterCollision :type "PrimitiveComponent Object Reference"))
  ;[1 1 1] AfterEndOverlap
  (if (and (== CharacterCollision (`Character.CapsuleComponent` (`GameplayStatics.GetPlayerCharacter` 0))) (not (`self.IsOffOverlapCharacter?`)))
    (`self.EndOverlapMoveUp`)))

(event `MoveUp`
  (bind (_returnvalue_roll _returnvalue_pitch _returnvalue_yaw) (`KismetMathLibrary.BreakRotator` (`Actor.K2_GetActorRotation` (`self.GetOwner`))))
  ;[1 1 1] Когда ключ найден, можно двигать лифт
  (`self.IsCharacterOnLift?` true)
  (`KismetSystemLibrary.MoveComponentTo` (`Actor.RootComponent` (`GameplayStatics.GetPlayerCharacter` 0)) (`SceneComponent.K2_GetComponentLocation` (`self.PointOfAttachCharacter`)) (`Actor.K2_GetActorRotation` (`GameplayStatics.GetPlayerCharacter` 0)) true true 0.2 true)
  (`Actor.K2_AttachToComponent` (`GameplayStatics.GetPlayerCharacter` 0) (`self.PointOfAttachCharacter`) "None" "SnapToTarget" "KeepWorld" "KeepWorld" true)
  (`KismetSystemLibrary.MoveComponentTo` (`Actor.RootComponent` (`self.GetOwner`)) (`self.UpLocation`) (`KismetMathLibrary.MakeRotator` _returnvalue_roll _returnvalue_pitch (+ _returnvalue_yaw 180.0)) true true 4.0)
  (set `self.IsLockOpen?` false)
  (set `self.isLiftDown?` false)
  (`self.IsCharacterOnLift?` false)
  (`self.BeginOverlapMoveDown`))

(event `MoveDown`
  (bind (_returnvalue_roll _returnvalue_pitch _returnvalue_yaw) (`KismetMathLibrary.BreakRotator` (`Actor.K2_GetActorRotation` (`self.GetOwner`))))
  ;[1 1 1] Когда ключ найден, можно двигать лифт
  (`self.IsCharacterOnLift?` true)
  (`KismetSystemLibrary.MoveComponentTo` (`Actor.RootComponent` (`GameplayStatics.GetPlayerCharacter` 0)) (`SceneComponent.K2_GetComponentLocation` (`self.PointOfAttachCharacter`)) (`Actor.K2_GetActorRotation` (`GameplayStatics.GetPlayerCharacter` 0)) true true)
  (`Actor.K2_AttachToComponent` (`GameplayStatics.GetPlayerCharacter` 0) (`self.PointOfAttachCharacter`) "None" "SnapToTarget" "KeepWorld" "KeepWorld" true)
  (`KismetSystemLibrary.MoveComponentTo` (`Actor.RootComponent` (`self.GetOwner`)) (`self.InitLocation`) (`KismetMathLibrary.MakeRotator` _returnvalue_roll _returnvalue_pitch (+ _returnvalue_yaw 180.0)) true true 4.0)
  (set `self.IsLockOpen?` false)
  (set `self.isLiftDown?` true)
  (`self.IsCharacterOnLift?` false)
  (`self.BeginOverlapMoveDown`))

(event `EndOverlapMoveUp`
  ;[1 1 1] AfterEndOverlap
  (if (`self.isLiftDown?`)
    (set `self.CurrentLocation` (`self.InitLocation`))
    (else
      (set `self.CurrentLocation` (`self.UpLocation`))))
  (`KismetSystemLibrary.MoveComponentTo` (`Actor.RootComponent` (`self.GetOwner`)) (`self.CurrentLocation`) (`Actor.K2_GetActorRotation` (`self.GetOwner`)) true true 1.0))

(fn `CheckRightPlacingsBigWall`
  (params (OverlappingPlatform :type "/Game/MagicTrigger/Blueprints/Quests/QuestSevenfoldSphere/BP_PlatformForBox_Parent Object Reference") (OtherPlatform :type "/Game/MagicTrigger/Blueprints/Quests/QuestSevenfoldSphere/BP_PlatformForBox_Parent Object Reference"))
  (returns (bCheckSuccess :type Boolean))
  (locals (OverlappingPlatform_ :type "/Game/MagicTrigger/Blueprints/Quests/QuestSevenfoldSphere/BP_PlatformForBox_Parent Object Reference") (OtherPlatform_ :type "/Game/MagicTrigger/Blueprints/Quests/QuestSevenfoldSphere/BP_PlatformForBox_Parent Object Reference"))
  (set `local.OverlappingPlatform_` OverlappingPlatform)
  (set `local.OtherPlatform_` OtherPlatform)
  (`/Engine/EditorBlueprintResources/StandardMacros.IsValid` (`/Game/MagicTrigger/Blueprints/Quests/QuestSevenfoldSphere/BP_PlatformForBox_Parent.CurrentBoxRef` (`local.OverlappingPlatform_`))
    (:`Is Valid`
      (if (`Actor.ActorHasTag` (`/Game/MagicTrigger/Blueprints/Quests/QuestSevenfoldSphere/BP_PlatformForBox_Parent.CurrentBoxRef` (`local.OverlappingPlatform_`)) (`self.OpenBigWallTag`))
        (`/Engine/EditorBlueprintResources/StandardMacros.IsValid` (`/Game/MagicTrigger/Blueprints/Quests/QuestSevenfoldSphere/BP_PlatformForBox_Parent.CurrentBoxRef` (`local.OtherPlatform_`))
          (:`Is Valid`
            (if (`Actor.ActorHasTag` (`/Game/MagicTrigger/Blueprints/Quests/QuestSevenfoldSphere/BP_PlatformForBox_Parent.CurrentBoxRef` (`local.OtherPlatform_`)) (`self.OpenBigWallTag`))
              (return true)
              (else
                (return false))))
          (:`Is Not Valid`
            (return false)))
        (else
          (return false))))
    (:`Is Not Valid`
      (return false))))

(fn `CheckRightPlacingsDown`
  (returns (IsLockOpen :type Boolean))
  (locals (SumOfRightPlacings :type Integer))
  (set `local.SumOfRightPlacings` 0)
  (for _array_element (`self.PlatformsDown`)
    (bind _currentboxref (`/Game/MagicTrigger/Blueprints/Quests/QuestSevenfoldSphere/BP_PlatformForBox_Parent.CurrentBoxRef` _array_element))
    (`/Engine/EditorBlueprintResources/StandardMacros.IsValid` _currentboxref
      (:`Is Valid`
        (if (== (`|GetArrayItem` (`Actor.Tags` _array_element)) (`|GetArrayItem` (`Actor.Tags` _currentboxref)))
          (`/Engine/EditorBlueprintResources/StandardMacros.IncrementInt` (`local.SumOfRightPlacings`))
          (else
            (break))))
      (:`Is Not Valid`
        (break))))
  (return (== (`KismetArrayLibrary.Array_Length` (`self.PlatformsDown`)) (`local.SumOfRightPlacings`))))

(fn `CheckRightPlacingsUp`
  (returns (IsLockOpen :type Boolean))
  (locals (PlatformsForBoxUpLoc :type "Array of /Game/MagicTrigger/Blueprints/Quests/QuestSevenfoldSphere/BP_PlatformForBox_Parent Object Reference") (CurrentPlatform :type "/Game/MagicTrigger/Blueprints/Quests/QuestSevenfoldSphere/BP_PlatformForBox_Parent Object Reference"))
  (for _array_element (`self.PlatformsUp`)
    (set `local.CurrentPlatform` _array_element)
    (`/Engine/EditorBlueprintResources/StandardMacros.IsValid` (`/Game/MagicTrigger/Blueprints/Quests/QuestSevenfoldSphere/BP_PlatformForBox_Parent.CurrentBoxRef` (`local.CurrentPlatform`))
      (:`Is Valid`
        (if (== (`|GetArrayItem` (`Actor.Tags` (`/Game/MagicTrigger/Blueprints/Quests/QuestSevenfoldSphere/BP_PlatformForBox_Parent.CurrentBoxRef` (`local.CurrentPlatform`)))) (`|GetArrayItem` (`Actor.Tags` (`local.CurrentPlatform`))))
          (return true)))))
  (return false))

(fn `IsCharacterOnLift?`
  (params (`_isOnLift?` :type Boolean))
  (if `_isOnLift?`
    (`Actor.DisableInput` (`GameplayStatics.GetPlayerCharacter` 0) (`GameplayStatics.GetPlayerController` 0))
    (message `/Game/Developers/OLDFiles/Interfaces/BPI_OwnerTargetSelection_OLD.OffWatchingActors_IF` (`GameplayStatics.GetPlayerCharacter` 0))
    (`CharacterMovementComponent.DisableMovement` (`Character.CharacterMovement` (`GameplayStatics.GetPlayerCharacter` 0)))
    (set `self.IsOffOverlapCharacter?` true)
    (`Actor.SetActorEnableCollision` (`GameplayStatics.GetPlayerCharacter` 0) false)
    (return)
    (else
      (`Actor.EnableInput` (`GameplayStatics.GetPlayerCharacter` 0) (`GameplayStatics.GetPlayerController` 0))
      (`CharacterMovementComponent.SetMovementMode` (`Character.CharacterMovement` (`GameplayStatics.GetPlayerCharacter` 0)) "MOVE_Walking" 0)
      ;[0.8213 0 0] Отсоединить от лифта (квест 1)
      (`Actor.K2_DetachFromActor` (`GameplayStatics.GetPlayerCharacter` 0) "KeepWorld" "KeepWorld" "KeepWorld")
      (`Actor.SetActorEnableCollision` (`GameplayStatics.GetPlayerCharacter` 0) true)
      (set `self.IsOffOverlapCharacter?` false)
      (return))))