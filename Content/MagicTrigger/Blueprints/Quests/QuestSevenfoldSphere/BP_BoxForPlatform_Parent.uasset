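; Parent Blueprint for the boxes in the Sevenfold Sphere quest's platform puzzle, able to return themselves when placed incorrectly.
; It records its starting location on BeginPlay.
; MoveBoxToInitLocation disables collision and physics, then chains three eased MoveComponentTo steps: lift, glide above the start point, descend.
; Collision and physics simulation are restored once the box is back in place.
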(event `self.ReceiveActorBeginOverlap`
  (params (OtherActor :type "Actor Object Reference"))
  (`parent.ReceiveActorBeginOverlap` OtherActor))

(event `self.ReceiveTick`
  (params (DeltaSeconds :type "Float (single-precision)"))
  (`parent.ReceiveTick` DeltaSeconds))

(event `self.ReceiveBeginPlay`
  ;[0.3092 0.5121 0] EventBeginPlay
  (`parent.ReceiveBeginPlay`)
  (set `self.InitLocation` (`self.K2_GetActorLocation`)))

(event `MoveBoxToInitLocation`
  (bind (_returnvalue_x _returnvalue_y _returnvalue_z) (`KismetMathLibrary.BreakVector` (`self.K2_GetActorLocation`)))
  (bind (_initlocation_x _initlocation_y _initlocation_z) (`KismetMathLibrary.BreakVector` (`self.InitLocation`)))
  ;[0.4155 0.4058 0] Переместить себя к начальному положению (когда неправильно расставлены)
  (`self.SetActorEnableCollision` false)
  (`PrimitiveComponent.SetSimulatePhysics` (`self.StaticMesh`) false)
  (`KismetSystemLibrary.MoveComponentTo` (`self.RootComponent`) (`KismetMathLibrary.MakeVector` _returnvalue_x _returnvalue_y (+ _returnvalue_z 100.0)) (`self.K2_GetActorRotation`) true true 2.0)
  (`KismetSystemLibrary.MoveComponentTo` (`self.RootComponent`) (`KismetMathLibrary.MakeVector` _initlocation_x _initlocation_y (+ _initlocation_z 100.0)) (`self.K2_GetActorRotation`) true true 3.0)
  (`KismetSystemLibrary.MoveComponentTo` (`self.RootComponent`) (`self.InitLocation`) (`self.K2_GetActorRotation`) true true 2.0)
  (`self.SetActorEnableCollision` true)
  (`PrimitiveComponent.SetSimulatePhysics` (`self.StaticMesh`) true))

(fn `UserConstructionScript`
  (`parent.UserConstructionScript`))