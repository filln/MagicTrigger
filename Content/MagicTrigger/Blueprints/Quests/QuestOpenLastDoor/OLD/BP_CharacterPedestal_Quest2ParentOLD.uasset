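; Legacy parent pedestal for the Open Last Door quest, with spinning glowing spheres and a floor disk that react to artifact copy placement.
; Enable, disable and activate events, also bound to debug keys, drive timelines that stop the spin, move the spheres up or back, and restart rotation.
; Activation dims the shared sphere and trim dynamic materials, returns the spheres, then restores the glow over the reset time to re-arm the pedestal.
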(event `self.ReceiveBeginPlay`
  ;[0.06764 0 0.7626] EventBeginPlay
  (bind _output_get (set `self.InitialMaxEmissive` (/ (/ 50.0 (`KismetMathLibrary.Conv_IntToDouble` (`self.CountOfSpheres`))) 4.0)))
  (`MaterialInstanceDynamic.SetScalarParameterValue` (`self.MaterialInstanceSpheres`) "EmissiveMultiplier" _output_get)
  (set `self.InitialRotationSphere` (`SceneComponent.RelativeRotation` (`self.CollisionSphere`)))
  (set `self.InitialRotationDisk` (`SceneComponent.RelativeRotation` (`self.Ruins_GreenBuffFloor`)))
  (set `self.DeltaRotationCollisionSphere` (`self.InitialDeltaRotationCollisionSphere`))
  (set `self.InitialLocationCollisionSphere` (`SceneComponent.RelativeLocation` (`self.CollisionSphere`))))

(event `self.ReceiveActorBeginOverlap`
  (params (OtherActor :type "Actor Object Reference"))
  (`parent.ReceiveActorBeginOverlap` OtherActor))

(event `EnablePedestal`
  (params (_LocationCopyOfArtifact :type "Vector Structure"))
  ;[0 0.4638 0.3575] Включение пьедестала (при появлении любой первой копии артефакта)
  (set `self.isEnable?` true :!label _label)
  (set `self.LocationCopyOfArtifact` _LocationCopyOfArtifact)
  (`KismetSystemLibrary.Delay` 0.5)
  (`self.MoveSpheresToArtifact`))

(event `Key|Four`
  (params (Key :type "Key Structure"))
  (:`Pressed`
    (goto _label)))

(event `RotationComponents`
  ;[0 0.5604 0.2609] Вращение компонентов
  (`SceneComponent.K2_AddLocalRotation` (`self.CollisionSphere`) (`KismetMathLibrary.MakeRotator` 0.0 0.0 (`self.DeltaRotationCollisionSphere`)) false false)
  (`SceneComponent.K2_AddLocalRotation` (`self.Ruins_GreenBuffFloor`) (`KismetMathLibrary.MakeRotator` 0.0 0.0 (`self.DeltaRotationBuffFloor`)) false false))

(event `self.ReceiveTick`
  (params (DeltaSeconds :type "Float (single-precision)"))
  ;[0 0.2899 0.5314] EventTick
  (`parent.ReceiveTick` DeltaSeconds)
  (`self.RotationComponents`))

(event `Key|Five`
  (params (Key :type "Key Structure"))
  (:`Pressed`
    ;[0 0.08696 0.7343] Выключение пьедестала (если установка не правильная)
    (`self.MoveSpheresToBegin` :!label _label_2)
    (`KismetSystemLibrary.Delay` 1.0)
    (set `self.isEnable?` false)))

(event `DisablePedestal`
  ;[0 0.08696 0.7343] Выключение пьедестала (если установка не правильная)
  (goto _label_2))

(event `ActivatePedestal`
  ;[0.6957 0.1256 0] Активация пьедестала (если установка правильная)
  (`self.AttenuationEmissive` :!label _label_3))

(event `Key|Six`
  (params (Key :type "Key Structure"))
  (:`Pressed`
    (goto _label_3)))

(event `MoveSpheresToArtifact`
  ;[0 0.09662 0.7247] Переместить сферы к Артефакту
  (`TimelineComponent.SetPlayRate` (`self.Timeline_StopRotation`) (/ 1.0 1.0))
  (set `self.DeltaRotationCollisionSphere_Tmp` (`self.InitialDeltaRotationCollisionSphere`))
  (bind (_direction _alpha) (`Timeline|Timeline_StopRotation`)
    (:`Update`
      (set `self.DeltaRotationCollisionSphere` (`KismetMathLibrary.Lerp` (`self.DeltaRotationCollisionSphere_Tmp`) 0.0 _alpha)))
    (:`Finished`
      (`KismetSystemLibrary.MoveComponentTo` (`self.CollisionSphere`) (`SceneComponent.RelativeLocation` (`self.HighPoint`)) (`SceneComponent.RelativeRotation` (`self.CollisionSphere`)) true true 1.0)
      (`TimelineComponent.SetPlayRate` (`self.Timeline_StartRotation`) (/ 1.0 1.0))
      (set `self.DeltaRotationCollisionSphere_Tmp` (* (`self.InitialDeltaRotationCollisionSphere`) 20.0))
      (bind (_direction_2 _alpha_2) (`Timeline|Timeline_StartRotation` :!via `PlayFromStart`)
        (:`Update`
          (set `self.DeltaRotationCollisionSphere` (`KismetMathLibrary.Lerp` 0.0 (`self.DeltaRotationCollisionSphere_Tmp`) _alpha_2)))))))

(event `RiseEmissive`
  ;[0 0.4445 0.3768] Осветление сфер и диска, установка готовности к включению
  (`TimelineComponent.SetPlayRate` (`self.Timeline_RiseEmissive`) (/ 1.0 (`self.TimeOfResetPedestals`)))
  (set `self.MaxEmissive_Tmp` (`self.InitialMaxEmissive`))
  (bind (_direction _alpha) (`Timeline|Timeline_RiseEmissive` :!via `PlayFromStart`)
    (:`Update`
      (`MaterialInstanceDynamic.SetScalarParameterValue` (`self.MaterialInstanceSpheres`) "EmissiveMultiplier" (`KismetMathLibrary.Lerp` 5.0 (`self.MaxEmissive_Tmp`) _alpha)))
    (:`Finished`
      (`MaterialInstanceDynamic.SetScalarParameterValue` (`self.MaterialInstanceJungleTrimMetalHole`) "EmissivePower" 5.0)
      (set `self.isEnable?` false))))

(event `AttenuationEmissive`
  ;[0 0.6087 0.2126] Затухание сфер и диска
  (`TimelineComponent.SetPlayRate` (`self.Timeline_AttenEmissive`) (/ 1.0 1.0))
  (set `self.MaxEmissive_Tmp` (`self.InitialMaxEmissive`))
  (bind (_direction _alpha) (`Timeline|Timeline_AttenEmissive` :!via `PlayFromStart`)
    (:`Update`
      (`MaterialInstanceDynamic.SetScalarParameterValue` (`self.MaterialInstanceSpheres`) "EmissiveMultiplier" (`KismetMathLibrary.Lerp` (`self.MaxEmissive_Tmp`) 5.0 _alpha)))
    (:`Finished`
      (`MaterialInstanceDynamic.SetScalarParameterValue` (`self.MaterialInstanceJungleTrimMetalHole`) "EmissivePower" 0.3)
      (`self.MoveSpheresToBegin`)
      (`KismetSystemLibrary.Delay` 1.0)
      (`self.RiseEmissive`))))

(event `MoveSpheresToBegin`
  ;[0.7537 0.06764 0] Переместить сферы к начальной точке
  (`TimelineComponent.SetPlayRate` (`self.Timeline_StopRotation1`) (/ 1.0 1.0))
  (set `self.DeltaRotationCollisionSphere_Tmp` (`self.DeltaRotationCollisionSphere`))
  (bind (_direction _alpha) (`Timeline|Timeline_StopRotation1`)
    (:`Update`
      (set `self.DeltaRotationCollisionSphere` (`KismetMathLibrary.Lerp` (`self.DeltaRotationCollisionSphere_Tmp`) 0.0 _alpha)))
    (:`Finished`
      (`KismetSystemLibrary.MoveComponentTo` (`self.CollisionSphere`) (`self.InitialLocationCollisionSphere`) (`SceneComponent.RelativeRotation` (`self.CollisionSphere`)) true true 1.0)
      (`TimelineComponent.SetPlayRate` (`self.Timeline_StartRotation1`) (/ 1.0 1.0))
      (set `self.DeltaRotationCollisionSphere_Tmp` (`self.InitialDeltaRotationCollisionSphere`))
      (bind (_direction_2 _alpha_2) (`Timeline|Timeline_StartRotation1` :!via `PlayFromStart`)
        (:`Update`
          (set `self.DeltaRotationCollisionSphere` (`KismetMathLibrary.Lerp` 0.0 (`self.DeltaRotationCollisionSphere_Tmp`) _alpha_2)))))))

(fn `UserConstructionScript`
  (bind _materialinstancespheres (`self.MaterialInstanceSpheres`))
  (`parent.UserConstructionScript`)
  (`|ExecutionSequence`
    (:`then_0`
      ;[0.4251 0.3962 0] Настроить материалы
      ;;[0.715 0.1063 0] Индикация заряда  сфер
      (bind _returnvalue (`PrimitiveComponent.CreateDynamicMaterialInstance` (`self.Sphere1`) 0 "/Game/MagicTrigger/Materials/AbilitySystem/M_AttackAbility.M_AttackAbility" "None"))
      (bind _output_get (set `self.MaterialInstanceSpheres` _returnvalue))
      (`MaterialInstanceDynamic.SetTextureParameterValue` _output_get "Texture" "/Game/MagicTrigger/Textures/T_FireBall_D.T_FireBall_D")
      (`MaterialInstanceDynamic.SetVectorParameterValue` _materialinstancespheres "EmissiveColor" (struct :`G` 0.385695 :`B` 0.91 :`A` 1.0))
      (`MaterialInstanceDynamic.SetScalarParameterValue` _materialinstancespheres "EmissiveMultiplier" (`self.InitialMaxEmissive`))
      (`MaterialInstanceDynamic.SetScalarParameterValue` (`self.MaterialInstanceSpheres`) "Metallic" 1.0)
      (for _array_element (`|MakeArray` (`self.Sphere2`) (`self.Sphere3`) (`self.Sphere4`) (`self.Sphere5`) (`self.Sphere6`) (`self.Sphere7`))
        (`PrimitiveComponent.SetMaterial` _array_element 0 (`self.MaterialInstanceSpheres`))))
    (:`then_1`
      ;;[0 0.1256 0.6957] Индикация готовности пьедестала
      (bind _returnvalue_2 (`PrimitiveComponent.CreateDynamicMaterialInstance` (`self.JungleTrim_Metal_Whole`) 0 null "None"))
      (bind _output_get_2 (set `self.MaterialInstanceJungleTrimMetalHole` _returnvalue_2))
      (`MaterialInstanceDynamic.SetScalarParameterValue` _output_get_2 "EmissivePower" 5.0))))