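; Quest manager for opening the last door, a placement puzzle across seven pedestals that it spawns at set points on BeginPlay.
; A looping timer polls until the player's SevenfoldSphere component is valid, binds to its finish event, then clears itself.
; On finish, it checks every pedestal for right placement.
; If all are right, it speeds up their rotating spheres; otherwise it resets all pedestals to their starting state.
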(event `self.ReceiveBeginPlay`
  (bind _returnvalue (`KismetSystemLibrary.K2_SetTimerDelegate` (delegate `CheckAndGetReferences`) 0.2 true))
  (set `self.BeginPlayTimer` _returnvalue)
  (`self.SpawnPedestals`))

(event `CheckAndGetReferences`
  (bind _returnvalue (`GameplayStatics.GetPlayerCharacter` 0))
  (`/Engine/EditorBlueprintResources/StandardMacros.IsValid` _returnvalue
    (:`Is Valid`
      (bind _asplayer_character_magic_trigger (cast `PlayerCharacterMagicTrigger` _returnvalue))
      (bind _returnvalue_2 (`PlayerCharacterMagicTrigger.GetSevenfoldSphereComponent` _asplayer_character_magic_trigger))
      (`/Engine/EditorBlueprintResources/StandardMacros.IsValid` _returnvalue_2
        (:`Is Valid`
          (bind _output_get (set `self.SevenfoldSphereComponent` _returnvalue_2))
          (add `SevenfoldSphereComponent.OnSevenfoldSphereFinish` _output_get (delegate `OnSevenfoldSphereFinish_Event_0`))
          (`KismetSystemLibrary.K2_ClearAndInvalidateTimerHandle` (`self.BeginPlayTimer`)))))))

(event `OnSevenfoldSphereFinish_Event_0`
  (`self.SSphereFinish`))

(fn `CheckOnRightPlacingsOnEveryPedestal`
  (returns (_bRightPlacings :type Boolean))
  (for _array_element (`self.PedestalsArray`)
    (if (not (`/Game/MagicTrigger/Blueprints/Quests/QuestOpenLastDoor/BP_OpenLastDoorPedestalParentTES.bRightPlacing` _array_element))
      (return false)))
  (return true))

(fn `Continue`
  (for _array_element (`self.PedestalsArray`)
    (`/Game/MagicTrigger/Blueprints/Quests/QuestOpenLastDoor/BP_OpenLastDoorPedestalParentTES.IncreaseRotationSpheresToMax3` _array_element)))

(fn `ReturnPedestalsToBeginAfterWrongSummaryPlacings`
  (for _array_element (`self.PedestalsArray`)
    (`/Game/MagicTrigger/Blueprints/Quests/QuestOpenLastDoor/BP_OpenLastDoorPedestalParentTES.ReturnToBeginAfterWrongSummaryPlacings` _array_element)))

(fn `SpawnPedestals`
  (bind _returnvalue (`|SpawnActorFromClass` "/Game/MagicTrigger/Blueprints/Quests/QuestOpenLastDoor/BP_OpenLastDoorPedestal1TES.BP_OpenLastDoorPedestal1TES_C" (`KismetMathLibrary.MakeTransform` (`self.PointOfPedestal1`) (struct) (`self.SpawnScale`)) "AlwaysSpawn" "OverrideRootScale" null null))
  (`KismetArrayLibrary.Array_Add` (`self.PedestalsArray`) _returnvalue)
  (bind _returnvalue_2 (`|SpawnActorFromClass` "/Game/MagicTrigger/Blueprints/Quests/QuestOpenLastDoor/BP_OpenLastDoorPedestal2TES.BP_OpenLastDoorPedestal2TES_C" (`KismetMathLibrary.MakeTransform` (`self.PointOfPedestal2`) (struct) (`self.SpawnScale`)) "AlwaysSpawn" "OverrideRootScale" null null))
  (`KismetArrayLibrary.Array_Add` (`self.PedestalsArray`) _returnvalue_2)
  (bind _returnvalue_3 (`|SpawnActorFromClass` "/Game/MagicTrigger/Blueprints/Quests/QuestOpenLastDoor/BP_OpenLastDoorPedestal3TES.BP_OpenLastDoorPedestal3TES_C" (`KismetMathLibrary.MakeTransform` (`self.PointOfPedestal3`) (struct) (`self.SpawnScale`)) "AlwaysSpawn" "OverrideRootScale" null null))
  (`KismetArrayLibrary.Array_Add` (`self.PedestalsArray`) _returnvalue_3)
  (bind _returnvalue_4 (`|SpawnActorFromClass` "/Game/MagicTrigger/Blueprints/Quests/QuestOpenLastDoor/BP_OpenLastDoorPedestal4TES.BP_OpenLastDoorPedestal4TES_C" (`KismetMathLibrary.MakeTransform` (`self.PointOfPedestal4`) (struct) (`self.SpawnScale`)) "AlwaysSpawn" "OverrideRootScale" null null))
  (`KismetArrayLibrary.Array_Add` (`self.PedestalsArray`) _returnvalue_4)
  (bind _returnvalue_5 (`|SpawnActorFromClass` "/Game/MagicTrigger/Blueprints/Quests/QuestOpenLastDoor/BP_OpenLastDoorPedestal5TES.BP_OpenLastDoorPedestal5TES_C" (`KismetMathLibrary.MakeTransform` (`self.PointOfPedestal5`) (struct) (`self.SpawnScale`)) "AlwaysSpawn" "OverrideRootScale" null null))
  (`KismetArrayLibrary.Array_Add` (`self.PedestalsArray`) _returnvalue_5)
  (bind _returnvalue_6 (`|SpawnActorFromClass` "/Game/MagicTrigger/Blueprints/Quests/QuestOpenLastDoor/BP_OpenLastDoorPedestal6TES.BP_OpenLastDoorPedestal6TES_C" (`KismetMathLibrary.MakeTransform` (`self.PointOfPedestal6`) (struct) (`self.SpawnScale`)) "AlwaysSpawn" "OverrideRootScale" null null))
  (`KismetArrayLibrary.Array_Add` (`self.PedestalsArray`) _returnvalue_6)
  (bind _returnvalue_7 (`|SpawnActorFromClass` "/Game/MagicTrigger/Blueprints/Quests/QuestOpenLastDoor/BP_OpenLastDoorPedestal7TES.BP_OpenLastDoorPedestal7TES_C" (`KismetMathLibrary.MakeTransform` (`self.PointOfPedestal7`) (struct) (`self.SpawnScale`)) "AlwaysSpawn" "OverrideRootScale" null null))
  (`KismetArrayLibrary.Array_Add` (`self.PedestalsArray`) _returnvalue_7))

(fn `SSphereFinish`
  (bind __brightplacings (`self.CheckOnRightPlacingsOnEveryPedestal`))
  (if __brightplacings
    (`self.Continue`)
    (else
      (`self.ReturnPedestalsToBeginAfterWrongSummaryPlacings`))))

(fn `UserConstructionScript`)