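; Parent pedestal for the open-last-door quest, with spinning glowing spheres that react to an overlapping SevenfoldSphere.
; Activation slows, dims and raises them, then compares the sphere's Number to CountOfSpheres, spinning up on a match or lowering and relighting otherwise.
; Separate events, not called here, handle a wrong overall placement by resetting and re-arming, or play a faster-spin, bobbing finale.
; Looping timers step rotation and emissive; MoveComponentTo handles vertical motion.
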(event `self.ReceiveBeginPlay`
  (set `self.CurrentDeltaRotationSpheres` (`self.Max1DeltaRotationSpheres`))
  (bind _returnvalue (`KismetSystemLibrary.K2_SetTimer` null "RotationComponents" (`self.TimersDeltaTime`) true))
  (set `self.RotationComponentsTimer` _returnvalue))

(event `MoveSpheresToHighPointInternal`
  (params (OverTime :type "Float (double-precision)"))
  (bind _spherescentralpoint (`self.SpheresCentralPoint`))
  (`KismetSystemLibrary.MoveComponentTo` _spherescentralpoint (`SceneComponent.RelativeLocation` (`self.HighPoint`)) (`SceneComponent.RelativeRotation` _spherescentralpoint) true true OverTime))

(event `self.SphereCollision.OnComponentBeginOverlap`
  (params (OverlappedComponent :type "PrimitiveComponent Object Reference") (OtherActor :type "Actor Object Reference") (OtherComp :type "PrimitiveComponent Object Reference") (OtherBodyIndex :type Integer) (bFromSweep :type Boolean) (SweepResult :type "HitResult Structure (by ref)"))
  (if (`self.bCanWork`)
    (bind _assevenfold_sphere (cast `SevenfoldSphere` OtherActor))
    (set `self.SevenfoldSphere` _assevenfold_sphere)
    (`self.Activate`)
    (set `self.bCanWork` false)))

(event `Activate`
  (set `self.RotationSpheresDeltaValue` (/ (`self.Max1DeltaRotationSpheres`) (/ (`self.RotationAndEmissiveSpheresTime`) (`self.TimersDeltaTime`))))
  (set `self.EmissiveSpheresDeltaValue` (/ (`self.MaxEmissive`) (/ (`self.RotationAndEmissiveSpheresTime`) (`self.TimersDeltaTime`))))
  (bind _returnvalue (`KismetSystemLibrary.K2_SetTimer` null "DecreaseRotationAndEmissiveSpheres" (`self.TimersDeltaTime`) true))
  (set `self.MainTimer` _returnvalue))

(event `MoveSpheresToLowerPointInternal`
  (params (OverTime :type "Float (double-precision)"))
  (bind _spherescentralpoint (`self.SpheresCentralPoint`))
  (`KismetSystemLibrary.MoveComponentTo` _spherescentralpoint (`SceneComponent.RelativeLocation` (`self.LowerPoint`)) (`SceneComponent.RelativeRotation` _spherescentralpoint) true true OverTime))

(event `MoveSpheresToHighPoint`
  (`|ExecutionSequence`
    (:`then_0`
      (`self.MoveSpheresToHighPointInternal` (`self.MoveSpheresTime`)))
    (:`then_1`
      (`KismetSystemLibrary.K2_SetTimerDelegate` (delegate `next`) 2.0))))

(event `next`
  (bind _brightplacings (`self.CheckOnRightPlacingInThisPedestal`))
  (bind _output_get (set `self.bRightPlacing` _brightplacings))
  (if _output_get
    (`self.Continue`)
    (else
      (`self.ReturnToBeginAfterWrongPlacing`))))

(event `ReturnToBeginAfterWrongPlacing`
  (`|ExecutionSequence`
    (:`then_0`
      (`self.MoveSpheresToLowerPointInternal` (`self.MoveSpheresTime`)))
    (:`then_1`
      (`KismetSystemLibrary.K2_SetTimerDelegate` (delegate `next1`) (`self.MoveSpheresTime`)))))

(event `next1`
  (bind _returnvalue (`KismetSystemLibrary.K2_SetTimer` null "IncreaseRotationAndEmissiveSpheres" (`self.TimersDeltaTime`) true))
  (set `self.MainTimer` _returnvalue))

(event `ReturnToBeginAfterWrongSummaryPlacings`
  (set `self.RotationSpheresDeltaValue` (/ (`self.Max2DeltaRotationSpheres`) (/ (`self.RotationSpheresTime`) (`self.TimersDeltaTime`))))
  (bind _returnvalue (`KismetSystemLibrary.K2_SetTimer` null "DecreaseRotationFromMax2ToZero" (`self.TimersDeltaTime`) true))
  (set `self.MainTimer` _returnvalue)
  (`KismetSystemLibrary.K2_SetTimerDelegate` (delegate `SetCanWorkToTrue`) (+ (`self.RotationSpheresTime`) (`self.RotationAndEmissiveSpheresTime`) (`self.MoveSpheresTime`))))

(event `SetCanWorkToTrue`
  (set `self.bCanWork` true))

(event `IncreaseRotationSpheresToMax3`
  (set `self.RotationSpheresDeltaValue` (/ (- (`self.Max3DeltaRotationSpheres`) (`self.Max2DeltaRotationSpheres`)) (/ (`self.RotationSpheresTime`) (`self.TimersDeltaTime`))))
  (bind _returnvalue (`KismetSystemLibrary.K2_SetTimer` null "IncreaseRotationSpheresToMax3_Internal" (`self.TimersDeltaTime`) true))
  (set `self.MainTimer` _returnvalue))

(event `BeginInflateSphere1`
  (`|ExecutionSequence`
    (:`then_0`
      (`self.MoveSpheresToLowerPointInternal` (`self.MoveSpheresHalfTime`)))
    (:`then_1`
      (`KismetSystemLibrary.K2_SetTimerDelegate` (delegate `EndInflateSphere1`) 0.5))))

(event `EndInflateSphere1`
  (`|ExecutionSequence`
    (:`then_0`
      (`self.MoveSpheresToHighPointInternal` (`self.MoveSpheresHalfTime`)))
    (:`then_1`
      (`KismetSystemLibrary.K2_SetTimerDelegate` (delegate `BeginInflateSphere2`) (`self.MoveSpheresTime`)))))

(event `BeginInflateSphere2`
  (bind _movesphereshalftime (`self.MoveSpheresHalfTime`))
  (`|ExecutionSequence`
    (:`then_0`
      (`self.MoveSpheresToLowerPointInternal` _movesphereshalftime))
    (:`then_1`
      (`KismetSystemLibrary.K2_SetTimerDelegate` (delegate `EndInflateSphere2`) _movesphereshalftime))))

(event `EndInflateSphere2`
  (`|ExecutionSequence`
    (:`then_0`
      (`self.MoveSpheresToHighPointInternal` 0.0))
    (:`then_1`
      (`KismetSystemLibrary.K2_SetTimerDelegate` (delegate `BeginInflateSphere3`) (`self.MoveSpheresTime`)))))

(event `BeginInflateSphere3`
  (bind _movesphereshalftime (`self.MoveSpheresHalfTime`))
  (`|ExecutionSequence`
    (:`then_0`
      (`self.MoveSpheresToLowerPointInternal` _movesphereshalftime))
    (:`then_1`
      (`KismetSystemLibrary.K2_SetTimerDelegate` (delegate `EndInflateSphere3`) _movesphereshalftime))))

(event `EndInflateSphere3`
  (bind _movespherestime (`self.MoveSpheresTime`))
  (`|ExecutionSequence`
    (:`then_0`
      (`self.MoveSpheresToHighPointInternal` _movespherestime))
    (:`then_1`
      (`KismetSystemLibrary.K2_SetTimerDelegate` (delegate `LastMoveSpheresToLowerPoint`) _movespherestime))))

(event `LastMoveSpheresToLowerPoint`
  (`self.MoveSpheresToLowerPointInternal` (`self.MoveSpheresTime`)))

(fn `CheckOnRightPlacingInThisPedestal`
  (returns (bRightPlacings :type Boolean))
  (bind _sevenfoldsphere (`self.SevenfoldSphere`))
  (`/Engine/EditorBlueprintResources/StandardMacros.IsValid` _sevenfoldsphere
    (:`Is Valid`
      (if (== (`self.CountOfSpheres`) (`SevenfoldSphere.Number` _sevenfoldsphere))
        (return true)
        (else
          _)))
    (:`Is Not Valid`
      _))
  (return false))

(fn `Continue`
  (set `self.RotationSpheresDeltaValue` (/ (`self.Max2DeltaRotationSpheres`) (/ (`self.RotationSpheresTime`) (`self.TimersDeltaTime`))))
  (bind _returnvalue (`KismetSystemLibrary.K2_SetTimer` null "IncreaseRotationSpheresToMax2" (`self.TimersDeltaTime`) true))
  (set `self.MainTimer` _returnvalue))

(fn `DecreaseRotationAndEmissiveSpheres`
  (set `self.CurrentDeltaRotationSpheres` (- (`self.CurrentDeltaRotationSpheres`) (`self.RotationSpheresDeltaValue`)))
  (if (> (`self.CurrentEmissive`) (`self.MinEmissive`))
    (bind _output_get (set `self.CurrentEmissive` (- (`self.CurrentEmissive`) (`self.EmissiveSpheresDeltaValue`))))
    (`MaterialInstanceDynamic.SetScalarParameterValue` (`self.SpheresMaterial`) (`self.EmissiveMultiplierName`) _output_get))
  (if (<= (`self.CurrentDeltaRotationSpheres`) 0.0)
    (set `self.CurrentDeltaRotationSpheres` 0.0)
    (set `self.CurrentEmissive` (`self.MinEmissive`))
    (`KismetSystemLibrary.K2_ClearAndInvalidateTimerHandle` (`self.MainTimer`))
    (`self.MoveSpheresToHighPoint`)
    (else
      (return))))

(fn `DecreaseRotationFromMax2ToZero`
  (set `self.CurrentDeltaRotationSpheres` (- (`self.CurrentDeltaRotationSpheres`) (`self.RotationSpheresDeltaValue`)))
  (if (<= (`self.CurrentDeltaRotationSpheres`) 0.0)
    (set `self.CurrentDeltaRotationSpheres` 0.0)
    (`KismetSystemLibrary.K2_ClearAndInvalidateTimerHandle` (`self.MainTimer`))
    (`self.ReturnToBeginAfterWrongPlacing`)
    (else
      (return))))

(fn `IncreaseRotationAndEmissiveSpheres`
  (set `self.CurrentDeltaRotationSpheres` (+ (`self.CurrentDeltaRotationSpheres`) (`self.RotationSpheresDeltaValue`)))
  (if (< (`self.CurrentEmissive`) (`self.MaxEmissive`))
    (bind _output_get (set `self.CurrentEmissive` (+ (`self.CurrentEmissive`) (`self.EmissiveSpheresDeltaValue`))))
    (`MaterialInstanceDynamic.SetScalarParameterValue` (`self.SpheresMaterial`) (`self.EmissiveMultiplierName`) _output_get))
  (if (>= (`self.CurrentDeltaRotationSpheres`) (`self.Max1DeltaRotationSpheres`))
    (set `self.CurrentDeltaRotationSpheres` (`self.Max1DeltaRotationSpheres`))
    (set `self.CurrentEmissive` (`self.MaxEmissive`))
    (`KismetSystemLibrary.K2_ClearAndInvalidateTimerHandle` (`self.MainTimer`))
    (else
      (return))))

(fn `IncreaseRotationSpheresToMax2`
  (set `self.CurrentDeltaRotationSpheres` (+ (`self.CurrentDeltaRotationSpheres`) (`self.RotationSpheresDeltaValue`)))
  (if (>= (`self.CurrentDeltaRotationSpheres`) (`self.Max2DeltaRotationSpheres`))
    (set `self.CurrentDeltaRotationSpheres` (`self.Max2DeltaRotationSpheres`))
    (`KismetSystemLibrary.K2_ClearAndInvalidateTimerHandle` (`self.MainTimer`))
    (else
      (return))))

(fn `IncreaseRotationSpheresToMax3_Internal`
  (set `self.CurrentDeltaRotationSpheres` (+ (`self.CurrentDeltaRotationSpheres`) (`self.RotationSpheresDeltaValue`)))
  (if (>= (`self.CurrentDeltaRotationSpheres`) (`self.Max3DeltaRotationSpheres`))
    (set `self.CurrentDeltaRotationSpheres` (`self.Max3DeltaRotationSpheres`))
    (`KismetSystemLibrary.K2_ClearAndInvalidateTimerHandle` (`self.MainTimer`))
    (`self.BeginInflateSphere1`)
    (else
      (return))))

(fn `RotationComponents`
  (`SceneComponent.K2_AddLocalRotation` (`self.SpheresCentralPoint`) (`KismetMathLibrary.MakeRotator` 0.0 0.0 (`self.CurrentDeltaRotationSpheres`)) false false)
  (`SceneComponent.K2_AddLocalRotation` (`self.Ruins_GreenBuffFloor`) (`KismetMathLibrary.MakeRotator` 0.0 0.0 (`self.DeltaRotationBuffFloor`)) false false))

(fn `UserConstructionScript`
  (bind _output_get (set `self.CurrentEmissive` (/ (`self.TotalEmissive`) (`KismetMathLibrary.Conv_IntToDouble` (`self.CountOfSpheres`)))))
  (set `self.MaxEmissive` _output_get))