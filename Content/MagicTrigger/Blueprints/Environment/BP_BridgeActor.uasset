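; BP_BridgeActor is a procedurally built physics bridge of chained segments between Start and End components.
; The construction script spawns Count evenly spaced static mesh segments along local X and places End one spacing past the last.
; On BeginPlay, a helper creates and attaches physics constraints at runtime, linking Start, each neighboring segment and End in sequence.
; All constraints lock swing and twist rotation.
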(event `self.ReceiveBeginPlay`
  (bind _bridgearr (`self.BridgeArr`))
  (bind _bridgearr_2 (`self.BridgeArr`))
  (bind _end (`self.End`))
  (bind _start (`self.Start`))
  (`self.SetPhysicsConstrained` _start _start (`|GetArrayItem` (`self.BridgeArr`)) "ACM_Locked" "ACM_Locked" "ACM_Locked")
  (for (_ _array_index) (`self.BridgeArr`)
    (if (< _array_index (`KismetArrayLibrary.Array_LastIndex` (`self.BridgeArr`)))
      (bind _output (`|GetArrayItem` _bridgearr _array_index))
      (`self.SetPhysicsConstrained` _output _output (`|GetArrayItem` _bridgearr (+ _array_index 1)) "ACM_Locked" "ACM_Locked" "ACM_Locked")))
  (`self.SetPhysicsConstrained` _end (`|GetArrayItem` _bridgearr_2 (`KismetArrayLibrary.Array_LastIndex` _bridgearr_2)) _end "ACM_Locked" "ACM_Locked" "ACM_Locked"))

(fn `SetPhysicsConstrained`
  (params (ParentOfAttachToComponent :type "SceneComponent Object Reference") (Component1 :type "PrimitiveComponent Object Reference") (Component2 :type "PrimitiveComponent Object Reference") (MotionTypeSwing1 :type "EAngularConstraintMotion Enum" :default "ACM_Free") (MotionTypeSwing2 :type "EAngularConstraintMotion Enum" :default "ACM_Free") (ConstraintTypeTwist :type "EAngularConstraintMotion Enum" :default "ACM_Free"))
  (locals (_Component1 :type "PrimitiveComponent Object Reference") (_Component2 :type "PrimitiveComponent Object Reference") (PhysicsConstrainedComponentRef :type "PhysicsConstraintComponent Object Reference") (_MotionTypeSwing1 :type "EAngularConstraintMotion Enum" :default "ACM_Free") (_ParentOfAttachToComponent :type "SceneComponent Object Reference") (_MotionTypeSwing2 :type "EAngularConstraintMotion Enum" :default "ACM_Free") (_ConstraintTypeTwist :type "EAngularConstraintMotion Enum" :default "ACM_Free"))
  (set `local._ParentOfAttachToComponent` ParentOfAttachToComponent)
  (set `local._Component1` Component1)
  (set `local._Component2` Component2)
  (set `local._MotionTypeSwing1` MotionTypeSwing1)
  (set `local._MotionTypeSwing2` MotionTypeSwing2)
  (set `local._ConstraintTypeTwist` ConstraintTypeTwist)
  (bind _returnvalue (`AddComponent|NODE_AddPhysicsConstraintComponent-2`))
  (set `local.PhysicsConstrainedComponentRef` _returnvalue)
  (`PhysicsConstraintComponent.SetAngularSwing1Limit` (`local.PhysicsConstrainedComponentRef`) (`local._MotionTypeSwing1`) 1.0)
  (`PhysicsConstraintComponent.SetAngularSwing2Limit` (`local.PhysicsConstrainedComponentRef`) (`local._MotionTypeSwing2`) 1.0)
  (`PhysicsConstraintComponent.SetAngularTwistLimit` (`local.PhysicsConstrainedComponentRef`) (`local._ConstraintTypeTwist`) 0.0)
  (`SceneComponent.K2_AttachToComponent` (`local.PhysicsConstrainedComponentRef`) (`local._ParentOfAttachToComponent`) "None" "KeepRelative" "KeepRelative" "KeepRelative" true)
  (`PhysicsConstraintComponent.SetConstrainedComponents` (`local.PhysicsConstrainedComponentRef`) (`local._Component1`) "None" (`local._Component2`) "None")
  (return))

(fn `UserConstructionScript`
  (for _index (range 1 (+ (`self.Count`) 1))
    (bind _returnvalue (`AddComponent|NODE_AddStaticMeshComponent-0` :`RelativeTransform` (`KismetMathLibrary.MakeTransform` (`KismetMathLibrary.MakeVector` (* _index (`self.Distance`))))))
    (`KismetArrayLibrary.Array_Add` (`self.BridgeArr`) _returnvalue))
  (`SceneComponent.K2_SetRelativeLocation` (`self.End`) (`KismetMathLibrary.MakeVector` (* (+ (`KismetArrayLibrary.Array_Length` (`self.BridgeArr`)) 1) (`self.Distance`))) false false))