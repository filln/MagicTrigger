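; Procedurally assembled castle environment actor with walls, pillars, a floor, and a treasury filled with gold.
; Its construction script populates instanced static mesh components using nested grid loops for the architecture and gold piles.
; Other instances, including skeletons, are placed at fixed intervals along three splines.
; The event graph is empty, and the reference-check function only tests the game mode, with its true return left unconnected.
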(event `self.ReceiveBeginPlay`
  ;[1 1 1] BeginPlay
)

(fn `CheckReferences_IF`
  (returns (bValid :type Boolean))
  (`/Engine/EditorBlueprintResources/StandardMacros.IsValid` (`GameplayStatics.GetGameMode`)
    (:`Is Not Valid`
      (return false))))

(fn `UserConstructionScript`
  (`|ExecutionSequence`
    (:`then_0`
      ;[0 0.4155 0.4058] Стены
      (for _array_element (`|MakeArray` (`self.InstancedStaticMesh`) (`self.InstancedStaticMesh1`) (`self.InstancedStaticMesh2`) (`self.InstancedStaticMesh3`) (`self.InstancedStaticMesh4`) (`self.InstancedStaticMesh5`) (`self.InstancedStaticMesh6`) (`self.InstancedStaticMesh7`))
        (for _index (range 8)
          (for _index_2 (range 7)
            (`InstancedStaticMeshComponent.AddInstance` _array_element (`KismetMathLibrary.MakeTransform` (`KismetMathLibrary.MakeVector` 47.876221 (* _index_2 -375.533661) (* _index -330.0)) (`KismetMathLibrary.MakeRotator` -90.0 0.0 180.0)))))))
    (:`then_1`
      (for _index_3 (range 4)
        (`InstancedStaticMeshComponent.AddInstance` (`self.InstancedStaticMesh9`) (`KismetMathLibrary.MakeTransform` (`KismetMathLibrary.MakeVector` 0.0 (* _index_3 1500.0)) (`KismetMathLibrary.MakeRotator` 0.0 0.0 -90.0) (3.0 3.0 3.0)))))
    (:`then_2`
      (for _index_4 (range 31)
        (bind _returnvalue_location (`KismetMathLibrary.BreakTransform` (`SplineComponent.GetTransformAtDistanceAlongSpline` (`self.Spline`) (* _index_4 500.0) "Local" false)))
        (`InstancedStaticMeshComponent.AddInstance` (`self.InstancedStaticMesh8`) (`KismetMathLibrary.MakeTransform` _returnvalue_location (struct :`Roll` 90.0)))))
    (:`then_3`
      (for _index_5 (range 31)
        (bind _returnvalue_location_2 (`KismetMathLibrary.BreakTransform` (`SplineComponent.GetTransformAtDistanceAlongSpline` (`self.Spline1`) (* _index_5 500.0) "Local" false)))
        (`InstancedStaticMeshComponent.AddInstance` (`self.InstancedStaticMesh10`) (`KismetMathLibrary.MakeTransform` _returnvalue_location_2 (struct :`Roll` 60.0) (2.0 2.0 2.0)))))
    (:`then_4`
      ;[0.657 0.1643 0] Колонны
      (for _index_6 (range 2)
        (for _index_7 (range 2)
          (`InstancedStaticMeshComponent.AddInstance` (`self.Pillars`) (`KismetMathLibrary.MakeTransform` (`KismetMathLibrary.MakeVector` (* _index_7 5700.0) (* _index_6 -5800.0) -8909.332031) (`KismetMathLibrary.MakeRotator` 0.0) (1.5 1.5 3.0))))))
    (:`then_5`
      ;[0.715 0 0.1076] Пол
      (for _index_8 (range 22)
        (for _index_9 (range 22)
          (`InstancedStaticMeshComponent.AddInstance` (`self.Floor`) (`KismetMathLibrary.MakeTransform` (`KismetMathLibrary.MakeVector` (* _index_9 265.0) (* _index_8 265.0)) (`KismetMathLibrary.MakeRotator` 0.0))))))
    (:`then_6`
      (for _index_10 (range 6)
        (bind _returnvalue_location_3 (`KismetMathLibrary.BreakTransform` (`SplineComponent.GetTransformAtDistanceAlongSpline` (`self.Spline2`) (* _index_10 1000.0) "Local" false)))
        (`InstancedStaticMeshComponent.AddInstance` (`self.Skeletons`) (`KismetMathLibrary.MakeTransform` _returnvalue_location_3))))
    (:`then_7`
      ;[0.4348 0.3865 0] Стены сокровищницы
      (for _index_11 (range 6)
        (for _index_12 (range 8)
          (`InstancedStaticMeshComponent.AddInstance` (`self.Wall`) (`KismetMathLibrary.MakeTransform` (`KismetMathLibrary.MakeVector` (* _index_12 255.0) 0.0 (* _index_11 -255.0)) (`KismetMathLibrary.MakeRotator` 0.0 0.0 180.0))))))
    (:`then_8`
      (for _index_13 (range 6)
        (for _index_14 (range 8)
          (`InstancedStaticMeshComponent.AddInstance` (`self.Wall1`) (`KismetMathLibrary.MakeTransform` (`KismetMathLibrary.MakeVector` (* _index_14 255.0) 0.0 (* _index_13 -255.0)) (`KismetMathLibrary.MakeRotator` 0.0))))))
    (:`then_9`
      (for _index_15 (range 14)
        (for _index_16 (range 8)
          (`InstancedStaticMeshComponent.AddInstance` (`self.Wall2`) (`KismetMathLibrary.MakeTransform` (`KismetMathLibrary.MakeVector` (* _index_16 255.0) (* _index_15 -255.0)) (`KismetMathLibrary.MakeRotator` 90.0))))))
    (:`then_10`
      (for _index_17 (range 14)
        (for _index_18 (range 8)
          (`InstancedStaticMeshComponent.AddInstance` (`self.Wall3`) (`KismetMathLibrary.MakeTransform` (`KismetMathLibrary.MakeVector` (* _index_18 255.0) (* _index_17 -255.0)) (`KismetMathLibrary.MakeRotator` 90.0))))))
    (:`then_11`
      (for _index_19 (range 14)
        (for _index_20 (range 6)
          (`InstancedStaticMeshComponent.AddInstance` (`self.Wall4`) (`KismetMathLibrary.MakeTransform` (`KismetMathLibrary.MakeVector` (* _index_20 255.0) (* _index_19 -255.0)) (`KismetMathLibrary.MakeRotator` 90.0))))))
    (:`then_12`
      ;[0.1353 0.686 0] Золото
      (for _index_21 (range 15)
        (for _index_22 (range 3)
          (`InstancedStaticMeshComponent.AddInstance` (`self.Gold`) (`KismetMathLibrary.MakeTransform` (`KismetMathLibrary.MakeVector` (* _index_22 215.0) (* _index_21 -225.0)) (`KismetMathLibrary.MakeRotator` 0.0) (2.0 2.0 2.0))))))
    (:`then_13`
      (for _index_23 (range 15)
        (for _index_24 (range 3)
          (`InstancedStaticMeshComponent.AddInstance` (`self.Gold1`) (`KismetMathLibrary.MakeTransform` (`KismetMathLibrary.MakeVector` (* _index_24 215.0) (* _index_23 -225.0)) (`KismetMathLibrary.MakeRotator` 0.0) (2.0 2.0 2.0))))))
    (:`then_14`
      (for _index_25 (range 15)
        (for _index_26 (range 3)
          (`InstancedStaticMeshComponent.AddInstance` (`self.Gold2`) (`KismetMathLibrary.MakeTransform` (`KismetMathLibrary.MakeVector` (* _index_26 215.0) (* _index_25 -225.0)) (`KismetMathLibrary.MakeRotator` 0.0) (2.0 2.0 2.0))))))))