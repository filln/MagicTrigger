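; Actor component for a fireball attack: it spawns a charging BP_FireBall in the owner's hand, then launches it at a target.
; CreateFireBall attaches a collisionless ball to a mesh socket, and a looping timer steps up its scale and dynamic-material emissive until maximum scale.
; MoveFireBallToTarget replaces it with a new ball at the same transform, copying the glow and passing damage, speed and target to its MoveToTarget.
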(event `self.ReceiveBeginPlay`
  (set `self.Owner` (`self.GetOwner`))
  (set `self.CountOfTimerStepsInHands` (`self.CalcCountOfStepsInHands`)))

(fn `CalcCountOfStepsInHands`
  (returns (CountOfStepsInHands :type "Float (double-precision)"))
  (bind (_sfireball_fireball _sfireball_owner _sfireball_timeinownershand) (break `/Game/MagicTrigger/Data/AttackAbilities/SFireBall` (`self.SFireBall`)))
  (return (/ _sfireball_timeinownershand (`self.ScaleAndEmissiveTimerTime`))))

(fn `CalcDeltaMultiplierOfEmissiveEveryTick`
  (params (CountOfTimerStepsInHands :type "Float (double-precision)"))
  (returns (DeltaMultiplierOfEmissiveEveryTick :type "Float (double-precision)"))
  (locals (DeltaMultiplierOfEmissive :type "Float (double-precision)" :default 0.0))
  (bind (_sfireball_fireball _sfireball_owner _sfireball_timeinownershand _sfireball_maxmultiplierofscaleinownershand _sfireball_maxemissivemultiplierinownershand) (break `/Game/MagicTrigger/Data/AttackAbilities/SFireBall` (`self.SFireBall`)))
  (set `local.DeltaMultiplierOfEmissive` (- _sfireball_maxemissivemultiplierinownershand (`/Game/MagicTrigger/Blueprints/AttackAbilities/BP_FireBall.CurrentMultiplierOfEmissive` (`self.BP_FireBallInHands`))))
  (return (/ (`local.DeltaMultiplierOfEmissive`) CountOfTimerStepsInHands)))

(fn `CalcDeltaMultiplierOfScaleEveryTick`
  (params (CountOfTimerStepsInHands :type "Float (double-precision)"))
  (returns (DeltaMultiplierOfScaleEveryTick :type "Float (double-precision)"))
  (locals (DeltaMultiplierOfScale :type "Float (double-precision)"))
  (bind (_sfireball_fireball _sfireball_owner _sfireball_timeinownershand _sfireball_maxmultiplierofscaleinownershand) (break `/Game/MagicTrigger/Data/AttackAbilities/SFireBall` (`self.SFireBall`)))
  (set `local.DeltaMultiplierOfScale` (- _sfireball_maxmultiplierofscaleinownershand (`/Game/MagicTrigger/Blueprints/AttackAbilities/BP_FireBall.CurrentMultiplierOfScale` (`self.BP_FireBallInHands`))))
  (return (/ (`local.DeltaMultiplierOfScale`) CountOfTimerStepsInHands)))

(fn `CreateFireBall`
  (params (OwnersMesh :type "SkeletalMeshComponent Object Reference"))
  (set `self.OwnersMesh` OwnersMesh)
  (if (`KismetSystemLibrary.IsValid` (`self.OwnersMesh`))
    (bind _returnvalue (`|SpawnActorFromClass` "/Game/MagicTrigger/Blueprints/AttackAbilities/BP_FireBall.BP_FireBall_C" (`SceneComponent.GetSocketTransform` (`self.OwnersMesh`) (`self.OwnersAttachSocket`) "RTS_World") "AlwaysSpawn" "OverrideRootScale" null null))
    (set `self.BP_FireBallInHands` _returnvalue)
    (`self.CreateMaterialFireBallInHands`)
    (`Actor.SetActorEnableCollision` (`self.BP_FireBallInHands`) false)
    (`Actor.K2_AttachToComponent` (`self.BP_FireBallInHands`) (`self.OwnersMesh`) (`self.OwnersAttachSocket`) "KeepWorld" "KeepWorld" "KeepWorld" true)
    (set `/Game/MagicTrigger/Blueprints/AttackAbilities/BP_FireBall.InitialScale` (`Actor.GetActorScale3D` (`self.BP_FireBallInHands`)) (`self.BP_FireBallInHands`))
    (`KismetSystemLibrary.K2_ClearAndInvalidateTimerHandle` (`self.ScaleAndEmissiveTimer`))
    (set `self.DeltaMultiplierOfScaleEveryTick` (`self.CalcDeltaMultiplierOfScaleEveryTick` (`self.CountOfTimerStepsInHands`)))
    (set `self.DeltaMultiplierOfEmissiveEveryTick` (`self.CalcDeltaMultiplierOfEmissiveEveryTick` (`self.CountOfTimerStepsInHands`)))
    (bind _returnvalue_2 (`KismetSystemLibrary.K2_SetTimer` null "ScaleAndEmissive" (`self.ScaleAndEmissiveTimerTime`) true))
    (set `self.ScaleAndEmissiveTimer` _returnvalue_2)
    (return)
    (else
      (return))))

(fn `CreateMaterialFireBallInFly`
  (bind _returnvalue (`PrimitiveComponent.CreateDynamicMaterialInstance` (`/Game/MagicTrigger/Blueprints/AttackAbilities/BP_FireBall.StaticMesh` (`self.BP_FireBallInFly`)) 0 (`/Game/MagicTrigger/Blueprints/AttackAbilities/BP_FireBall.SourceMaterial` (`self.BP_FireBallInFly`)) "None"))
  (bind _output_get (set `self.FireBallInFlyMaterial` _returnvalue))
  (`MaterialInstanceDynamic.SetTextureParameterValue` _output_get "Texture" (`/Game/MagicTrigger/Blueprints/AttackAbilities/BP_FireBall.TextureValue` (`self.BP_FireBallInFly`)))
  (`MaterialInstanceDynamic.SetVectorParameterValue` (`self.FireBallInFlyMaterial`) "EmissiveColor" (`/Game/MagicTrigger/Blueprints/AttackAbilities/BP_FireBall.EmissiveColor` (`self.BP_FireBallInHands`)))
  (`MaterialInstanceDynamic.SetScalarParameterValue` (`self.FireBallInFlyMaterial`) "EmissiveMultiplier" (`/Game/MagicTrigger/Blueprints/AttackAbilities/BP_FireBall.CurrentMultiplierOfEmissive` (`self.BP_FireBallInHands`)))
  (return))

(fn `CreateMaterialFireBallInHands`
  (bind _returnvalue (`PrimitiveComponent.CreateDynamicMaterialInstance` (`/Game/MagicTrigger/Blueprints/AttackAbilities/BP_FireBall.StaticMesh` (`self.BP_FireBallInHands`)) 0 (`/Game/MagicTrigger/Blueprints/AttackAbilities/BP_FireBall.SourceMaterial` (`self.BP_FireBallInHands`)) "None"))
  (bind _output_get (set `self.FireBallInHandsMaterial` _returnvalue))
  (`MaterialInstanceDynamic.SetTextureParameterValue` _output_get "Texture" (`/Game/MagicTrigger/Blueprints/AttackAbilities/BP_FireBall.TextureValue` (`self.BP_FireBallInHands`)))
  (`MaterialInstanceDynamic.SetVectorParameterValue` (`self.FireBallInHandsMaterial`) "EmissiveColor" (`/Game/MagicTrigger/Blueprints/AttackAbilities/BP_FireBall.EmissiveColor` (`self.BP_FireBallInHands`)))
  (`MaterialInstanceDynamic.SetScalarParameterValue` (`self.FireBallInHandsMaterial`) "EmissiveMultiplier" (`/Game/MagicTrigger/Blueprints/AttackAbilities/BP_FireBall.CurrentMultiplierOfEmissive` (`self.BP_FireBallInHands`)))
  (return))

(fn `MoveFireBallToTarget`
  (params (OwnersController :type "Controller Object Reference") (BallsTarget :type "Actor Object Reference"))
  (locals (OwnersController_ :type "Controller Object Reference") (Target_ :type "Actor Object Reference"))
  (bind (_sfireball_fireball _sfireball_owner _sfireball_timeinownershand _sfireball_maxmultiplierofscaleinownershand _sfireball_maxemissivemultiplierinownershand _sfireball_timeofmove _sfireball_damage _sfireball_multiplierofdamage _sfireball_spawnsocket _sfireball_multiplierofscaleyetdestroy _sfireball_timeofscaleyetdestroy _sfireball_speedofmovetotarget) (break `/Game/MagicTrigger/Data/AttackAbilities/SFireBall` (`self.SFireBall`)))
  (set `local.OwnersController_` OwnersController)
  (set `local.Target_` BallsTarget)
  (if (and (`KismetSystemLibrary.IsValid` (`local.OwnersController_`)) (`KismetSystemLibrary.IsValid` (`local.Target_`)) (`KismetSystemLibrary.IsValid` (`self.Owner`)))
    (set `self.SFireBallMoveToTargetInput` (make `/Game/MagicTrigger/Data/AttackAbilities/SFireBallMoveToTargetInputs` (`self.Owner`) (`local.OwnersController_`) (`local.Target_`) (`self.DamageTypeClass`) (* _sfireball_damage _sfireball_multiplierofdamage) _sfireball_speedofmovetotarget))
    (bind _returnvalue (`|SpawnActorFromClass` "/Game/MagicTrigger/Blueprints/AttackAbilities/BP_FireBall.BP_FireBall_C" (`Actor.GetTransform` (`self.BP_FireBallInHands`)) "AlwaysSpawn" "OverrideRootScale" null null))
    (set `self.BP_FireBallInFly` _returnvalue)
    (`self.CreateMaterialFireBallInFly`)
    (`Actor.K2_DetachFromActor` (`self.BP_FireBallInHands`) "KeepWorld" "KeepWorld" "KeepWorld")
    (`Actor.K2_DestroyActor` (`self.BP_FireBallInHands`))
    (`/Game/MagicTrigger/Blueprints/AttackAbilities/BP_FireBall.MoveToTarget` (`self.BP_FireBallInFly`) (`self.SFireBallMoveToTargetInput`))
    (return)
    (else
      (`/Engine/EditorBlueprintResources/StandardMacros.IsValid` (`local.Target_`)
        (:`Is Valid`
          (return))
        (:`Is Not Valid`
          (`Actor.K2_DestroyActor` (`self.BP_FireBallInHands`))
          (return))))))

(fn `ScaleAndEmissive`
  (bind (_sfireball_fireball _sfireball_owner _sfireball_timeinownershand _sfireball_maxmultiplierofscaleinownershand) (break `/Game/MagicTrigger/Data/AttackAbilities/SFireBall` (`self.SFireBall`)))
  (set `/Game/MagicTrigger/Blueprints/AttackAbilities/BP_FireBall.CurrentMultiplierOfScale` (+ (`/Game/MagicTrigger/Blueprints/AttackAbilities/BP_FireBall.CurrentMultiplierOfScale` (`self.BP_FireBallInHands`)) (`self.DeltaMultiplierOfScaleEveryTick`)) (`self.BP_FireBallInHands`))
  (`Actor.SetActorScale3D` (`self.BP_FireBallInHands`) (* (`/Game/MagicTrigger/Blueprints/AttackAbilities/BP_FireBall.InitialScale` (`self.BP_FireBallInHands`)) (`/Game/MagicTrigger/Blueprints/AttackAbilities/BP_FireBall.CurrentMultiplierOfScale` (`self.BP_FireBallInHands`))))
  (set `/Game/MagicTrigger/Blueprints/AttackAbilities/BP_FireBall.CurrentMultiplierOfEmissive` (+ (`/Game/MagicTrigger/Blueprints/AttackAbilities/BP_FireBall.CurrentMultiplierOfEmissive` (`self.BP_FireBallInHands`)) (`self.DeltaMultiplierOfEmissiveEveryTick`)) (`self.BP_FireBallInHands`))
  (`MaterialInstanceDynamic.SetScalarParameterValue` (`self.FireBallInHandsMaterial`) "EmissiveMultiplier" (`/Game/MagicTrigger/Blueprints/AttackAbilities/BP_FireBall.CurrentMultiplierOfEmissive` (`self.BP_FireBallInHands`)))
  (if (>= (`/Game/MagicTrigger/Blueprints/AttackAbilities/BP_FireBall.CurrentMultiplierOfScale` (`self.BP_FireBallInHands`)) _sfireball_maxmultiplierofscaleinownershand)
    (`KismetSystemLibrary.K2_ClearAndInvalidateTimerHandle` (`self.ScaleAndEmissiveTimer`))
    (return)
    (else
      (return))))