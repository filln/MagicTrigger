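; BP_MeleeAttackComponent is a component that performs melee hit detection and applies damage.
; TraceAttack runs a configurable sphere trace from a start point along a given direction, scaled by the attack length.
; DoAttack calls that trace and, on a hit, clears the AttackTimer handle and damages the hit actor with the caller's damage parameters.
; The file clears that timer but never sets it.
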(fn `DoAttack`
  (params (StartTrace :type "Vector Structure") (EndTraceUnit :type "Vector Structure") (ActorsToIgnore :type "Array of Actor Object Reference") (BaseDamage :type "Float (double-precision)") (EventInstigator :type "Controller Object Reference") (DamageCauser :type "Actor Object Reference") (DamageTypeClass :type "DamageType Class Reference"))
  (bind _traceoutput (`self.TraceAttack` (`local.StartTrace`) (`local.EndTraceUnit`) (`local.ActorsToIgnore`)))
  (if (`.ReturnValue_5_E3AFA2314F9AE7F7820C4A92B06AED6A` (break `/Game/MagicTrigger/Data/STraceOutput` _traceoutput))
    (`KismetSystemLibrary.K2_ClearAndInvalidateTimerHandle` (`self.AttackTimer`))
    (`GameplayStatics.ApplyDamage` (`.HitActor` (`GameplayStatics.BreakHitResult` (break `/Game/MagicTrigger/Data/STraceOutput` _traceoutput))) (`local.BaseDamage`) (`local.EventInstigator`) (`local.DamageCauser`) (`local.DamageTypeClass`))
    (return)
    (else
      (return))))

(fn `TraceAttack`
  (params (StartTrace :type "Vector Structure") (EndTraceUnit :type "Vector Structure") (ActorsToIgnore :type "Array of Actor Object Reference"))
  (returns (TraceOutput :type "/Game/MagicTrigger/Data/STraceOutput Structure"))
  (locals (EndTrace :type "Vector Structure"))
  (set `local.EndTrace` (+ (`local.StartTrace`) (* (`local.EndTraceUnit`) (`self.AttackLengthTrace`))))
  (bind (_outhit _returnvalue) (`KismetSystemLibrary.SphereTraceSingle` (`local.StartTrace`) (`local.EndTrace`) (`self.TraceSphereRadius`) (`self.TraceChannel`) (`self.TraceComplex`) ActorsToIgnore (`self.DrawDebugType`) true (`self.TraceColor`) (`self.TraceHitColor`) (`self.DrawTime`)))
  (return (make `/Game/MagicTrigger/Data/STraceOutput` _outhit _returnvalue)))