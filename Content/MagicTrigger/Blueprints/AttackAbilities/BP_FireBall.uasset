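; BP_FireBall is a fireball projectile actor for an attack ability, launched at a target actor through the MoveToTarget event.
; It enables collision and interpolates its root to the target's location captured at launch, deriving travel time from distance and speed rather than homing.
; On arrival it spawns an emitter, applies damage only if it overlaps the target, then destroys itself after a short delay.
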(event `MoveToTarget`
  (params (SFireBallMoveToTargetInput :type "/Game/MagicTrigger/Data/AttackAbilities/SFireBallMoveToTargetInputs Structure"))
  (bind (_sfireballmovetotargetinput_owner _sfireballmovetotargetinput_ownerscontroller _sfireballmovetotargetinput_target _sfireballmovetotargetinput_damagetypeclass _sfireballmovetotargetinput_damage _sfireballmovetotargetinput_speedofmovetotarget) (break `/Game/MagicTrigger/Data/AttackAbilities/SFireBallMoveToTargetInputs` (`self.SFireBallMoveToTargetInput`)))
  (bind (_sfireballmovetotargetinput_owner_2 _sfireballmovetotargetinput_ownerscontroller_2 _sfireballmovetotargetinput_target_2) (break `/Game/MagicTrigger/Data/AttackAbilities/SFireBallMoveToTargetInputs` (`self.SFireBallMoveToTargetInput`)))
  (set `self.SFireBallMoveToTargetInput` SFireBallMoveToTargetInput)
  (`self.SetActorEnableCollision` true)
  (set `self.TargetLocation` (`self.K2_GetActorLocation` _sfireballmovetotargetinput_target_2))
  (`KismetSystemLibrary.MoveComponentTo` (`self.RootComponent`) (`self.TargetLocation`) (`SceneComponent.RelativeRotation` (`self.RootComponent`)) false false (`self.CalcTimeOfMoveToTarget` _sfireballmovetotargetinput_target _sfireballmovetotargetinput_speedofmovetotarget))
  (`GameplayStatics.SpawnEmitterAtLocation` (`self.EmitterTemplate`) (`self.K2_GetActorLocation`))
  (`self.DoDamage` (`self.SFireBallMoveToTargetInput`))
  (`KismetSystemLibrary.K2_SetTimerDelegate` (delegate `DestroySelf`) 0.5))

(event `DestroySelf`
  (`self.K2_DestroyActor`))

(fn `CalcTimeOfMoveToTarget`
  (params (Target :type "Actor Object Reference") (Speed :type "Float (double-precision)"))
  (returns (TimeOfMoveToTarget :type "Float (double-precision)"))
  (return (/ (`self.GetDistanceTo` (`local.Target`)) (`local.Speed`))))

(fn `DoDamage`
  (params (SFireBallMoveToTargetInput :type "/Game/MagicTrigger/Data/AttackAbilities/SFireBallMoveToTargetInputs Structure"))
  (locals (Input :type "/Game/MagicTrigger/Data/AttackAbilities/SFireBallMoveToTargetInputs Structure"))
  (bind (_input_owner _input_ownerscontroller _input_target _input_damagetypeclass _input_damage) (break `/Game/MagicTrigger/Data/AttackAbilities/SFireBallMoveToTargetInputs` (`local.Input`)))
  (bind (_input_owner_2 _input_ownerscontroller_2 _input_target_2) (break `/Game/MagicTrigger/Data/AttackAbilities/SFireBallMoveToTargetInputs` (`local.Input`)))
  (set `local.Input` SFireBallMoveToTargetInput)
  (if (`self.IsOverlappingActor` _input_target_2)
    (`GameplayStatics.ApplyDamage` _input_target _input_damage _input_ownerscontroller _input_owner _input_damagetypeclass)
    (return)
    (else
      (return))))

(fn `UserConstructionScript`)