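; Player animation manager actor that holds the action and animation state flags for jumping, attacking, throwing, and lifting or putting down objects.
; It registers with the ReferenceAggregator and polls until ObserveManager is valid to track observe mode.
; IsPlayingAnimation functions toggle gates on conflicting actions, with fixed delays timing jump, attack and throw.
; Other events relay attack traces, throw spawning and attach/detach messages to the player character, or report noise for enemies.
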(event `self.ReceiveBeginPlay`
  ;[0.686 0.1353 0] EventBeginPlay
  (bind _referenceaggregator (`/Game/MagicTrigger/Blueprints/FunctionLibraries/BPFL_ReferenceAggregator.GetReferenceAggregator`))
  (bind _output_get (set `self.referenceAggregator` _referenceaggregator))
  (set `/Game/MagicTrigger/Blueprints/CoreClasses/BP_ReferenceAggregator.animationManager` self _output_get)
  (`/Engine/EditorBlueprintResources/StandardMacros.IsValid` (`/Game/MagicTrigger/Blueprints/CoreClasses/BP_ReferenceAggregator.observeManager` (`self.referenceAggregator`)) :!label _label
    (:`Is Valid`
      (add `/Game/MagicTrigger/Blueprints/Observe/BP_ObserveManager.onObserveMode` (`/Game/MagicTrigger/Blueprints/CoreClasses/BP_ReferenceAggregator.observeManager` (`self.referenceAggregator`)) (delegate `onObserveMode_Event_0`)))
    (:`Is Not Valid`
      (`KismetSystemLibrary.Delay` 0.2)
      (goto _label))))

(event `onObserveMode_Event_0`
  (params (`isObserveMode?` :type Boolean))
  ;[0.686 0.1353 0] EventBeginPlay
  (set `self.isObserveMode?` `isObserveMode?`))

(event `StartJump`
  ;[0 0.009662 0.8116] Прыжок
  (if (`self.IsCanJump?`)
    (`self.IsPlayingAnimationJump` true)
    (`Character.Jump` (`GameplayStatics.GetPlayerCharacter` 0))
    (`KismetSystemLibrary.Delay` 1.9)
    (if (not (`self.IsCanJump?`))
      (`self.IsPlayingAnimationJump` false))))

(event `ReportNoise`
  ;[0.6667 0 0.1564] Создать шум для врага
  (`AISense_Hearing.ReportNoiseEvent` (`self.K2_GetActorLocation` (`GameplayStatics.GetPlayerCharacter` 0)) 1.0 null 0.0 "Noise"))

(event `StopJump`
  ;[0 0.009662 0.8116] Прыжок
  (`Character.StopJumping` (`GameplayStatics.GetPlayerCharacter` 0)))

(event `AttackAnimation`
  ;[0 0.5024 0.3189] Атака
  (if (`self.isCanAttack?`)
    (`self.IsPlayingAnimationAttack` true)
    (`KismetSystemLibrary.Delay` 1.5)
    (if (not (`self.isCanAttack?`))
      (`self.IsPlayingAnimationAttack` false))))

(event `StartTraceAttack`
  ;[0 0.5024 0.3189] Атака
  (message `/Game/MagicTrigger/Blueprints/Interfaces/BPI_Animation.StartTraceAttack` (`GameplayStatics.GetPlayerCharacter` 0)))

(event `StopTraceAttack`
  ;[0 0.5024 0.3189] Атака
  (message `/Game/MagicTrigger/Blueprints/Interfaces/BPI_Animation.StopTraceAttack` (`GameplayStatics.GetPlayerCharacter` 0)))

(event `ThrowAnimation`
  ;[0.6667 0.1546 0] Бросок
  (if (`self.IsCanThrow?`)
    (`self.IsPlayingAnimationThrow` true)
    (`KismetSystemLibrary.Delay` 1.1)
    (if (not (`self.IsCanThrow?`))
      (`self.IsPlayingAnimationThrow` false))))

(event `ThrowObject`
  ;[0.6667 0.1546 0] Бросок
  (message `/Game/MagicTrigger/Blueprints/Interfaces/BPI_Animation.SpawnThrowableActor` (`GameplayStatics.GetPlayerCharacter` 0)))

(event `AttachThrowableActor`
  ;[0.05797 0.7633 0] Поднимание и опускание предмета
  (message `/Game/MagicTrigger/Blueprints/Interfaces/BPI_Animation.AttachThrowableActor` (`GameplayStatics.GetPlayerCharacter` 0)))

(event `AttachCarriedActor`
  ;[0.05797 0.7633 0] Поднимание и опускание предмета
  (message `/Game/MagicTrigger/Blueprints/Interfaces/BPI_Animation.AttachCarriedActor` (`GameplayStatics.GetPlayerCharacter` 0)))

(event `DetachLiftingActor`
  ;[0.05797 0.7633 0] Поднимание и опускание предмета
  (message `/Game/MagicTrigger/Blueprints/Interfaces/BPI_Animation.DetachLiftingActor` (`GameplayStatics.GetPlayerCharacter` 0)))

(fn `IsPlayingAnimationAttack`
  (params (`_isPlaying?` :type Boolean))
  (if `_isPlaying?`
    (set `self.isAttack?` true)
    (set `self.isCanRun?` false)
    (set `self.IsCanJump?` false)
    (set `self.isCanAttack?` false)
    (set `self.isCanInteract?` false)
    (set `self.IsCanThrow?` false)
    (else
      (set `self.isAttack?` false)
      (set `self.isCanRun?` true)
      (set `self.IsCanJump?` true)
      (set `self.isCanAttack?` true)
      (set `self.isCanInteract?` true)
      (set `self.IsCanThrow?` true)))
  (return))

(fn `IsPlayingAnimationJump`
  (params (`_isPlaying?` :type Boolean))
  (if `_isPlaying?`
    (set `self.isCanInteract?` false)
    (else
      (set `self.isCanInteract?` true))))

(fn `IsPlayingAnimationLiftUp1Hand`
  (params (`_isPlaying?` :type Boolean))
  (if `_isPlaying?`
    (set `self.isLiftUp1Hand` true)
    (`/Game/MagicTrigger/Animations/PlayerCharacter/ABP_PlayerCharacter.SetVarForAnimLiftUp1HandObject` (`self.kachujinAnimations`))
    (set `self.isCanAttack?` false)
    (set `self.IsCanThrow?` false)
    (set `self.isCanRun?` false)
    (set `self.IsCanJump?` false)
    (set `self.isCanInteract?` false)
    (else
      (set `self.isLiftUp1Hand` false)
      (set `self.isCanAttack?` true)
      (set `self.IsCanThrow?` true)
      (set `self.isCanRun?` true)
      (set `self.IsCanJump?` true)
      (set `self.isCanInteract?` true)))
  (return))

(fn `IsPlayingAnimationLiftUp2Hand`
  (params (`_isPlaying?` :type Boolean))
  (if `_isPlaying?`
    (set `self.isLiftUp2Hands` true)
    (set `self.isCanAttack?` false)
    (set `self.IsCanThrow?` false)
    (set `self.isCanRun?` false)
    (set `self.IsCanJump?` false)
    (set `self.isCanInteract?` false)
    (else
      (set `self.isCanRun?` true)
      (set `self.isCanInteract?` true)))
  (return))

(fn `IsPlayingAnimationPutDown1Hand`
  (params (`_isPlaying?` :type Boolean))
  (if `_isPlaying?`
    (set `self.isPutDown1Hand` true)
    (`/Game/MagicTrigger/Animations/PlayerCharacter/ABP_PlayerCharacter.SetVarForAnimPutDown1HandObject` (`self.kachujinAnimations`))
    (set `self.isCanAttack?` false)
    (set `self.IsCanThrow?` false)
    (set `self.isCanRun?` false)
    (set `self.IsCanJump?` false)
    (set `self.isCanInteract?` false)
    (else
      (set `self.isPutDown1Hand` false)
      (set `self.isCanAttack?` true)
      (set `self.IsCanThrow?` true)
      (set `self.isCanRun?` true)
      (set `self.IsCanJump?` true)
      (set `self.isCanInteract?` true)))
  (return))

(fn `IsPlayingAnimationPutDown2Hand`
  (params (`_isPlaying?` :type Boolean))
  (if `_isPlaying?`
    (set `self.isLiftUp2Hands` false)
    (set `self.isCanAttack?` false)
    (set `self.IsCanThrow?` false)
    (set `self.isCanRun?` false)
    (set `self.IsCanJump?` false)
    (set `self.isCanInteract?` false)
    (else
      (set `self.isCanAttack?` true)
      (set `self.IsCanThrow?` true)
      (set `self.isCanRun?` true)
      (set `self.IsCanJump?` true)
      (set `self.isCanInteract?` true)))
  (return))

(fn `IsPlayingAnimationThrow`
  (params (`_isPlaying?` :type Boolean))
  (if `_isPlaying?`
    (set `self.IsCanThrow?` false)
    (set `self.isCanAttack?` false)
    (set `self.isThrowing?` true)
    (set `self.isCanInteract?` false)
    (else
      (set `self.IsCanThrow?` true)
      (set `self.isCanAttack?` true)
      (set `self.isThrowing?` false)
      (set `self.isCanInteract?` true)))
  (return))

(fn `UserConstructionScript`)