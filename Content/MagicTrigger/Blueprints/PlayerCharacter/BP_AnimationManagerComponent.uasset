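; Player animation manager component that holds action state for jumping, throwing, attacking, one- and two-handed lifting and putting down, carrying and damage.
; SetPlayingAnimation functions toggle Can* flags so actions block one another, with delayed resets as fallbacks for throw and attack.
; Interface getters expose the state, while interface events forward noise, trace and attach/detach calls to the owner.
; One-handed put-down uses a negative play rate to play in reverse.
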(event `StartJump`
  ;[0 0.009662 0.8116] Прыжок
  (if (`self.bCanJump`)
    (`self.SetPlayingAnimationJump` true)
    (`Character.Jump` (`GameplayStatics.GetPlayerCharacter` 0))
    (`KismetSystemLibrary.Delay` 1.9)
    (if (not (`self.bCanJump`))
      (`self.SetPlayingAnimationJump` false))))

(event `StopJump`
  ;[0 0.009662 0.8116] Прыжок
  (`Character.StopJumping` (`GameplayStatics.GetPlayerCharacter` 0)))

(event `/Game/MagicTrigger/Blueprints/Interfaces/BPI_AnimationManager.ReportNoise_IF`
  ;[0.6667 0 0.1564] Создать шум для врага
  (message `/Game/MagicTrigger/Blueprints/Interfaces/BPI_AnimationManager.ReportNoise_IF` (`self.GetOwner`)))

(event `self.ReceiveBeginPlay`
  ;[1 1 1] BeginPlay
  (bind _referenceaggregator (`/Game/MagicTrigger/Blueprints/FunctionLibraries/BPFL_ReferenceAggregator.GetReferenceAggregator`))
  (set `/Game/MagicTrigger/Blueprints/CoreClasses/BP_ReferenceAggregator.BP_AnimationManagerComponent` self _referenceaggregator)
  (set `self.AnimInstance` (`SkeletalMeshComponent.GetAnimInstance` (`Character.Mesh` (`GameplayStatics.GetPlayerCharacter` 0)))))

(event `/Game/MagicTrigger/Blueprints/Interfaces/BPI_AnimationManager.SetPlayingAnimationJump_IF`
  (params (bPlaying :type Boolean))
  ;[0 0.009662 0.8116] Прыжок
  (`self.SetPlayingAnimationJump` bPlaying))

(event `ThrowAnimation`
  ;[0.6667 0.1546 0] Бросок
  (if (`self.bCanThrow`)
    (`self.SetPlayingAnimationThrow` true)
    (`KismetSystemLibrary.Delay` 1.1)
    (if (not (`self.bCanThrow`))
      (`self.SetPlayingAnimationThrow` false))))

(event `/Game/MagicTrigger/Blueprints/Interfaces/BPI_AnimationManager.SetPlayingAnimationThrow_IF`
  (params (bPlaying :type Boolean))
  ;[0.6667 0.1546 0] Бросок
  (`self.SetPlayingAnimationThrow` bPlaying))

(event `AttackAnimation`
  ;[0 0.5024 0.3189] Атака
  (if (`self.bCanAttack`)
    (`self.SetPlayingAnimationAttack` true)
    (`KismetSystemLibrary.Delay` 1.5)
    (if (not (`self.bCanAttack`))
      (`self.SetPlayingAnimationAttack` false))))

(event `/Game/MagicTrigger/Blueprints/Interfaces/BPI_AnimationManager.StartTraceAttack_IF`
  ;[0 0.5024 0.3189] Атака
  (message `/Game/MagicTrigger/Blueprints/Interfaces/BPI_AnimationManager.StartTraceAttack_IF` (`self.GetOwner`)))

(event `/Game/MagicTrigger/Blueprints/Interfaces/BPI_AnimationManager.SetCanInteract`
  (params (bCanInteract :type Boolean))
  ;[1 1 1] Interact
  (set `self.bCanInteract` bCanInteract))

(event `/Game/MagicTrigger/Blueprints/Interfaces/BPI_AnimationManager.StopTraceAttack_IF`
  ;[0 0.5024 0.3189] Атака
  (message `/Game/MagicTrigger/Blueprints/Interfaces/BPI_AnimationManager.StopTraceAttack_IF` (`self.GetOwner`)))

(event `/Game/MagicTrigger/Blueprints/Interfaces/BPI_AnimationManager.AttachThrowableActor_IF`
  ;[0.05798 0.7633 0] Поднимание и опускание предмета
  (message `/Game/MagicTrigger/Blueprints/Interfaces/BPI_AnimationManager.AttachThrowableActor_IF` (`self.GetOwner`)))

(event `/Game/MagicTrigger/Blueprints/Interfaces/BPI_AnimationManager.SetPlayingAnimationAttack_IF`
  (params (bPlaying :type Boolean))
  ;[0 0.5024 0.3189] Атака
  (`self.SetPlayingAnimationAttack` bPlaying))

(event `/Game/MagicTrigger/Blueprints/Interfaces/BPI_AnimationManager.AttachLiftingActor_IF`
  ;[0.05798 0.7633 0] Поднимание и опускание предмета
  (message `/Game/MagicTrigger/Blueprints/Interfaces/BPI_AnimationManager.AttachLiftingActor_IF` (`self.GetOwner`)))

(event `/Game/MagicTrigger/Blueprints/Interfaces/BPI_AnimationManager.DetachLiftingActor_IF`
  ;[0.05798 0.7633 0] Поднимание и опускание предмета
  (message `/Game/MagicTrigger/Blueprints/Interfaces/BPI_AnimationManager.DetachLiftingActor_IF` (`self.GetOwner`)))

(event `/Game/MagicTrigger/Blueprints/Interfaces/BPI_AnimationManager.SetGettingDamage_IF`
  (params (bGettingDamage :type Boolean))
  ;[1 1 1] Повреждения
  (set `self.bGettingDamage` bGettingDamage))

(event `/Game/MagicTrigger/Blueprints/Interfaces/BPI_AnimationManager.SetPlayingAnimationLiftUp1Hand_IF`
  (params (bPlaying :type Boolean))
  ;[0.05798 0.7633 0] Поднимание и опускание предмета
  (`self.SetPlayingAnimationLiftUp1Hand` bPlaying))

(event `/Game/MagicTrigger/Blueprints/Interfaces/BPI_AnimationManager.SetPlayingAnimationPutDown1Hand_IF`
  (params (bPlaying :type Boolean))
  ;[0.05798 0.7633 0] Поднимание и опускание предмета
  (`self.SetPlayingAnimationPutDown1Hand` bPlaying))

(event `/Game/MagicTrigger/Blueprints/Interfaces/BPI_AnimationManager.SetPlayingAnimationLiftUp2Hand_IF`
  (params (bPlaying :type Boolean))
  ;[0.05798 0.7633 0] Поднимание и опускание предмета
  (`self.SetPlayingAnimationLiftUp2Hand` bPlaying))

(event `/Game/MagicTrigger/Blueprints/Interfaces/BPI_AnimationManager.SetPlayingAnimationPutDown2Hand_IF`
  (params (bPlaying :type Boolean))
  ;[0.05798 0.7633 0] Поднимание и опускание предмета
  (`self.SetPlayingAnimationPutDown2Hand` bPlaying))

(event `/Game/MagicTrigger/Blueprints/Interfaces/BPI_AnimationManager.SetCarrying_IF`
  (params (bCarrying :type Boolean))
  ;[0.05798 0.7633 0] Поднимание и опускание предмета
  (set `self.bCarrying` bCarrying))

(fn `GetAnimationManagerComponent_IF`
  (returns (AnimationManagerComponent :type "ActorComponent Object Reference"))
  (return null))

(fn `GetAttacking_IF`
  (returns (bAttacking :type Boolean))
  (return (`self.bAttacking`)))

(fn `GetCarrying_IF`
  (returns (bCarrying :type Boolean))
  (return (`self.bCarrying`)))

(fn `GetDying_IF`
  (returns (bDying :type Boolean))
  (return (`self.bDying`)))

(fn `GetGettingDamage_IF`
  (returns (bGettingDamage :type Boolean))
  (return (`self.bGettingDamage`)))

(fn `GetLiftingUp1Hand_IF`
  (returns (bLiftingUp1Hand :type Boolean))
  (return (`self.bLiftingUp1Hand`)))

(fn `GetLiftingUp2Hands_IF`
  (returns (bLiftingUp2Hands :type Boolean))
  (return (`self.bLiftingUp2Hands`)))

(fn `GetPlayRateLiftingThrowingObject_IF`
  (returns (PlayRateLiftingThrowingObject :type "Float (double-precision)"))
  (return (`self.PlayRateLiftingThrowingObject`)))

(fn `GetPutingDown1Hand_IF`
  (returns (bPutingDown1Hand :type Boolean))
  (return (`self.bPutingDown1Hand`)))

(fn `GetStartPositionLiftingThrowingObject_IF`
  (returns (StartPositionLiftingThrowingObject :type "Float (double-precision)"))
  (return (`self.StartPositionLiftingThrowingObject`)))

(fn `GetThrowing_IF`
  (returns (bThrowing :type Boolean))
  (return (`self.bThrowing`)))

(fn `GetWatchingNow_IF`
  (returns (bWatchingNow :type Boolean))
  (return (`self.bWatchingNow`)))

(fn `SetPlayingAnimationAttack`
  (params (bPlaying :type Boolean))
  (if bPlaying
    (set `self.bAttacking` true)
    (set `self.bCanRun` false)
    (set `self.bCanJump` false)
    (set `self.bCanAttack` false)
    (set `self.bCanInteract` false)
    (set `self.bCanThrow` false)
    (else
      (set `self.bAttacking` false)
      (set `self.bCanRun` true)
      (set `self.bCanJump` true)
      (set `self.bCanAttack` true)
      (set `self.bCanInteract` true)
      (set `self.bCanThrow` true)))
  (return))

(fn `SetPlayingAnimationJump`
  (params (bPlaying :type Boolean))
  (if bPlaying
    (set `self.bCanInteract` false)
    (else
      (set `self.bCanInteract` true))))

(fn `SetPlayingAnimationLiftUp1Hand`
  (params (bPlaying :type Boolean))
  (if bPlaying
    (set `self.bLiftingUp1Hand` true)
    (set `self.PlayRateLiftingThrowingObject` 2.0)
    (set `self.StartPositionLiftingThrowingObject` 0.0)
    (set `self.bCanAttack` false)
    (set `self.bCanThrow` false)
    (set `self.bCanRun` false)
    (set `self.bCanJump` false)
    (set `self.bCanInteract` false)
    (else
      (set `self.bLiftingUp1Hand` false)
      (set `self.bCanAttack` true)
      (set `self.bCanThrow` true)
      (set `self.bCanRun` true)
      (set `self.bCanJump` true)
      (set `self.bCanInteract` true)))
  (return))

(fn `SetPlayingAnimationLiftUp2Hand`
  (params (bPlaying :type Boolean))
  (if bPlaying
    (set `self.bLiftingUp2Hands` true)
    (set `self.bCanAttack` false)
    (set `self.bCanThrow` false)
    (set `self.bCanRun` false)
    (set `self.bCanJump` false)
    (set `self.bCanInteract` false)
    (else
      (set `self.bCanRun` true)
      (set `self.bCanInteract` true)))
  (return))

(fn `SetPlayingAnimationPutDown1Hand`
  (params (bPlaying :type Boolean))
  (if bPlaying
    (set `self.bPutingDown1Hand` true)
    (set `self.PlayRateLiftingThrowingObject` -2.0)
    (set `self.StartPositionLiftingThrowingObject` 3.0)
    (set `self.bCanAttack` false)
    (set `self.bCanThrow` false)
    (set `self.bCanRun` false)
    (set `self.bCanJump` false)
    (set `self.bCanInteract` false)
    (else
      (set `self.bPutingDown1Hand` false)
      (set `self.bCanAttack` true)
      (set `self.bCanThrow` true)
      (set `self.bCanRun` true)
      (set `self.bCanJump` true)
      (set `self.bCanInteract` true)))
  (return))

(fn `SetPlayingAnimationPutDown2Hand`
  (params (bPlaying :type Boolean))
  (if bPlaying
    (set `self.bLiftingUp2Hands` false)
    (set `self.bCanAttack` false)
    (set `self.bCanThrow` false)
    (set `self.bCanRun` false)
    (set `self.bCanJump` false)
    (set `self.bCanInteract` false)
    (else
      (set `self.bCanAttack` true)
      (set `self.bCanThrow` true)
      (set `self.bCanRun` true)
      (set `self.bCanJump` true)
      (set `self.bCanInteract` true)))
  (return))

(fn `SetPlayingAnimationThrow`
  (params (bPlaying :type Boolean))
  (if bPlaying
    (set `self.bCanThrow` false)
    (set `self.bCanAttack` false)
    (set `self.bThrowing` true)
    (set `self.bCanInteract` false)
    (else
      (set `self.bCanThrow` true)
      (set `self.bCanAttack` true)
      (set `self.bThrowing` false)
      (set `self.bCanInteract` true)))
  (return))

(fn `StopAnimations`
  (if (`AnimInstance.Montage_IsPlaying` (`self.AnimInstance`) "/Game/MagicTrigger/Animations/PlayerCharacter/Attack/AM_Player_FightIdle.AM_Player_FightIdle")
    (`AnimInstance.Montage_Stop` (`self.AnimInstance`) 0.0 "/Game/MagicTrigger/Animations/PlayerCharacter/Attack/AM_Player_FightIdle.AM_Player_FightIdle")
    (return)
    (else
      (return))))