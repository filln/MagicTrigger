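; Player character component that lets its owner lift, carry, put down or destroy an object of LiftUpClass.
; LiftUp picks an overlapping actor, preferring the observed one, and PutDown requires a clear forward trace plus a surface hit; both then start animations.
; Separate attach and detach events move the object to a mesh socket or the traced point, toggling its collision.
; Owner and object are accessed through interface messages.
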(event `self.ReceiveBeginPlay`
  (set `self.Owner` (`self.GetOwner`)))

(event `DetachLiftingActor`
  (bind (_detachliftingactortraceout_bblockinghit _detachliftingactortraceout_binitialoverlap _detachliftingactortraceout_time _detachliftingactortraceout_distance _detachliftingactortraceout_location) (`GameplayStatics.BreakHitResult` (`self.DetachLiftingActorTraceOut`)))
  (`/Engine/EditorBlueprintResources/StandardMacros.IsValid` (`self.LiftUpObject`)
    (:`Is Valid`
      (set `self.Owner` (`self.GetOwner`))
      (`Actor.K2_DetachFromActor` (`self.LiftUpObject`) "KeepWorld" "KeepWorld" "KeepWorld")
      (bind _pointputdowntransform (message `/Game/MagicTrigger/Blueprints/Interfaces/BPI_PlayerCharacter.GetPointPutDownTransform_IF` (`self.Owner`)))
      (`KismetSystemLibrary.MoveComponentTo` (`Actor.RootComponent` (`self.LiftUpObject`)) _detachliftingactortraceout_location (.rotation _pointputdowntransform) false false 0.3)
      (`Actor.SetActorEnableCollision` (`self.LiftUpObject`) true)
      (set `self.LiftUpObject` null))))

(event `AttachLiftingActor`
  (`/Engine/EditorBlueprintResources/StandardMacros.IsValid` (`self.LiftUpObject`)
    (:`Is Valid`
      (bind _attachsocket (message `/Game/MagicTrigger/Blueprints/Interfaces/BPI_LiftingObjects.GetAttachSocket_IF` (`self.LiftUpObject`)))
      (set `self.AttachSocket` _attachsocket)
      (`Actor.SetActorEnableCollision` (`self.LiftUpObject`) false)
      (bind _mesh (message `/Game/MagicTrigger/Blueprints/Interfaces/BPI_PlayerCharacter.GetMesh_IF` (`self.Owner`)))
      (set `self.OwnersMesh` _mesh)
      (`KismetSystemLibrary.MoveComponentTo` (`Actor.RootComponent` (`self.LiftUpObject`)) (`SceneComponent.GetSocketLocation` (`self.OwnersMesh`) (`self.AttachSocket`)) (`SceneComponent.K2_GetComponentRotation` (`Actor.RootComponent` (`self.LiftUpObject`))))
      (`Actor.K2_AttachToComponent` (`self.LiftUpObject`) (`self.OwnersMesh`) (`self.AttachSocket`) "SnapToTarget" "KeepWorld" "KeepWorld" true))))

(fn `DestroyLiftingActor`
  (`Actor.K2_DestroyActor` (`self.LiftUpObject`))
  (set `self.LiftUpObject` null))

(fn `FindLifUpObject`
  (returns (LifUpObject :type "Actor Object Reference"))
  (locals (OverlappingActors :type "Array of Actor Object Reference") (ObservedActor :type "Actor Object Reference") (CurrentActorInLoop :type "Actor Object Reference"))
  (bind _interactcollision (message `/Game/MagicTrigger/Blueprints/Interfaces/BPI_PlayerCharacter.GetInteractCollision_IF` (`self.GetOwner`)))
  (set `local.OverlappingActors` (`PrimitiveComponent.GetOverlappingActors` _interactcollision (`self.LiftUpClass`)))
  (if (!= (`KismetArrayLibrary.Array_Length` (`local.OverlappingActors`)) 0)
    (bind _observedactor (message `/Game/MagicTrigger/Blueprints/Interfaces/BPI_OwnerTargetSelection.GetObservedActor_IF` (`self.GetOwner`)))
    (bind _output_get (set `local.ObservedActor` _observedactor))
    (`/Engine/EditorBlueprintResources/StandardMacros.IsValid` _output_get
      (:`Is Valid`
        ;[1 1 1] Если актор в коллизии равен наблюдаемому, то назначить его.
        (for _array_element (`local.OverlappingActors`)
          (set `local.CurrentActorInLoop` _array_element)
          (`/Engine/EditorBlueprintResources/StandardMacros.IsValid` (`local.CurrentActorInLoop`)
            (:`Is Valid`
              (if (== (`local.CurrentActorInLoop`) (`local.ObservedActor`))
                (set `self.LiftUpObject` (`local.CurrentActorInLoop`))
                (break)))))
        (`/Engine/EditorBlueprintResources/StandardMacros.IsValid` (`self.LiftUpObject`)
          (:`Is Valid`
            (return (`self.LiftUpObject`)))
          (:`Is Not Valid`
            _)))
      (:`Is Not Valid`
        _))
    ;[1 1 1] Найти первый валидный актор.
    (for _array_element_2 (`local.OverlappingActors`)
      (set `local.CurrentActorInLoop` _array_element_2)
      (`/Engine/EditorBlueprintResources/StandardMacros.IsValid` (`local.CurrentActorInLoop`)
        (:`Is Valid`
          (set `self.LiftUpObject` (`local.CurrentActorInLoop`))
          (break))))
    (return (`self.LiftUpObject`))
    (else
      (return null))))

(fn `LiftUp`
  (`/Engine/EditorBlueprintResources/StandardMacros.IsValid` (`self.LiftUpObject`)
    (:`Is Valid`
      (return))
    (:`Is Not Valid`
      (bind _lifupobject (`self.FindLifUpObject`))
      (`/Engine/EditorBlueprintResources/StandardMacros.IsValid` _lifupobject
        (:`Is Valid`
          (message `/Game/MagicTrigger/Blueprints/Interfaces/BPI_OwnerTargetSelection.OffWatchingActors_IF` (`self.GetOwner`))
          (set `self.LiftUpObjectTransform` (`Actor.GetTransform` (`self.LiftUpObject`)))
          (message `/Game/MagicTrigger/Blueprints/Interfaces/BPI_LiftingObjects.SetPlayingAnimationLiftUp_IF` (`self.LiftUpObject`) true)
          (return))
        (:`Is Not Valid`
          (return))))))

(fn `PutDown`
  (`/Engine/EditorBlueprintResources/StandardMacros.IsValid` (`self.LiftUpObject`)
    (:`Is Valid`
      (bind _returnvalue (`self.TraceObstacle`))
      (if _returnvalue
        (return)
        (else
          (bind _returnvalue_2 (`self.TracePutDownPoint`))
          (if _returnvalue_2
            (message `/Game/MagicTrigger/Blueprints/Interfaces/BPI_LiftingObjects.SetPlayingAnimationPutDown_IF` (`self.LiftUpObject`) true)
            (return)
            (else
              (return))))))
    (:`Is Not Valid`
      (return))))

(fn `TraceObstacle`
  (returns (ReturnValue :type Boolean))
  (locals (OwnerLoc :type "Actor Object Reference") (TraceStartLoc :type "Vector Structure") (TraceEndLoc :type "Vector Structure"))
  (set `local.OwnerLoc` (`self.GetOwner`))
  (bind _sockettransform (message `/Game/MagicTrigger/Blueprints/Interfaces/BPI_PlayerCharacter.GetSocketTransform_IF` (`local.OwnerLoc`) "Hips"))
  (set `local.TraceStartLoc` (.location _sockettransform))
  (bind _updownliftingarrow (message `/Game/MagicTrigger/Blueprints/Interfaces/BPI_PlayerCharacter.GetUpDownLiftingArrow_IF` (`local.OwnerLoc`)))
  (set `local.TraceEndLoc` (+ (`local.TraceStartLoc`) (* (`SceneComponent.GetForwardVector` _updownliftingarrow) (`self.DistanceOfTrace`))))
  (bind (_outhit _returnvalue) (`KismetSystemLibrary.LineTraceSingle` (`local.TraceStartLoc`) (`local.TraceEndLoc`) "TraceTypeQuery1" true (`|MakeArray` (`self.LiftUpObject`) (`local.OwnerLoc`)) "None" true (struct :`R` 1.0 :`A` 1.0) (struct :`G` 1.0 :`A` 1.0) 10000.0))
  (return _returnvalue))

(fn `TracePutDownPoint`
  (returns (ReturnValue :type Boolean))
  (locals (EndTrace :type "Transform Structure") (StartTrace :type "Transform Structure") (EndTraceLocation :type "Vector Structure"))
  (bind _endtrace (`local.EndTrace`))
  (bind _starttrace_location (`KismetMathLibrary.BreakTransform` (`local.StartTrace`)))
  (bind _pointputdowntransform (message `/Game/MagicTrigger/Blueprints/Interfaces/BPI_PlayerCharacter.GetPointPutDownTransform_IF` (`self.Owner`)))
  (set `local.EndTrace` _pointputdowntransform)
  (bind _pointstarttracetoputdownpointtransform (message `/Game/MagicTrigger/Blueprints/Interfaces/BPI_PlayerCharacter.GetPointStartTraceToPutDownPointTransform_IF` (`self.Owner`)))
  (set `local.StartTrace` _pointstarttracetoputdownpointtransform)
  (set `local.EndTraceLocation` (`KismetMathLibrary.MakeVector` (.x (.location _endtrace)) (.y (.location _endtrace)) (+ (.z (.location _endtrace)) (`self.DeltaTraceZ`))))
  (bind (_outhit _returnvalue) (`KismetSystemLibrary.LineTraceSingle` _starttrace_location (`local.EndTraceLocation`) "TraceTypeQuery1" true (`|MakeArray` (`self.LiftUpObject`) (`self.Owner`)) "None" true (struct :`R` 1.0 :`A` 1.0) (struct :`G` 1.0 :`A` 1.0) 10.0))
  (set `self.DetachLiftingActorTraceOut` _outhit)
  (return _returnvalue))