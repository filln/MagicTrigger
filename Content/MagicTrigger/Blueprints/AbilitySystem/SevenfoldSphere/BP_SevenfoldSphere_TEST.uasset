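; BP_SevenfoldSphere_TEST is a test actor for the Sevenfold Sphere ability that pulses in size and glow when spawned.
; Its construction script puts a dynamic M_AttackAbility material instance on the static mesh.
; From BeginPlay, one timeline plays forward and then reverses on finish, lerping actor scale between its initial value and a MaxScale multiple, and EmissiveMultiplier between zero and MaxEmissive.
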(event `self.ReceiveBeginPlay`
  (`self.IncreaseScaleAndEmissiveAfterSpawn`))

(event `IncreaseScaleAndEmissiveAfterSpawn`
  (set `self.InitialScale` (`self.GetActorScale3D`))
  (bind (_direction _newtrack_0) (`Timeline|ScaleAndEmissiveTimeline` :!label _label)
    (:`Update`
      (`self.ScaleAndEmissiveTimelineUpdate` _newtrack_0))
    (:`Finished`
      (`self.DecreaseScaleAndEmissiveAfterSpawn`))))

(event `DecreaseScaleAndEmissiveAfterSpawn`
  (goto _label :!via `Reverse`))

(fn `ScaleAndEmissiveTimelineUpdate`
  (params (InAlpha :type "Float (double-precision)"))
  (`MaterialInstanceDynamic.SetScalarParameterValue` (`self.Material`) "EmissiveMultiplier" (`KismetMathLibrary.Lerp` 0.0 (`self.MaxEmissive`) InAlpha))
  (`self.SetActorScale3D` (* (`self.InitialScale`) (`KismetMathLibrary.Lerp` 1.0 (`self.MaxScale`) InAlpha))))

(fn `UserConstructionScript`
  (bind _staticmesh (`self.StaticMesh`))
  (bind _returnvalue (`PrimitiveComponent.CreateDynamicMaterialInstance` _staticmesh 0 "/Game/MagicTrigger/Materials/AbilitySystem/M_AttackAbility.M_AttackAbility" "None"))
  (bind _output_get (set `self.Material` _returnvalue))
  (`PrimitiveComponent.SetMaterial` _staticmesh 0 _output_get))