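; Older observe manager that provides target lock-on, keeping the player character facing one observed actor.
; ObserveActors gathers actors in a supplied collision by class, exclusion class and interface, bubble-sorts them by distance, then picks or cycles the target, notifying it by interface messages.
; Observe mode changes character movement, while a looping timer turns the player's yaw toward the target during movement.
; AutoSwitchActors retargets to the nearest remaining actor or ends observation.
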(event `self.ReceiveBeginPlay`
  (bind _animationmanager (`/Game/MagicTrigger/Blueprints/CoreClasses/ReferenceAggregator.animationManager` (`self.referenceAggregator`)))
  (`|ExecutionSequence`
    (:`then_0`
      (bind _referenceaggregator (`/Game/MagicTrigger/Blueprints/FunctionLibraries/BPFL_ReferenceAggregator.GetReferenceAggregator`))
      (bind _output_get (set `self.referenceAggregator` _referenceaggregator))
      ;[0 0.3865 0.4348] SELF
      (set `/Game/MagicTrigger/Blueprints/CoreClasses/ReferenceAggregator.observeManager` null _output_get)
      (`/Engine/EditorBlueprintResources/StandardMacros.IsValid` _animationmanager :!label _label
        (:`Is Valid`
          (set `self.animationManager` _animationmanager))
        (:`Is Not Valid`
          (`KismetSystemLibrary.Delay` 0.2)
          (goto _label))))
    (:`then_1`
      (bind _returnvalue (`KismetSystemLibrary.K2_SetTimerDelegate` (delegate `EventFindLookActor`) 0.01 true))
      (bind _output_get_2 (set `self.FindLookActorTimer` _returnvalue))
      (`KismetSystemLibrary.K2_PauseTimerHandle` _output_get_2))))

(event `EventFindLookActor`
  (if (> (`KismetMathLibrary.VSize` (`self.GetVelocity` (`GameplayStatics.GetPlayerCharacter` 0))) 0.0)
    (`self.FindLookActor`)))

(event `ObserveActors`
  (params (__ClassFilter :type "Actor Class Reference") (`__ClassFilter(NOT)` :type "Actor Class Reference") (__InterfaceFilter :type "Interface Class Reference") (ObserveSphereCollision :type "SphereComponent Object Reference"))
  (if (`KismetSystemLibrary.IsValidClass` __ClassFilter)
    (if (`KismetSystemLibrary.IsValidClass` (`self.classFilter`))
      (if (== __ClassFilter (`self.classFilter`))
        (bind _isfindactor (`self.SwitchActors` :!label _label_2))
        (if _isfindactor
          (`self.FindLookActor`)
          (`KismetSystemLibrary.K2_UnPauseTimerHandle` (`self.FindLookActorTimer`)))
        (else
          ;[0.1836 0 0.6453] Если входная ссылка не равна classFilter, то параметры наблюдения поменялись, значит отключить наблюдение и начать наблюдение заново
          (`self.OffObserveActor`)
          (set `self.classFilter` __ClassFilter :!label _label_3)
          (set `self.classFilter(NOT)` `__ClassFilter(NOT)`)
          (set `self.interfaceFilter` __InterfaceFilter)
          (`/Engine/EditorBlueprintResources/StandardMacros.IsValid` ObserveSphereCollision
            (:`Is Valid`
              (set `self.observeCollision` ObserveSphereCollision)
              (goto _label_2))
            (:`Is Not Valid`
              ;[0.3865 0 0.44] Если коллизия не выбрана
              (`KismetSystemLibrary.PrintString` "ObserveCollision is not valid, you must set collision")))))
      (else
        (goto _label_3)))
    (else
      ;[0.1353 0.686 0] Если входной класс не выбран
      (`KismetSystemLibrary.PrintString` "ClassFilter is not valid, you must set this"))))

(fn `AddObservableActor`
  (params (AddedActor :type "Actor Object Reference"))
  (`/Engine/EditorBlueprintResources/StandardMacros.IsValid` (`self.observableActor`)
    (:`Is Valid`
      (`KismetArrayLibrary.Array_Add` (`self.observableActorsArr`) AddedActor)
      (return))
    (:`Is Not Valid`
      (return))))

(fn `AutoSwitchActors`
  (params (_EndOverlappingActor :type "Actor Object Reference"))
  (locals (SortedOverlappingActors :type "Array of Actor Object Reference") (EndOverlappingActor :type "Actor Object Reference") (OverlappingActors :type "Array of Actor Object Reference"))
  (`/Engine/EditorBlueprintResources/StandardMacros.IsValid` (`self.observableActor`)
    (:`Is Valid`
      (if (== _EndOverlappingActor (`self.observableActor`))
        (if (`KismetSystemLibrary.DoesImplementInterface` _EndOverlappingActor (`self.interfaceFilter`))
          (set `local.EndOverlappingActor` _EndOverlappingActor)
          (bind __overlappingactorswithinterface (`self.GetOverlappingActorsWithInterface` (`local.OverlappingActors`)))
          (if (!= (`KismetArrayLibrary.Array_Length` __overlappingactorswithinterface) 0)
            ;[0.3865 0.4348 0] Если остаются Акторы в сфере после потери наблюдаемого, переключиться на ближайшего актора
            (bind __sortedoverlappingactors (`self.SortActorsByDistance` __overlappingactorswithinterface))
            (set `local.SortedOverlappingActors` __sortedoverlappingactors)
            (set `self.observableActor` (`|GetArrayItem` (`local.SortedOverlappingActors`)))
            (message `/Game/MagicTrigger/Blueprints/Interfaces/BPI_Observe.BecomeNotObservable` (`local.EndOverlappingActor`))
            (message `/Game/MagicTrigger/Blueprints/Interfaces/BPI_Observe.BecomeObservable` (`self.observableActor`))
            (return)
            (else
              ;[0.6087 0 0.2151] Если Актор был последним в сфере, выключить наблюдение
              (`self.OffObserveActor`)
              (return)))
          (else
            (return)))
        (else
          (return))))
    (:`Is Not Valid`
      (return))))

(fn `FindLookActor`
  (bind _returnvalue (`GameplayStatics.GetPlayerCharacter` 0))
  (bind (_returnvalue_roll _returnvalue_pitch) (`KismetMathLibrary.BreakRotator` (`self.K2_GetActorRotation` _returnvalue)))
  (bind (_returnvalue_roll_2 _returnvalue_pitch_2 _returnvalue_yaw) (`KismetMathLibrary.BreakRotator` (`KismetMathLibrary.FindLookAtRotation` (`self.K2_GetActorLocation` _returnvalue) (`self.K2_GetActorLocation` (`self.observableActor`)))))
  (`/Engine/EditorBlueprintResources/StandardMacros.IsValid` (`self.observableActor`)
    (:`Is Valid`
      (`self.K2_SetActorRotation` _returnvalue (`KismetMathLibrary.MakeRotator` _returnvalue_roll _returnvalue_pitch _returnvalue_yaw) false)
      (return))
    (:`Is Not Valid`
      (return))))

(fn `GetOverlappingActorsWithInterface`
  (params (__OverlappingActors :type "Array of Actor Object Reference"))
  (returns (_OverlappingActorsWithInterface :type "Array of Actor Object Reference"))
  (locals (OverlappingActors :type "Array of Actor Object Reference") (CurrentOverlapActor :type "Actor Object Reference") (isFilter :type Boolean))
  (bind _overlappingactors (`PrimitiveComponent.GetOverlappingActors` (`self.ObserveCollision`) (`self.classFilter(NOT)`)))
  (set `local.OverlappingActors` __OverlappingActors)
  (`KismetArrayLibrary.Array_Clear` (`local.OverlappingActors`))
  (for _array_element (`PrimitiveComponent.GetOverlappingActors` (`self.ObserveCollision`) (`self.classFilter`))
    (set `local.CurrentOverlapActor` _array_element)
    (if (`KismetSystemLibrary.DoesImplementInterface` (`local.CurrentOverlapActor`) (`self.interfaceFilter`))
      (if (`KismetSystemLibrary.IsValidClass` (`self.classFilter(NOT)`))
        (if (!= (`KismetArrayLibrary.Array_Length` _overlappingactors) 0)
          (set `local.isFilter` false)
          (for _array_element_2 _overlappingactors
            (if (== _array_element_2 (`local.CurrentOverlapActor`))
              (set `local.isFilter` true)
              (break)))
          (if (not (`local.isFilter`))
            (`KismetArrayLibrary.Array_Add` (`local.OverlappingActors`) (`local.CurrentOverlapActor`)))
          (else
            (`KismetArrayLibrary.Array_Add` (`local.OverlappingActors`) (`local.CurrentOverlapActor`))))
        (else
          (`KismetArrayLibrary.Array_Add` (`local.OverlappingActors`) (`local.CurrentOverlapActor`))))))
  (return (`local.OverlappingActors`)))

(fn `ObserveMode`
  (params (`__On/Off` :type Boolean))
  (bind _charactermovement (`Character.CharacterMovement` (`GameplayStatics.GetPlayerCharacter` 0)))
  (if `__On/Off`
    (`self.onObserveMode` true)
    (set `CharacterMovementComponent.bOrientRotationToMovement` false _charactermovement)
    (set `CharacterMovementComponent.AirControl` 1.0 _charactermovement)
    (else
      (`self.onObserveMode` false)
      (set `CharacterMovementComponent.bOrientRotationToMovement` true _charactermovement)
      (set `CharacterMovementComponent.AirControl` 0.5 _charactermovement)))
  (return))

(fn `OffObserveActor`
  (`/Engine/EditorBlueprintResources/StandardMacros.IsValid` (`self.observableActor`)
    (:`Is Valid`
      (message `/Game/MagicTrigger/Blueprints/Interfaces/BPI_Observe.BecomeNotObservable` (`self.observableActor`))
      (set `self.observableActor` null)
      (set `self.classFilter` null)
      (set `self.classFilter(NOT)` null)
      (set `self.interfaceFilter` null)
      (set `self.observeCollision` null)
      (`KismetSystemLibrary.K2_PauseTimerHandle` (`self.FindLookActorTimer`))
      (`self.ObserveMode` false)
      (return))
    (:`Is Not Valid`
      (return))))

(fn `OnObserveNewActor`
  (params (__OverlappingActors :type "Array of Actor Object Reference"))
  (bind _output (`|GetArrayItem` __OverlappingActors))
  (set `self.observableActor` _output)
  (message `/Game/MagicTrigger/Blueprints/Interfaces/BPI_Observe.BecomeObservable` _output)
  (`self.ObserveMode` true)
  (return))

(fn `SelectObserveObjects`)

(fn `SortActorsByDistance`
  (params (__OverlappingActors :type "Array of Actor Object Reference"))
  (returns (_SortedOverlappingActors :type "Array of Actor Object Reference"))
  (locals (OverlappingActors :type "Array of Actor Object Reference") (CurrentIndex :type Integer))
  (bind _returnvalue (- (`KismetArrayLibrary.Array_Length` (`local.OverlappingActors`)) 2))
  (set `local.OverlappingActors` __OverlappingActors)
  (if (not (<= (`KismetArrayLibrary.Array_Length` (`local.OverlappingActors`)) 1))
    (for _ (range (+ _returnvalue 1))
      (for _index (range (+ _returnvalue 1))
        (set `local.CurrentIndex` _index)
        (if (< (`self.GetDistanceTo` (`|GetArrayItem` (`local.OverlappingActors`) (+ (`local.CurrentIndex`) 1)) (`GameplayStatics.GetPlayerCharacter` 0)) (`self.GetDistanceTo` (`|GetArrayItem` (`local.OverlappingActors`) (`local.CurrentIndex`)) (`GameplayStatics.GetPlayerCharacter` 0)))
          (`KismetArrayLibrary.Array_Swap` (`local.OverlappingActors`) (+ (`local.CurrentIndex`) 1) (`local.CurrentIndex`))))))
  (return (`local.OverlappingActors`)))

(fn `SwitchActors`
  (returns (IsFindActor :type Boolean))
  (locals (OverlappingActors :type "Array of Actor Object Reference") (SortedOverlappingActors :type "Array of Actor Object Reference"))
  ;[0.1546 0 0.6746] Взять Акторы с интерфейсом в массив, если их не меньше один+один(в методе сортировки), то отсортировать массив, затем проверить, есть ли Акторы в наблюдении
  (bind __overlappingactorswithinterface (`self.GetOverlappingActorsWithInterface` (`local.OverlappingActors`)))
  (if (!= (`KismetArrayLibrary.Array_Length` __overlappingactorswithinterface) 0)
    (bind __sortedoverlappingactors (`self.SortActorsByDistance` __overlappingactorswithinterface))
    (set `local.SortedOverlappingActors` __sortedoverlappingactors)
    (`/Engine/EditorBlueprintResources/StandardMacros.IsValid` (`self.observableActor`)
      (:`Is Valid`
        ;[0 0.5314 0.2899] Переключаться между акторами, если их больше одного
        (if (== (`KismetArrayLibrary.Array_Length` (`local.SortedOverlappingActors`)) 1)
          ;[0.4541 0 0.3715] Переключиться на нового
          (`self.OnObserveNewActor` (`local.SortedOverlappingActors`))
          (return true)
          (else
            (`self.SwitchMoreThanOneActor` (`local.SortedOverlappingActors`))
            (return true))))
      (:`Is Not Valid`
        ;;[0.5604 0.2609 0] Переключиться на нового
        (`self.OnObserveNewActor` (`local.SortedOverlappingActors`))
        (return true)))
    (else
      (return false))))

(fn `SwitchMoreThanOneActor`
  (params (__OverlappingActors :type "Array of Actor Object Reference"))
  (locals (OverlappingActors :type "Array of Actor Object Reference") (CurrentIndex :type Integer) (CurrentActor :type "Actor Object Reference"))
  (bind _output_get (set `local.OverlappingActors` __OverlappingActors))
  (for (_array_element _array_index) _output_get
    (set `local.CurrentIndex` _array_index)
    (bind _output_get_2 (set `local.CurrentActor` _array_element))
    (if (== _output_get_2 (`self.observableActor`))
      (if (== (`local.CurrentIndex`) (`KismetArrayLibrary.Array_LastIndex` (`local.OverlappingActors`)))
        ;[0 0.6957 0.1256] Если наблюдаемый актор не найден в массиве или найден в конце массива, то переключиться на нулевой индекс
        (set `self.observableActor` (`|GetArrayItem` (`local.OverlappingActors`)) :!label _label)
        (message `/Game/MagicTrigger/Blueprints/Interfaces/BPI_Observe.BecomeNotObservable` (`local.CurrentActor`))
        (message `/Game/MagicTrigger/Blueprints/Interfaces/BPI_Observe.BecomeObservable` (`self.observableActor`))
        (else
          ;[0 0.1643 0.657] Если наблюдаемый актор найден не в конце массива, то переключиться на след. индекс
          (set `self.observableActor` (`|GetArrayItem` (`local.OverlappingActors`) (+ (`local.CurrentIndex`) 1)))
          (message `/Game/MagicTrigger/Blueprints/Interfaces/BPI_Observe.BecomeNotObservable` (`local.CurrentActor`))
          (message `/Game/MagicTrigger/Blueprints/Interfaces/BPI_Observe.BecomeObservable` (`self.observableActor`))
          (break)))
      (elif (== (`local.CurrentIndex`) (`KismetArrayLibrary.Array_LastIndex` (`local.OverlappingActors`)))
        (goto _label))))
  (return))

(fn `UserConstructionScript`)