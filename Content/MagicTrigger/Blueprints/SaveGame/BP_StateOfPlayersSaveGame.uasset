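; A SaveGame Blueprint that stores a snapshot of the player's state for saving and loading.
; It holds life, defence and damage with their maximums, a damage multiplier, the player location, level name and a screenshot.
; SetPlayerState writes all of these fields at once and GetPlayerState returns them together, with no validation or other logic.
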(fn `GetPlayerState`
  (returns (Life :type "Float (double-precision)") (Defence :type "Float (double-precision)") (Damage :type "Float (double-precision)") (MaxLife :type "Float (double-precision)") (MaxDefence :type "Float (double-precision)") (MaxDamage :type "Float (double-precision)") (MultiplierOfDamage :type "Float (double-precision)") (ScreenShot :type "TextureRenderTarget2D Object Reference") (PlayerLocation :type "Vector Structure") (LevelName :type Name))
  (return (`self.Life`) (`self.Defence`) (`self.Damage`) (`self.MaxLife`) (`self.MaxDefence`) (`self.MaxDamage`) (`self.MultiplierOfDamage`) (`self.ScreenShot`) (`self.PlayerLocation`) (`self.LevelName`)))

(fn `SetPlayerState`
  (params (Life :type "Float (double-precision)") (Defence :type "Float (double-precision)") (Damage :type "Float (double-precision)") (MaxLife :type "Float (double-precision)") (MaxDefence :type "Float (double-precision)") (MaxDamage :type "Float (double-precision)") (MultiplierOfDamage :type "Float (double-precision)") (PlayerLocation :type "Vector Structure") (ScreenShot :type "TextureRenderTarget2D Object Reference") (LevelName :type Name))
  (set `self.Life` Life)
  (set `self.Defence` Defence)
  (set `self.Damage` Damage)
  (set `self.MaxLife` MaxLife)
  (set `self.MaxDefence` MaxDefence)
  (set `self.MaxDamage` MaxDamage)
  (set `self.MultiplierOfDamage` MultiplierOfDamage)
  (set `self.PlayerLocation` PlayerLocation)
  (set `self.ScreenShot` ScreenShot)
  (set `self.LevelName` LevelName)
  (return))