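; Legacy enemy Character Blueprint with health, stun, death and player-targeting support.
; Entering the RunAISphere restarts AI logic; leaving does nothing, and the BeginPlay reference-check timer is never started.
; Damage is divided by Defence and freezes movement; death stops AI, sets a lifespan and removes the enemy from player targeting.
; Observation shows a HUD widget and custom-depth outline, interface getters expose enemy data, and Attack and Roaring are simple state flags.
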(event `self.ReceiveBeginPlay`
  ;[0.7247 0.09662 0] EventBeginPlay
)

(event `self.DoBeginPlay_IF`
  ;[0.7247 0.09662 0] EventBeginPlay
)

(event `Attack`
  ;[0.1449 0.6764 0] Attack
  (if (not (`self.bAttack`))
    (set `self.bAttack` true)))

(event `self.BeforeBeginPlay_IF`
  ;[0.7247 0.09662 0] EventBeginPlay
  (bind _bvalid (`self.CheckReferences_IF`))
  (if _bvalid
    (`KismetSystemLibrary.K2_ClearAndInvalidateTimerHandle` (`self.BeginPlayTimer`))
    (`self.DoBeginPlay_IF`)))

(event `StopAttack`
  ;[0.1449 0.6764 0] Attack
  (if (`self.bAttack`)
    (set `self.bAttack` false)))

(event `self.StartBeginPlayTimer_IF`
  ;[0.7247 0.09662 0] EventBeginPlay
  (bind _returnvalue (`KismetSystemLibrary.K2_SetTimerDelegate` (delegate `self.BeforeBeginPlay_IF`) (`self.BeginPlayTimerTime`) true))
  (set `self.BeginPlayTimer` _returnvalue))

(event `self.ReceiveAnyDamage`
  (params (Damage :type "Float (single-precision)") (DamageType :type "DamageType Object Reference") (InstigatedBy :type "Controller Object Reference") (DamageCauser :type "Actor Object Reference"))
  ;[0.06764 0 0.7626] Получение повреждений, DamageInterface
  (`self.GetDamage` true Damage))

(event `TargetSelectionInterface.IsObserved`
  ;[0.2416 0.5797 0] Если под наблюдением перса
  (if (`self.bDying`)
    (message `/Game/MagicTrigger/Blueprints/Interfaces/BPI_OwnerTargetSelection.RemoveAndSwitchActors_IF` (`GameplayStatics.GetPlayerCharacter` 0) self)
    (else
      (`/Engine/EditorBlueprintResources/StandardMacros.IsValid` (`GameplayStatics.GetPlayerController` 0)
        (:`Is Valid`
          (`/Engine/EditorBlueprintResources/StandardMacros.IsValid` (`PlayerController.GetHUD` (`GameplayStatics.GetPlayerController` 0))
            (:`Is Valid`
              (message `/Game/MagicTrigger/Blueprints/Interfaces/BPI_HUD.SetEnemy_IF` (`PlayerController.GetHUD` (`GameplayStatics.GetPlayerController` 0)) self)
              (message `/Game/MagicTrigger/Blueprints/Interfaces/BPI_HUD.ShowObserveEnemyWidget_IF` (`PlayerController.GetHUD` (`GameplayStatics.GetPlayerController` 0)))
              ;;[1 0 0.6562] Отрисовать рамку, если под наблюдением перса
              (`PrimitiveComponent.SetRenderCustomDepth` (`self.Mesh`) true)
              (set `self.bObserved` true))))))))

(event `TargetSelectionInterface.IsNotObserved`
  ;[0.2416 0.5797 0] Если под наблюдением перса
  (`/Engine/EditorBlueprintResources/StandardMacros.IsValid` (`GameplayStatics.GetPlayerController` 0)
    (:`Is Valid`
      (`/Engine/EditorBlueprintResources/StandardMacros.IsValid` (`PlayerController.GetHUD` (`GameplayStatics.GetPlayerController` 0))
        (:`Is Valid`
          (message `/Game/MagicTrigger/Blueprints/Interfaces/BPI_HUD.HideObserveEnemyWidget_IF` (`PlayerController.GetHUD` (`GameplayStatics.GetPlayerController` 0)))
          ;;[0.4928 0.3285 0] Скрыть рамку
          (`PrimitiveComponent.SetRenderCustomDepth` (`self.Mesh`) false)
          (set `self.bObserved` false))))))

(event `Roaring`
  ;[0.4831 0.3382 0] Визуальный сигнал о том, что обнаружен перс --- не используется, см таск на анимацию рычания.
  (set `self.bRoaring` true))

(event `StopRoaring`
  ;[0.4831 0.3382 0] Визуальный сигнал о том, что обнаружен перс --- не используется, см таск на анимацию рычания.
  (set `self.bRoaring` false))

(event `self.RunAISphere.OnComponentBeginOverlap`
  (params (OverlappedComponent :type "PrimitiveComponent Object Reference") (OtherActor :type "Actor Object Reference") (OtherComp :type "PrimitiveComponent Object Reference") (OtherBodyIndex :type Integer) (bFromSweep :type Boolean) (SweepResult :type "HitResult Structure (by ref)"))
  ;[0.09662 0 0.7333] Запустить ИИ, если перс подошел в пределы коллизии
  (bind _ascharacter (cast `Character` OtherActor))
  (if (== _ascharacter (`GameplayStatics.GetPlayerCharacter` 0))
    (`/Engine/EditorBlueprintResources/StandardMacros.IsValid` (`AIBlueprintHelperLibrary.GetAIController` self)
      (:`Is Valid`
        (`BrainComponent.RestartLogic` (`AIController.BrainComponent` (`AIBlueprintHelperLibrary.GetAIController` self)))))))

(event `self.RunAISphere.OnComponentEndOverlap`
  (params (OverlappedComponent :type "PrimitiveComponent Object Reference") (OtherActor :type "Actor Object Reference") (OtherComp :type "PrimitiveComponent Object Reference") (OtherBodyIndex :type Integer))
  ;[0.09662 0 0.7333] Запустить ИИ, если перс подошел в пределы коллизии
)

(fn `CheckReferences_IF`
  (returns (bValid :type Boolean))
  (`/Engine/EditorBlueprintResources/StandardMacros.IsValid` (`AIBlueprintHelperLibrary.GetAIController` self)
    (:`Is Valid`
      (return true))
    (:`Is Not Valid`
      (return false))))

(fn `Die`
  (bind _returnvalue (`GameplayStatics.GetPlayerCharacter` 0))
  (set `self.Life` 0.0)
  (set `self.bDying` true)
  (bind _asaic_enemy_old (cast `/Game/Developers/OLDFiles/AIC_Enemy_OLD` (`self.GetController`)))
  (`BrainComponent.StopLogic` (`AIController.BrainComponent` _asaic_enemy_old) "")
  (`CharacterMovementComponent.DisableMovement` (`self.CharacterMovement`))
  (`self.SetLifeSpan` (`self.Lifespan`))
  (if (`KismetSystemLibrary.DoesImplementInterface` _returnvalue "/Game/MagicTrigger/Blueprints/Interfaces/BPI_OwnerTargetSelection.BPI_OwnerTargetSelection_C")
    (message `/Game/MagicTrigger/Blueprints/Interfaces/BPI_OwnerTargetSelection.RemoveAndSwitchActors_IF` _returnvalue self)
    (return)))

(fn `FindLookPlayer`
  (bind (_returnvalue_roll _returnvalue_pitch) (`KismetMathLibrary.BreakRotator` (`self.K2_GetActorRotation`)))
  (bind (_returnvalue_roll_2 _returnvalue_pitch_2 _returnvalue_yaw) (`KismetMathLibrary.BreakRotator` (`KismetMathLibrary.FindLookAtRotation` (`self.K2_GetActorLocation`) (`self.K2_GetActorLocation` (`GameplayStatics.GetPlayerCharacter` 0)))))
  (`/Engine/EditorBlueprintResources/StandardMacros.IsValid` (`GameplayStatics.GetPlayerCharacter` 0)
    (:`Is Valid`
      (`self.K2_SetActorRotation` (`KismetMathLibrary.MakeRotator` _returnvalue_roll _returnvalue_pitch _returnvalue_yaw))
      (return))
    (:`Is Not Valid`
      (return))))

(fn `GetDamage`
  (params (IsGetDamage :type Boolean) (_Damage :type "Float (double-precision)"))
  (locals (__Damage :type "Float (double-precision)"))
  (bind _returnvalue (- (`self.Life`) (/ (`local.__Damage`) (`self.Defence`))))
  (bind _output_get (set `self.bGetDamage` IsGetDamage))
  (set `local.__Damage` _Damage)
  (if _output_get
    (if (> _returnvalue 0.0)
      (set `self.Life` _returnvalue)
      (if (`|EnumEquality` (`CharacterMovementComponent.MovementMode` (`self.CharacterMovement`)) "MOVE_None")
        (set `self.InitialMovementMode` "MOVE_Walking")
        (else
          (set `self.InitialMovementMode` (`CharacterMovementComponent.MovementMode` (`self.CharacterMovement`)))))
      (`CharacterMovementComponent.DisableMovement` (`self.CharacterMovement`))
      (return)
      (else
        ;[0.02899 0 0.8018] Когда враг умирает
        (`self.Die`)))
    (else
      (`CharacterMovementComponent.SetMovementMode` (`self.CharacterMovement`) (`self.InitialMovementMode`) 0)
      (if (`self.bStunningAfterGetDamage`)
        (`self.Stunning` true)
        (return)))))

(fn `GetDying_IF`
  (returns (bDying :type Boolean))
  (return (`self.bDying`)))

(fn `GetEnemy_IF`
  (returns (Enemy :type "Actor Object Reference"))
  (return self))

(fn `GetIcon_IF`
  (returns (Icon :type "Texture2D Object Reference"))
  (return (`self.Icon`)))

(fn `GetLife_IF`
  (returns (Life :type "Float (double-precision)"))
  (return (`self.Life`)))

(fn `GetMaxLife_IF`
  (returns (MaxLife :type "Float (double-precision)"))
  (return (`self.MaxLife`)))

(fn `GetName_IF`
  (returns (Name :type Text))
  (return (`self.Name`)))

(fn `Stunning`
  (params (_IsStunning :type Boolean))
  (if _IsStunning
    (if (`|EnumEquality` (`CharacterMovementComponent.MovementMode` (`self.CharacterMovement`)) "MOVE_None")
      (set `self.InitialMovementMode` "MOVE_Walking")
      (else
        (set `self.InitialMovementMode` (`CharacterMovementComponent.MovementMode` (`self.CharacterMovement`)))))
    (`CharacterMovementComponent.DisableMovement` (`self.CharacterMovement`))
    (set `self.bStunning` true)
    (else
      (`CharacterMovementComponent.SetMovementMode` (`self.CharacterMovement`) (`self.InitialMovementMode`) 0)
      (set `self.bStunning` false)
      (set `self.bStunningAfterGetDamage` false))))

(fn `UserConstructionScript`
  ;[0.4638 0.3575 0] Радиус сферы, по оверлапу которой включается ИИ
  (`SphereComponent.SetSphereRadius` (`self.RunAISphere`) (`self.RunAISphereRadius`) true))