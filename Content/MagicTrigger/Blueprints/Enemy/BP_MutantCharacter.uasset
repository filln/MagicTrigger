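; Mutant enemy character that passes player tracking, roaring, attack and damage events through to its parent enemy Blueprint.
; Construction script sizes the AI-activation sphere and fills the behavior tree settings struct, without calling the parent's construction script.
; Per-hand start events run looping timers that trace from hand sockets via BPMeleeAttack.
; A hit on a non-BP_Enemy actor clears the timer and applies damage; stop events also clear it.
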(event `self.SetPlayer&EnemyRef`
  (params (PlayerRef :type "Object Object Reference"))
  ;[0 0.5121 0.3092] SetPlayerRef
  (`parent.SetPlayer&EnemyRef` PlayerRef))

(event `self.ReceiveBeginPlay`
  ;[0.7923 0 0.02933] EventBeginPlay
  (`parent.ReceiveBeginPlay`))

(event `self.UnSetPlayer&EnemyRef`
  ;[0 0.5121 0.3092] SetPlayerRef
  (`parent.UnSetPlayer&EnemyRef`))

(event `self.Roaring`
  ;[0.4831 0.3382 0] Roaring
  (`parent.Roaring`))

(event `self.StopRoaring`
  ;[0.4831 0.3382 0] Roaring
  (`parent.StopRoaring`))

(event `self.Attack`
  ;[0.7633 0 0.05866] Attack
  (`parent.Attack`))

(event `self.GetDamage`
  (params (IsGetDamage :type Boolean) (_Damage :type "Float (single-precision)"))
  ;[1 1 1] Damage
  (`parent.GetDamage` IsGetDamage _Damage))

(event `self.StopAttack`
  ;[0.7633 0 0.05866] Attack
  (`parent.StopAttack`))

(event `StartTraceAttackRightHand`
  ;[0 0.2609 0.5604] AttackTracing
  (bind _returnvalue (`KismetSystemLibrary.K2_SetTimer` null "TraceAttackRightHand" 0.02 true))
  (set `/Game/MagicTrigger/Blueprints/AttackAbbilities/BP_MeleeAttackComponent.AttackTimer` _returnvalue (`self.BP_MeleeAttack`)))

(event `StopTraceAttackRightHand`
  ;[0 0.2609 0.5604] AttackTracing
  (`KismetSystemLibrary.K2_ClearAndInvalidateTimerHandle` (`/Game/MagicTrigger/Blueprints/AttackAbbilities/BP_MeleeAttackComponent.AttackTimer` (`self.BP_MeleeAttack`)) :!label _label))

(event `StopTraceAttackLeftHand`
  ;[0 0.2609 0.5604] AttackTracing
  (goto _label))

(event `StartTraceAttackLeftHand`
  ;[0 0.2609 0.5604] AttackTracing
  (bind _returnvalue (`KismetSystemLibrary.K2_SetTimer` null "TraceAttackLeftHand" 0.02 true))
  (set `/Game/MagicTrigger/Blueprints/AttackAbbilities/BP_MeleeAttackComponent.AttackTimer` _returnvalue (`self.BP_MeleeAttack`)))

(fn `TraceAttackLeftHand`
  (bind _traceoutput (`/Game/MagicTrigger/Blueprints/AttackAbbilities/BP_MeleeAttackComponent.TraceAttack` (`self.BP_MeleeAttack`) (`SceneComponent.GetSocketLocation` (`self.Mesh`) "LeftHandSocket1") (`SceneComponent.GetForwardVector` (`self.ArrowLeftHand`)) (`|MakeArray` null :!type "Actor Object Reference")))
  (if (`.ReturnValue_5_E3AFA2314F9AE7F7820C4A92B06AED6A` (break `/Game/MagicTrigger/Data/STraceOutput` _traceoutput))
    (bind (_bblockinghit _binitialoverlap _time _distance _location _impactpoint _normal _impactnormal _physmat _hitactor) (`GameplayStatics.BreakHitResult` (break `/Game/MagicTrigger/Data/STraceOutput` _traceoutput)))
    (castclass `/Game/MagicTrigger/Blueprints/Enemy/BP_Enemy` (`GameplayStatics.GetObjectClass` _hitactor)
      (:`CastFailed`
        (`KismetSystemLibrary.K2_ClearAndInvalidateTimerHandle` (`/Game/MagicTrigger/Blueprints/AttackAbbilities/BP_MeleeAttackComponent.AttackTimer` (`self.BP_MeleeAttack`)))
        (`GameplayStatics.ApplyDamage` _hitactor (`self.Damage`) (`AIBlueprintHelperLibrary.GetAIController` self) self)))))

(fn `TraceAttackRightHand`
  (bind _traceoutput (`/Game/MagicTrigger/Blueprints/AttackAbbilities/BP_MeleeAttackComponent.TraceAttack` (`self.BP_MeleeAttack`) (`SceneComponent.GetSocketLocation` (`self.Mesh`) "RightHandSocket1") (`SceneComponent.GetForwardVector` (`self.ArrowRightHand`)) (`|MakeArray` null :!type "Actor Object Reference")))
  (if (`.ReturnValue_5_E3AFA2314F9AE7F7820C4A92B06AED6A` (break `/Game/MagicTrigger/Data/STraceOutput` _traceoutput))
    (bind (_bblockinghit _binitialoverlap _time _distance _location _impactpoint _normal _impactnormal _physmat _hitactor) (`GameplayStatics.BreakHitResult` (break `/Game/MagicTrigger/Data/STraceOutput` _traceoutput)))
    (castclass `/Game/MagicTrigger/Blueprints/Enemy/BP_Enemy` (`GameplayStatics.GetObjectClass` _hitactor)
      (:`CastFailed`
        (`KismetSystemLibrary.K2_ClearAndInvalidateTimerHandle` (`/Game/MagicTrigger/Blueprints/AttackAbbilities/BP_MeleeAttackComponent.AttackTimer` (`self.BP_MeleeAttack`)))
        (`GameplayStatics.ApplyDamage` _hitactor (`self.Damage`) (`AIBlueprintHelperLibrary.GetAIController` self) self)))))

(fn `UserConstructionScript`
  ;[0.1353 0 0.6942] Радиус сферы, по оверлапу которой включается ИИ
  (`SphereComponent.SetSphereRadius` (`self.RunAISphere`) 4000.0 true)
  (set `self.ToBehaviorTreeStruct` (make `/Game/MagicTrigger/Data/SToBehaviorTree` 1.0 3000.0 600.0 90.0 700.0 5.0 (`self.K2_GetActorLocation`))))