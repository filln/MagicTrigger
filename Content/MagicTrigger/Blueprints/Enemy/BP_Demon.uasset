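; BP_Demon is a boss enemy that registers itself as the boss with the artifact manager and attacks the player with fireballs.
; A looping timer retries reference checks for game mode, AI controller and manager before registering.
; Damage is divided by Defence and triggers death at zero life, without interrupting movement because no hit animation is needed.
; Fireball creation and launch at the player are delegated to BPFireBallComponent.
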(event `self.ReceiveBeginPlay`
  ;[0.6474 0 0.176] EventBeginPlay
  (`parent.ReceiveBeginPlay`)
  (`self.StartBeginPlayTimer_IF`))

(event `self.DoBeginPlay_IF`
  ;[0.6474 0 0.176] EventBeginPlay
  (set `/Game/MagicTrigger/Blueprints/Items/Artifact/BP_ArtifactManager.BossCharacter` self (`self.BP_ArtifactManager`)))

(event `self.BeforeBeginPlay_IF`
  ;[0.6474 0 0.176] EventBeginPlay
  (bind _bvalid (`self.CheckReferences_IF`))
  (if _bvalid
    (`KismetSystemLibrary.K2_ClearAndInvalidateTimerHandle` (`self.BeginPlayTimer`))
    (`self.DoBeginPlay_IF`)))

(event `self.StartBeginPlayTimer_IF`
  ;[0.6474 0 0.176] EventBeginPlay
  (bind _returnvalue (`KismetSystemLibrary.K2_SetTimerDelegate` (delegate `self.BeforeBeginPlay_IF`) (`self.BeginPlayTimerTime`) true))
  (set `self.BeginPlayTimer` _returnvalue))

(event `self.ReceiveActorBeginOverlap`
  (params (OtherActor :type "Actor Object Reference"))
  (`parent.ReceiveActorBeginOverlap` OtherActor))

(event `self.ReceiveTick`
  (params (DeltaSeconds :type "Float (single-precision)"))
  (`parent.ReceiveTick` DeltaSeconds))

(event `self.ReceiveAnyDamage`
  (params (Damage :type "Float (single-precision)") (DamageType :type "DamageType Object Reference") (InstigatedBy :type "Controller Object Reference") (DamageCauser :type "Actor Object Reference"))
  (`self.GetDamage` true Damage))

(event `self.GetDamage`
  (params (IsGetDamage :type Boolean) (_Damage :type "Float (single-precision)"))
  (bind _returnvalue (- (`self.Life`) (/ _Damage (`self.Defence`))))
  ;[0.4445 0.3768 0] Получение повреждений. Не отключая возможность двигаться при получении удара ( т.к. не нужна анимация получения удара, которая в конце включает возможность двигаться)
  (bind _output_get (set `self.bGetDamage` IsGetDamage))
  (if _output_get
    (if (> _returnvalue 0.0)
      (set `self.Life` _returnvalue)
      (else
        (`self.Die`)))))

(event `CreateFireBall`
  ;[1 1 1] FireBall
  (`/Game/MagicTrigger/Blueprints/AttackAbilities/BP_FireBallComponent.CreateFireBall` (`self.BP_FireBallComponent`) (`self.Mesh`)))

(event `MoveFireBallToTarget`
  ;[1 1 1] FireBall
  (`/Game/MagicTrigger/Blueprints/AttackAbilities/BP_FireBallComponent.MoveFireBallToTarget` (`self.BP_FireBallComponent`) (`AIBlueprintHelperLibrary.GetAIController` self) (`GameplayStatics.GetPlayerCharacter` 0)))

(fn `CheckReferences_IF`
  (returns (bValid :type Boolean))
  (`/Engine/EditorBlueprintResources/StandardMacros.IsValid` (`GameplayStatics.GetGameMode`)
    (:`Is Valid`
      (`/Engine/EditorBlueprintResources/StandardMacros.IsValid` (`AIBlueprintHelperLibrary.GetAIController` self)
        (:`Is Valid`
          (bind _bp_artifactmanager (message `/Game/MagicTrigger/Blueprints/Interfaces/BPI_GameMode.GetArtifactManager_IF` (`GameplayStatics.GetGameMode`)))
          (set `self.BP_ArtifactManager` _bp_artifactmanager)
          (`/Engine/EditorBlueprintResources/StandardMacros.IsValid` (`self.BP_ArtifactManager`)
            (:`Is Valid`
              (return true))
            (:`Is Not Valid`
              (return false))))
        (:`Is Not Valid`
          (return false))))
    (:`Is Not Valid`
      (return false))))

(fn `UserConstructionScript`
  (`parent.UserConstructionScript`))