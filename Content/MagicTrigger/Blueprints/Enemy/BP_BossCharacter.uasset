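; Boss enemy character that extends a parent enemy class, inheriting its boss-ball attack and damage transfer.
; On BeginPlay it retries until the ArtifactManager is valid, then registers itself there.
; GetDamage scales damage by multiplier over defence without interrupting movement; at zero life it stops AI logic and movement, then sets a lifespan.
; Construction fills boss-ball and behavior tree settings; overlapping thrown rocks are set to ignore Pawns.
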(event `self.ReceiveActorBeginOverlap`
  (params (OtherActor :type "Actor Object Reference"))
  (`parent.ReceiveActorBeginOverlap` OtherActor))

(event `self.ReceiveBeginPlay`
  ;[0.6474 0 0.176] EventBeginPlay
  (`parent.ReceiveBeginPlay`)
  (bind _referenceaggregator (`/Game/MagicTrigger/Blueprints/FunctionLibraries/BPFL_ReferenceAggregator.GetReferenceAggregator`))
  (bind _artifactmanager (`/Game/MagicTrigger/Blueprints/CoreClasses/BP_ReferenceAggregator.artifactManager` _referenceaggregator))
  (`/Engine/EditorBlueprintResources/StandardMacros.IsValid` _artifactmanager :!label _label
    (:`Is Valid`
      (set `/Game/MagicTrigger/Blueprints/Items/Artifact/BP_ArtifactManager.BossCharacter` self _artifactmanager))
    (:`Is Not Valid`
      (`KismetSystemLibrary.Delay` 0.5)
      (goto _label))))

(event `self.ReceiveTick`
  (params (DeltaSeconds :type "Float (single-precision)"))
  (`parent.ReceiveTick` DeltaSeconds))

(event `self.CreateBossBall`
  (`parent.CreateBossBall`))

(event `self.MoveBossBallToTarget`
  (`parent.MoveBossBallToTarget`))

(event `self.CapsuleComponent.OnComponentBeginOverlap`
  (params (OverlappedComponent :type "PrimitiveComponent Object Reference") (OtherActor :type "Actor Object Reference") (OtherComp :type "PrimitiveComponent Object Reference") (OtherBodyIndex :type Integer) (bFromSweep :type Boolean) (SweepResult :type "HitResult Structure (by ref)"))
  ;[0.2222 0 0.6062] Реакция врага на брошенный персом камень
  (bind _asbp_throwable_rock (cast `/Game/MagicTrigger/Blueprints/Items/LiftingObjects/BP_ThrowableRock` OtherActor))
  (`PrimitiveComponent.SetCollisionResponseToChannel` (`/Game/MagicTrigger/Blueprints/Items/LiftingObjects/BP_LiftingObject.Box` _asbp_throwable_rock) "ECC_Pawn" "ECR_Ignore"))

(event `/Game/MagicTrigger/Blueprints/Interfaces/BPI_Damage.TransferDamage`
  (params (_Damage :type "Float (single-precision)") (_MultiplierOfDamage :type "Float (single-precision)"))
  (`parent.TransferDamage` _Damage _MultiplierOfDamage))

(event `self.GetDamage`
  (params (IsGetDamage :type Boolean) (_Damage :type "Float (single-precision)") (_MultiplierOfDamage :type "Float (single-precision)"))
  (bind _returnvalue (- (`self.Life`) (/ (* _Damage _MultiplierOfDamage) (`self.Defence`))))
  ;[0.4445 0.3768 0] Получение повреждений. Не отключая возможность двигаться при получении удара ( т.к. не нужна анимация получения удара, которая в конце включает возможность двигаться)
  (bind _output_get (set `self.isGetDamage` IsGetDamage))
  (if _output_get
    (if (> _returnvalue 0.0)
      (set `self.Life` _returnvalue)
      (else
        (set `self.Life` 0.0)
        (set `self.isDying` true)
        (bind _asaic_enemy (cast `/Game/MagicTrigger/AI/Enemy/AIC_Enemy` (`self.GetController`)))
        (`BrainComponent.StopLogic` (`AIController.BrainComponent` _asaic_enemy) "")
        (`CharacterMovementComponent.DisableMovement` (`self.CharacterMovement`))
        (`self.SetLifeSpan` 5.0)))))

(fn `UserConstructionScript`
  (`parent.UserConstructionScript`)
  (set `self.BossBallStruct` (make `/Game/MagicTrigger/Data/SBossBall` null self 1.175952 2.5 1000.0 0.25 (`self.Damage`) 1.0 "BossBallSocket" 2.0 0.2))
  (set `self.ToBehaviorTreeStruct` (make `/Game/MagicTrigger/Data/SToBehaviorTree` 2.8 3000.0 2500.0 1500.0 2000.0 5.0 (`self.K2_GetActorLocation`))))