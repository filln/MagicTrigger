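; Player controller that applies the mouse sensitivity setting to look input.
; On BeginPlay it caches the initial yaw, pitch and roll input scales, then reads the saved sensitivity from the game instance through an interface message.
; SetInputRotationScale, also exposed as an interface event, computes base × multiplier + addend, scales the cached values by it and sends the result back to the game instance settings.
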(event `self.ReceiveBeginPlay`
  ;[0 0.009662 0.8116] Запомнить начальные значения множителей вращения
  (set `self.InitialInputYawScale` (`self.InputYawScale`))
  (set `self.InitialInputPitchScale` (`self.InputPitchScale`))
  (set `self.InitialInputRollScale` (`self.InputRollScale`))
  ;[0 0.08696 0.7343] Прочитать и задать значение чувствительности мыши
  (bind _gamesettings (message `/Game/MagicTrigger/Blueprints/Interfaces/BPI_GameInstance.GetGameSettingsStruct_IF` (`GameplayStatics.GetGameInstance`)))
  (`self.SetInputRotationScale` (break `/Game/MagicTrigger/Data/SGameSettings` _gamesettings) 1.0))

(event `/Game/MagicTrigger/Blueprints/Interfaces/BPI_PlayerController.SetInputRotationScale_IF`
  (params (mouseSensBaseValue :type "Float (single-precision)") (mouseSensMultiplier :type "Float (single-precision)") (mouseSensAddend :type "Float (single-precision)"))
  (`self.SetInputRotationScale` mouseSensBaseValue mouseSensMultiplier mouseSensAddend))

(fn `SetInputRotationScale`
  (params (_mouseSensBaseValue :type "Float (double-precision)") (_mouseSensMultiplier :type "Float (double-precision)") (_mouseSensAddend :type "Float (double-precision)"))
  (locals (mouseSens :type "Float (double-precision)" :default 0.0))
  (set `local.mouseSens` (+ (* _mouseSensBaseValue _mouseSensMultiplier) _mouseSensAddend))
  (set `self.InputPitchScale` (* (`self.InitialInputPitchScale`) (`local.mouseSens`)))
  (set `self.InputRollScale` (* (`self.InitialInputRollScale`) (`local.mouseSens`)))
  (set `self.InputYawScale` (* (`self.InitialInputYawScale`) (`local.mouseSens`)))
  (`/Engine/EditorBlueprintResources/StandardMacros.IsValid` (`GameplayStatics.GetGameInstance`)
    (:`Is Valid`
      (message `/Game/MagicTrigger/Blueprints/Interfaces/BPI_GameInstance.SetGameSettingsStruct` (`GameplayStatics.GetGameInstance`) (make `/Game/MagicTrigger/Data/SGameSettings` (`local.mouseSens`)))
      (return))
    (:`Is Not Valid`
      (return))))

(fn `UserConstructionScript`)