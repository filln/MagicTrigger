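; BP_PlayerState stores a player's combat stats: life, defence, damage, their maximums and a damage multiplier.
; Interface getters and setters expose each stat individually, while GetPlayerState and SetPlayerState pack or unpack them all as one struct.
; It also keeps a separate begin-game state struct, set and read through the interface.
; It is a pure data holder, with no clamping or gameplay logic.
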(event `self.ReceiveBeginPlay`)

(event `/Game/MagicTrigger/Blueprints/Interfaces/BPI_PlayerState.SetBeginGamePlayerState_IF`
  (params (SPlayerState :type "/Game/MagicTrigger/Data/SPlayerState Structure"))
  (set `self.BeginGamePlayerState` SPlayerState))

(event `/Game/MagicTrigger/Blueprints/Interfaces/BPI_PlayerState.SetMultiplierOfDamage_IF`
  (params (MultiplierOfDamage :type "Float (single-precision)"))
  (set `self.MultiplierOfDamage` MultiplierOfDamage))

(event `/Game/MagicTrigger/Blueprints/Interfaces/BPI_PlayerState.SetMaxDamage_IF`
  (params (MaxDamage :type "Float (single-precision)"))
  (set `self.MaxDamage` MaxDamage))

(event `/Game/MagicTrigger/Blueprints/Interfaces/BPI_PlayerState.SetMaxDefence_IF`
  (params (MaxDefence :type "Float (single-precision)"))
  (set `self.MaxDefence` MaxDefence))

(event `/Game/MagicTrigger/Blueprints/Interfaces/BPI_PlayerState.SetDamage_IF`
  (params (Damage :type "Float (single-precision)"))
  (set `self.Damage` Damage))

(event `/Game/MagicTrigger/Blueprints/Interfaces/BPI_PlayerState.SetDefence_IF`
  (params (Defence :type "Float (single-precision)"))
  (set `self.Defence` Defence))

(event `/Game/MagicTrigger/Blueprints/Interfaces/BPI_PlayerState.SetMaxLife_IF`
  (params (MaxLife :type "Float (single-precision)"))
  (set `self.MaxLife` MaxLife))

(event `/Game/MagicTrigger/Blueprints/Interfaces/BPI_PlayerState.SetLife_IF`
  (params (Life :type "Float (single-precision)"))
  (set `self.Life` Life))

(event `/Game/MagicTrigger/Blueprints/Interfaces/BPI_PlayerState.SetPlayerState_IF`
  (params (States :type "/Game/MagicTrigger/Data/SPlayerState Structure"))
  (`self.SetPlayerState` States))

(fn `GetBeginGamePlayerState_IF`
  (returns (SPlayerState :type "/Game/MagicTrigger/Data/SPlayerState Structure"))
  (return (`self.BeginGamePlayerState`)))

(fn `GetDamage_IF`
  (returns (Damage :type "Float (double-precision)"))
  (return (`self.Damage`)))

(fn `GetDefence_IF`
  (returns (Defence :type "Float (double-precision)"))
  (return (`self.Defence`)))

(fn `GetLife_IF`
  (returns (Life :type "Float (double-precision)"))
  (return (`self.Life`)))

(fn `GetMaxDamage_IF`
  (returns (MaxDamage :type "Float (double-precision)"))
  (return (`self.MaxDamage`)))

(fn `GetMaxDefence_IF`
  (returns (MaxDefence :type "Float (double-precision)"))
  (return (`self.MaxDefence`)))

(fn `GetMaxLife_IF`
  (returns (MaxLife :type "Float (double-precision)"))
  (return (`self.MaxLife`)))

(fn `GetMultiplierOfDamage_IF`
  (returns (MultiplierOfDamage :type "Float (double-precision)"))
  (return (`self.MultiplierOfDamage`)))

(fn `GetPlayerState`
  (returns (States :type "/Game/MagicTrigger/Data/SPlayerState Structure"))
  (return (make `/Game/MagicTrigger/Data/SPlayerState` (`self.Life`) (`self.Defence`) (`self.Damage`) (`self.MaxLife`) (`self.MaxDefence`) (`self.MaxDamage`) (`self.MultiplierOfDamage`))))

(fn `GetPlayerState_IF`
  (returns (States :type "/Game/MagicTrigger/Data/SPlayerState Structure"))
  (return (`self.GetPlayerState`)))

(fn `SetPlayerState`
  (params (States :type "/Game/MagicTrigger/Data/SPlayerState Structure"))
  (set `self.Life` States_Life_2_503268C04DB2F14DD8DBBCB0E45FEAA6)
  (set `self.Defence` States_Defence_4_2035395F4AF0F7242619CD8F7593F3EA)
  (set `self.Damage` States_Damage_6_FC699E3F4D548881F36102BC9D1DAE46)
  (set `self.MaxLife` States_MaxLife_8_D4CC596944AFCB3CED80649AC7BCD1F4)
  (set `self.MaxDefence` States_MaxDefence_10_B29570E646DCDD0E21191CAE66834B08)
  (set `self.MaxDamage` States_MaxDamage_12_1AA334A94A02E7BF3EA34FBCCFD277D1)
  (set `self.MultiplierOfDamage` States_MultiplierOfDamage_14_CE8D4E064906F220F1F0D7B0CD3EE257)
  (return))

(fn `UserConstructionScript`)