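; BP_LifeStatue is an interactable angel statue that refills the player's life while they stand still, with a custom-depth highlight when observed.
; BeginPlay polls until the player's animation manager and PlayerState are valid.
; Interact blocks further interaction and raises the spotlight, then a timeline scaled for a constant heal rate restores life through interface calls while dimming the point light.
; Movement or completion reverses the lights, then re-enables interaction.
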(event `TargetSelectionInterface.IsObserved`
  ;[0.5701 0 0.2542] Нарисовать рамку, если под наблюдением перса
  (`PrimitiveComponent.SetRenderCustomDepth` (`self.SM_Plains_Angel_Statue_01`) true))

(event `TargetSelectionInterface.IsNotObserved`
  ;[0.5701 0 0.2542] Нарисовать рамку, если под наблюдением перса
  (`PrimitiveComponent.SetRenderCustomDepth` (`self.SM_Plains_Angel_Statue_01`) false))

(event `self.ReceiveBeginPlay`
  (bind _playerstate (`Pawn.PlayerState` (`GameplayStatics.GetPlayerCharacter` 0)))
  ;[0.6281 0 0.1955] EventBeginPlay
  (bind _animationmanagercomponent (message `/Game/MagicTrigger/Blueprints/Interfaces/BPI_AnimationManager.GetAnimationManagerComponent_IF` (`GameplayStatics.GetPlayerCharacter` 0)))
  (`/Engine/EditorBlueprintResources/StandardMacros.IsValid` _animationmanagercomponent :!label _label
    (:`Is Valid`
      (set `self.BP_AnimationManagerComponent` _animationmanagercomponent)
      (`/Engine/EditorBlueprintResources/StandardMacros.IsValid` _playerstate :!label _label_2
        (:`Is Valid`
          (set `self.PlayerState` _playerstate)
          (`LightComponent.SetIntensity` (`self.SpotLight`) 0.0)
          (`LightComponent.SetIntensity` (`self.PointLight`) (`self.MaxIntensityPointLight`)))
        (:`Is Not Valid`
          (`KismetSystemLibrary.Delay` 0.2)
          (goto _label_2))))
    (:`Is Not Valid`
      (`KismetSystemLibrary.Delay` 0.2)
      (goto _label))))

(event `/Game/MagicTrigger/Blueprints/Interfaces/BPI_Interaction.Interact`
  ;[0.686 0 0.1369] Начать пополнять здоровье
  (set `self.InitialLocationCharacter` (`self.K2_GetActorLocation` (`GameplayStatics.GetPlayerCharacter` 0)))
  (message `/Game/MagicTrigger/Blueprints/Interfaces/BPI_AnimationManager.SetCanInteract` (`self.BP_AnimationManagerComponent`) false)
  (bind (_direction _alpha) (`Timeline|Timeline_0` :!via `PlayFromStart`)
    (:`Update`
      (`LightComponent.SetIntensity` (`self.SpotLight`) (`KismetMathLibrary.Lerp` 0.0 (`self.MaxIntensitySpotLight`) _alpha)))
    (:`Finished`
      (`self.AddLife`))))

(event `ReversIntensityLight`
  ;[0.1449 0 0.6844] Возврат интенсивности света ламп
  (set `self.CurrentIntensityPointLight` (`LightComponentBase.Intensity` (`self.PointLight`)))
  (bind (_direction _alpha) (`Timeline|Timeline_3` :!via `ReverseFromEnd`)
    (:`Update`
      (`LightComponent.SetIntensity` (`self.SpotLight`) (`KismetMathLibrary.Lerp` 0.0 (`self.MaxIntensitySpotLight`) _alpha))
      (`LightComponent.SetIntensity` (`self.PointLight`) (`KismetMathLibrary.Lerp` (`self.MaxIntensityPointLight`) (`self.CurrentIntensityPointLight`) _alpha)))
    (:`Finished`
      (message `/Game/MagicTrigger/Blueprints/Interfaces/BPI_AnimationManager.SetCanInteract` (`self.BP_AnimationManagerComponent`) true))))

(event `AddLife`
  ;[0.6087 0 0.2151] Пополнить здоровье, если перс не двигается и здоровья меньше максимального
  (if (< (`self.GetLife`) (`self.GetMaxLife`))
    (set `self.CurrentLife` (`self.GetLife`))
    (`TimelineComponent.SetPlayRate` (`self.Timeline_2`) (/ 1.0 (/ (- (`self.GetMaxLife`) (`self.CurrentLife`)) 10.0)))
    (bind (_direction _life _pointlight) (`Timeline|Timeline_2` :!via `PlayFromStart` :!label _label_3)
      (:`Update`
        (if (== (`self.K2_GetActorLocation` (`GameplayStatics.GetPlayerCharacter` 0)) (`self.InitialLocationCharacter`) :`ErrorTolerance` 0.1)
          (message `/Game/MagicTrigger/Blueprints/Interfaces/BPI_PlayerState.SetLife_IF` (`self.PlayerState`) (`KismetMathLibrary.Lerp` (`self.CurrentLife`) (`self.GetMaxLife`) _life))
          (`LightComponent.SetIntensity` (`self.PointLight`) (`KismetMathLibrary.Lerp` (`self.MaxIntensityPointLight`) 0.0 _pointlight))
          (else
            (`self.StopTimeline_2`)
            (`self.ReversIntensityLight`))))
      (:`Finished`
        (`self.ReversIntensityLight`)))
    (else
      (`self.ReversIntensityLight`))))

(event `StopTimeline_2`
  ;[0.6087 0 0.2151] Пополнить здоровье, если перс не двигается и здоровья меньше максимального
  (goto _label_3 :!via `Stop`))

(fn `GetInteractionText`
  (returns (InteractionText :type Text))
  (return (`self.InteractionText`)))

(fn `GetLife`
  (returns (Life :type "Float (double-precision)"))
  (bind _life (message `/Game/MagicTrigger/Blueprints/Interfaces/BPI_PlayerState.GetLife_IF` (`self.PlayerState`)))
  (return _life))

(fn `GetMaxLife`
  (returns (MaxLife :type "Float (double-precision)"))
  (bind _maxlife (message `/Game/MagicTrigger/Blueprints/Interfaces/BPI_PlayerState.GetMaxLife_IF` (`self.PlayerState`)))
  (return _maxlife))

(fn `UserConstructionScript`)