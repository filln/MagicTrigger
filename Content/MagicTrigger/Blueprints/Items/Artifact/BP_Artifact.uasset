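; Artifact actor with a green emissive material that animates its spawn, activation and deactivation as one of several artifact copies.
; On spawn it pulses scale and glow up and back down.
; Activation moves it to the last copy's location while brightening, then scales it, flashes and destroys it; deactivation does the same without glow changes.
; Timings come from the passed ArtifactManagerStruct, with timeline play rates set to 1/duration.
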(event `self.ReceiveBeginPlay`
  (`parent.ReceiveBeginPlay`)
  (set `self.EffectsOnSpawArtifact` (make `/Game/MagicTrigger/Data/SEffectsOnSpawArtifact` 0.2 1.8 80.0))
  (`self.EffectsOnSpawn`))

(event `self.ReceiveActorBeginOverlap`
  (params (OtherActor :type "Actor Object Reference"))
  (`parent.ReceiveActorBeginOverlap` OtherActor))

(event `self.ReceiveTick`
  (params (DeltaSeconds :type "Float (single-precision)"))
  (`parent.ReceiveTick` DeltaSeconds))

(event `ActivateArtifact`
  (params (_ArtifactManagerStruct :type "/Game/MagicTrigger/Data/SArtifactManager Structure"))
  ;[0 0.02899 0.7923] Активировать Артефакт
  ;;[0 0.1353 0.686] Начать активацию Артефакта
  (set `self.ArtifactManagerStruct` _ArtifactManagerStruct)
  (`self.MoveAndEmissive`))

(event `DeactivateArtifact`
  (params (_ArtifactManagerStruct :type "/Game/MagicTrigger/Data/SArtifactManager Structure"))
  ;[0 0.3672 0.4541] Деактивировать Артефакт
  ;;[0.3382 0 0.4889] Начать деактивацию Артефакта
  (set `self.ArtifactManagerStruct` _ArtifactManagerStruct)
  (`self.Move`))

(event `MoveAndEmissive`
  (bind (_artifactmanagerstruct_maxemissive _artifactmanagerstruct_multiplierofmaxemissive _artifactmanagerstruct_timeofmove _artifactmanagerstruct_timeofscale _artifactmanagerstruct_multiplierofscale _artifactmanagerstruct_timeofscalelastcopy _artifactmanagerstruct_multiplierofscalelastcopy _artifactmanagerstruct_timeofmovepedestalsspheres _artifactmanagerstruct_locationlastcopy) (break `/Game/MagicTrigger/Data/SArtifactManager` (`self.ArtifactManagerStruct`)))
  (bind (_artifactmanagerstruct_maxemissive_2 _artifactmanagerstruct_multiplierofmaxemissive_2) (break `/Game/MagicTrigger/Data/SArtifactManager` (`self.ArtifactManagerStruct`)))
  (bind (_artifactmanagerstruct_maxemissive_3 _artifactmanagerstruct_multiplierofmaxemissive_3 _artifactmanagerstruct_timeofmove_2 _artifactmanagerstruct_timeofscale_2 _artifactmanagerstruct_multiplierofscale_2) (break `/Game/MagicTrigger/Data/SArtifactManager` (`self.ArtifactManagerStruct`)))
  ;[0 0.02899 0.7923] Активировать Артефакт
  ;;[0.3285 0 0.4987] Двигаться к последней копии и светиться с возрастающей интенсивностью
  (set `self.InitialLocation` (`self.K2_GetActorLocation`))
  (`TimelineComponent.SetPlayRate` (`self.Timeline_Move&Emissive`) (/ 1.0 _artifactmanagerstruct_timeofmove))
  (bind (_direction _emissive) (`Timeline|Timeline_Move&Emissive` :!via `PlayFromStart`)
    (:`Update`
      (`MaterialInstanceDynamic.SetScalarParameterValue` (`self.MaterialInst`) "EmissiveMultiplier" (`KismetMathLibrary.Lerp` 0.0 _artifactmanagerstruct_maxemissive _emissive))
      (`self.K2_SetActorLocation` (`KismetMathLibrary.VLerp` (`self.InitialLocation`) _artifactmanagerstruct_locationlastcopy _emissive)))
    (:`Finished`
      (`self.Scale` _artifactmanagerstruct_timeofscale_2 _artifactmanagerstruct_multiplierofscale_2)
      (`KismetSystemLibrary.Delay` _artifactmanagerstruct_timeofscale_2)
      (`self.MultiplyEmissiveAndDestroy` _artifactmanagerstruct_maxemissive_2 _artifactmanagerstruct_multiplierofmaxemissive_2))))

(event `Move`
  (bind (_artifactmanagerstruct_maxemissive _artifactmanagerstruct_multiplierofmaxemissive _artifactmanagerstruct_timeofmove _artifactmanagerstruct_timeofscale _artifactmanagerstruct_multiplierofscale _artifactmanagerstruct_timeofscalelastcopy _artifactmanagerstruct_multiplierofscalelastcopy _artifactmanagerstruct_timeofmovepedestalsspheres _artifactmanagerstruct_locationlastcopy) (break `/Game/MagicTrigger/Data/SArtifactManager` (`self.ArtifactManagerStruct`)))
  ;[0 0.3672 0.4541] Деактивировать Артефакт
  ;;[0 0.3962 0.4251] Двигаться к последней копии
  (set `self.InitialLocation` (`self.K2_GetActorLocation`))
  (`TimelineComponent.SetPlayRate` (`self.Timeline_Move`) (/ 1.0 _artifactmanagerstruct_timeofmove))
  (bind (_direction _emissive) (`Timeline|Timeline_Move` :!via `PlayFromStart`)
    (:`Update`
      (`self.K2_SetActorLocation` (`KismetMathLibrary.VLerp` (`self.InitialLocation`) _artifactmanagerstruct_locationlastcopy _emissive)))
    (:`Finished`
      (`self.ScaleAndDestroy`))))

(event `MultiplyEmissiveAndDestroy`
  (params (_MaxEmissive :type "Float (double-precision)") (_MultiplierOfMaxEmissive :type "Float (double-precision)"))
  ;[0 0.02899 0.7923] Активировать Артефакт
  ;;[0 0.7247 0.09662] Увеличить свечение и удалиться
  (`MaterialInstanceDynamic.SetScalarParameterValue` (`self.MaterialInst`) "EmissiveMultiplier" (* _MaxEmissive _MultiplierOfMaxEmissive))
  (`KismetSystemLibrary.Delay` 0.1)
  (`self.K2_DestroyActor`))

(event `ScaleAndDestroy`
  (bind (_artifactmanagerstruct_maxemissive _artifactmanagerstruct_multiplierofmaxemissive _artifactmanagerstruct_timeofmove _artifactmanagerstruct_timeofscale _artifactmanagerstruct_multiplierofscale) (break `/Game/MagicTrigger/Data/SArtifactManager` (`self.ArtifactManagerStruct`)))
  ;[0 0.3672 0.4541] Деактивировать Артефакт
  ;;[0.657 0 0.1662] Увеличиться и удалиться
  (`self.Scale` _artifactmanagerstruct_timeofscale _artifactmanagerstruct_multiplierofscale)
  (`KismetSystemLibrary.Delay` _artifactmanagerstruct_timeofscale)
  (`self.K2_DestroyActor`))

(event `Scale`
  (params (_TimeOfScale :type "Float (double-precision)") (_MultiplierOfScale :type "Float (double-precision)"))
  (bind _initialscalebox (`self.InitialScaleBox`))
  (bind _initialscalemesh (`self.InitialScaleMesh`))
  ;[0.3768 0 0.4498] Увеличиться
  (set `self.InitialScaleBox` (`SceneComponent.K2_GetComponentScale` (`self.Box`)))
  (set `self.InitialScaleMesh` (`SceneComponent.K2_GetComponentScale` (`self.StaticMesh`)))
  (`TimelineComponent.SetPlayRate` (`self.Timeline_Scale`) (/ 1.0 _TimeOfScale))
  (bind (_direction _scale) (`Timeline|Timeline_Scale` :!via `PlayFromStart`)
    (:`Update`
      (`SceneComponent.SetWorldScale3D` (`self.Box`) (`KismetMathLibrary.VLerp` _initialscalebox (* _initialscalebox _MultiplierOfScale) _scale))
      (`SceneComponent.SetWorldScale3D` (`self.StaticMesh`) (`KismetMathLibrary.VLerp` _initialscalemesh (* _initialscalemesh _MultiplierOfScale) _scale)))))

(event `EffectsOnSpawn`
  (bind (_effectsonspawartifact_timeofscale _effectsonspawartifact_multiplierofscale _effectsonspawartifact_multiplierofemissive) (break `/Game/MagicTrigger/Data/SEffectsOnSpawArtifact` (`self.EffectsOnSpawArtifact`)))
  (bind (_effectsonspawartifact_timeofscale_2 _effectsonspawartifact_multiplierofscale_2) (break `/Game/MagicTrigger/Data/SEffectsOnSpawArtifact` (`self.EffectsOnSpawArtifact`)))
  (bind (_effectsonspawartifact_timeofscale_3 _effectsonspawartifact_multiplierofscale_3 _effectsonspawartifact_multiplierofemissive_2) (break `/Game/MagicTrigger/Data/SEffectsOnSpawArtifact` (`self.EffectsOnSpawArtifact`)))
  ;[0.8116 0 0.009777] Эффекты при спавне копии артефакта
  (`self.Scale` _effectsonspawartifact_timeofscale _effectsonspawartifact_multiplierofscale)
  (`self.Emissive` _effectsonspawartifact_timeofscale 1.0 _effectsonspawartifact_multiplierofemissive)
  (`KismetSystemLibrary.Delay` _effectsonspawartifact_timeofscale_2)
  (`self.Scale` _effectsonspawartifact_timeofscale_2 (/ 1.0 _effectsonspawartifact_multiplierofscale_2))
  (`self.Emissive` _effectsonspawartifact_timeofscale_3 _effectsonspawartifact_multiplierofemissive_2 1.0))

(event `Emissive`
  (params (_TimeOfEmissive :type "Float (double-precision)") (_MinMultiplierOfEmissive :type "Float (double-precision)") (_MaxMultiplierOfEmissive :type "Float (double-precision)"))
  ;[0.4155 0.4058 0] Изменить свечение
  (`TimelineComponent.SetPlayRate` (`self.Timeline_Emissive`) (/ 1.0 _TimeOfEmissive))
  (bind (_direction _emissive) (`Timeline|Timeline_Emissive` :!via `PlayFromStart`)
    (:`Update`
      (`MaterialInstanceDynamic.SetScalarParameterValue` (`self.MaterialInst`) "EmissiveMultiplier" (`KismetMathLibrary.Lerp` _MinMultiplierOfEmissive _MaxMultiplierOfEmissive _emissive)))))

(fn `UserConstructionScript`
  (bind _returnvalue (`PrimitiveComponent.CreateDynamicMaterialInstance` (`self.StaticMesh`) 0 "/Game/MagicTrigger/Materials/M_Ability.M_Ability" "None"))
  (bind _output_get (set `self.MaterialInst` _returnvalue))
  (`MaterialInstanceDynamic.SetTextureParameterValue` _output_get "Texture" "/Game/MagicTrigger/Textures/T_Artifact_D.T_Artifact_D")
  (`MaterialInstanceDynamic.SetVectorParameterValue` (`self.MaterialInst`) "EmissiveColor" (struct :`G` 1.0 :`B` 0.381713 :`A` 1.0))
  (`MaterialInstanceDynamic.SetScalarParameterValue` (`self.MaterialInst`) "EmissiveMultiplier" 1.0))