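; Manager for the artifact pedestal puzzle: spawns numbered artifact copies at the player's throwing hand, linking each to any free pedestal it overlaps.
; Once the copy limit is reached, CastArtifactAbility activates or deactivates copies and pedestals by matching cast order to pedestal sphere count.
; If all match, the last copy scales up after timed delays, damaging an overlapped boss and revealing the end-game text.
; Either outcome then spawns a fresh artifact.
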(event `self.ReceiveBeginPlay`
  ;[0.2319 0.5894 0] EventBeginPlay
  (`|ExecutionSequence`
    (:`then_0`
      (bind _referenceaggregator (`/Game/MagicTrigger/Blueprints/FunctionLibraries/BPFL_ReferenceAggregator.GetReferenceAggregator`))
      (set `/Game/MagicTrigger/Blueprints/CoreClasses/BP_ReferenceAggregator.artifactManager` self _referenceaggregator)
      (set `self.referenceAggregator` _referenceaggregator)
      (set `self.KachujinCharacterRef` (`/Game/MagicTrigger/Blueprints/CoreClasses/BP_ReferenceAggregator.PlayerCharacter` (`self.referenceAggregator`))))
    (:`then_1`
      (set `self.ArtifactManagerStruct` (make `/Game/MagicTrigger/Data/SArtifactManager` 1000.0 5.0 3.0 1.0 1.5 3.0 25.0 1.0)))))

(event `CastArtifactAbility`
  (bind (_artifactmanagerstruct_maxemissive _artifactmanagerstruct_multiplierofmaxemissive _artifactmanagerstruct_timeofmove _artifactmanagerstruct_timeofscale _artifactmanagerstruct_multiplierofscale _artifactmanagerstruct_timeofscalelastcopy _artifactmanagerstruct_multiplierofscalelastcopy _artifactmanagerstruct_timeofmovepedestalsspheres) (break `/Game/MagicTrigger/Data/SArtifactManager` (`self.ArtifactManagerStruct`)))
  (bind _arrartifactref (`self.ArrArtifactRef`))
  ;[0.4638 0.3575 0] Скастовать абилку артефакта и проверить на правило расстановки
  (if (== (`KismetArrayLibrary.Array_Length` (`self.ArrArtifactRef`)) (`self.MaxLengthArrArtifactRef`))
    (bind _output_get (set `self.LastCopyOfArtifact` (`|GetArrayItem` _arrartifactref (`KismetArrayLibrary.Array_LastIndex` _arrartifactref))))
    (set `self.ArtifactManagerStruct` (make `/Game/MagicTrigger/Data/SArtifactManager` _artifactmanagerstruct_maxemissive _artifactmanagerstruct_multiplierofmaxemissive _artifactmanagerstruct_timeofmove _artifactmanagerstruct_timeofscale _artifactmanagerstruct_multiplierofscale _artifactmanagerstruct_timeofscalelastcopy _artifactmanagerstruct_multiplierofscalelastcopy _artifactmanagerstruct_timeofmovepedestalsspheres (`self.K2_GetActorLocation` _output_get)))
    (bind __isrightplacing_ (`self.CheckSumOfRightPlacings` (`self.ArrArtifactRef`)))
    (set `self.IsRightPlacings?` __isrightplacing_)
    (`self.EnableArtifact`)))

(event `EnableArtifact`
  ;[0.3189 0.5024 0] Включить Артефакт
  (for _index (range (+ (- (`KismetArrayLibrary.Array_Length` (`self.ArrArtifactRef`)) 2) 1))
    (bind _output (`|GetArrayItem` (`self.ArrArtifactRef`) _index))
    (`/Engine/EditorBlueprintResources/StandardMacros.IsValid` (`/Game/MagicTrigger/Blueprints/Items/Artifact/BP_Artifact.BP_CharacterPedestal_Quest2` _output)
      (:`Is Valid`
        (if (`/Game/MagicTrigger/Blueprints/Items/Artifact/BP_Artifact.IsRightPlacing?` _output)
          (`/Game/MagicTrigger/Blueprints/Items/Artifact/BP_Artifact.ActivateArtifact` _output (`self.ArtifactManagerStruct`))
          (`/Game/MagicTrigger/Blueprints/Items/Quest2/BP_CharacterPedestal_Quest2Parent.ActivatePedestal` (`/Game/MagicTrigger/Blueprints/Items/Artifact/BP_Artifact.BP_CharacterPedestal_Quest2` _output))
          (else
            (`/Game/MagicTrigger/Blueprints/Items/Artifact/BP_Artifact.DeactivateArtifact` _output (`self.ArtifactManagerStruct`))
            (`/Game/MagicTrigger/Blueprints/Items/Quest2/BP_CharacterPedestal_Quest2Parent.DisablePedestal` (`/Game/MagicTrigger/Blueprints/Items/Artifact/BP_Artifact.BP_CharacterPedestal_Quest2` _output)))))
      (:`Is Not Valid`
        (`/Game/MagicTrigger/Blueprints/Items/Artifact/BP_Artifact.DeactivateArtifact` _output (`self.ArtifactManagerStruct`)))))
  (if (`self.IsRightPlacings?`)
    (`self.ActivateLastCopy`)
    (else
      (`self.DeactivateLactCopy`))))

(event `ActivateLastCopy`
  (bind _lastcopyofartifact (`self.LastCopyOfArtifact`))
  (bind (_artifactmanagerstruct_maxemissive _artifactmanagerstruct_multiplierofmaxemissive _artifactmanagerstruct_timeofmove _artifactmanagerstruct_timeofscale) (break `/Game/MagicTrigger/Data/SArtifactManager` (`self.ArtifactManagerStruct`)))
  (bind (_artifactmanagerstruct_maxemissive_2 _artifactmanagerstruct_multiplierofmaxemissive_2 _artifactmanagerstruct_timeofmove_2 _artifactmanagerstruct_timeofscale_2 _artifactmanagerstruct_multiplierofscale _artifactmanagerstruct_timeofscalelastcopy _artifactmanagerstruct_multiplierofscalelastcopy) (break `/Game/MagicTrigger/Data/SArtifactManager` (`self.ArtifactManagerStruct`)))
  ;[0.8116 0.009662 0] Активировать последнюю копию артефакта
  (set `self.RotationForNewArtifact` (`self.K2_GetActorRotation` _lastcopyofartifact))
  (set `self.ScaleForNewArtefact` (`self.GetActorScale3D` _lastcopyofartifact))
  (`/Game/MagicTrigger/Blueprints/Items/Quest2/BP_CharacterPedestal_Quest2Parent.ActivatePedestal` (`/Game/MagicTrigger/Blueprints/Items/Artifact/BP_Artifact.BP_CharacterPedestal_Quest2` (`self.LastCopyOfArtifact`)))
  (`KismetSystemLibrary.Delay` (+ _artifactmanagerstruct_timeofmove _artifactmanagerstruct_timeofscale))
  (`MaterialInstanceDynamic.SetScalarParameterValue` (`/Game/MagicTrigger/Blueprints/Items/Artifact/BP_Artifact.MaterialInst` (`self.LastCopyOfArtifact`)) "EmissiveMultiplier" _artifactmanagerstruct_maxemissive)
  (`/Game/MagicTrigger/Blueprints/Items/Artifact/BP_Artifact.Scale` (`self.LastCopyOfArtifact`) _artifactmanagerstruct_timeofscalelastcopy _artifactmanagerstruct_multiplierofscalelastcopy)
  (`KismetSystemLibrary.Delay` _artifactmanagerstruct_timeofscalelastcopy)
  (`|ExecutionSequence`
    (:`then_0`
      (`self.DoDamage`))
    (:`then_1`
      (`/Game/MagicTrigger/Blueprints/Items/Artifact/BP_Artifact.MultiplyEmissiveAndDestroy` (`self.LastCopyOfArtifact`) _artifactmanagerstruct_maxemissive_2 _artifactmanagerstruct_multiplierofmaxemissive_2)
      (set `self.LastCopyOfArtifact` null)
      (`self.SpawnNewArtifact`))))

(event `DeactivateLactCopy`
  (bind _lastcopyofartifact (`self.LastCopyOfArtifact`))
  (bind _lastcopyofartifact_2 (`self.LastCopyOfArtifact`))
  (bind (_artifactmanagerstruct_maxemissive _artifactmanagerstruct_multiplierofmaxemissive _artifactmanagerstruct_timeofmove _artifactmanagerstruct_timeofscale _artifactmanagerstruct_multiplierofscale) (break `/Game/MagicTrigger/Data/SArtifactManager` (`self.ArtifactManagerStruct`)))
  ;[0 0.09662 0.7247] Деактивировать последнюю копию Артефакта
  (set `self.RotationForNewArtifact` (`self.K2_GetActorRotation` _lastcopyofartifact))
  (set `self.ScaleForNewArtefact` (`self.GetActorScale3D` _lastcopyofartifact))
  (`/Engine/EditorBlueprintResources/StandardMacros.IsValid` (`/Game/MagicTrigger/Blueprints/Items/Artifact/BP_Artifact.BP_CharacterPedestal_Quest2` _lastcopyofartifact_2)
    (:`Is Valid`
      (if (`/Game/MagicTrigger/Blueprints/Items/Artifact/BP_Artifact.IsRightPlacing?` _lastcopyofartifact_2)
        (`/Game/MagicTrigger/Blueprints/Items/Quest2/BP_CharacterPedestal_Quest2Parent.ActivatePedestal` (`/Game/MagicTrigger/Blueprints/Items/Artifact/BP_Artifact.BP_CharacterPedestal_Quest2` (`self.LastCopyOfArtifact`)))
        (else
          (`/Game/MagicTrigger/Blueprints/Items/Quest2/BP_CharacterPedestal_Quest2Parent.DisablePedestal` (`/Game/MagicTrigger/Blueprints/Items/Artifact/BP_Artifact.BP_CharacterPedestal_Quest2` (`self.LastCopyOfArtifact`))))))
    (:`Is Not Valid`
      _))
  (`KismetSystemLibrary.Delay` (+ _artifactmanagerstruct_timeofmove _artifactmanagerstruct_timeofscale))
  (`/Game/MagicTrigger/Blueprints/Items/Artifact/BP_Artifact.Scale` (`self.LastCopyOfArtifact`) _artifactmanagerstruct_timeofscale _artifactmanagerstruct_multiplierofscale)
  (`KismetSystemLibrary.Delay` _artifactmanagerstruct_timeofscale)
  (`self.K2_DestroyActor` (`self.LastCopyOfArtifact`))
  (set `self.LastCopyOfArtifact` null)
  (`self.SpawnNewArtifact`))

(event `DoDamage`
  ;[0.03865 0.7827 0] Атаковать врага
  (`PrimitiveComponent.SetCollisionResponseToChannel` (`/Game/MagicTrigger/Blueprints/Items/LiftingObjects/BP_LiftingObject.Box` (`self.LastCopyOfArtifact`)) "ECC_Pawn" "ECR_Overlap")
  (`/Engine/EditorBlueprintResources/StandardMacros.IsValid` (`self.BossCharacter`)
    (:`Is Valid`
      (if (`self.IsOverlappingActor` (`self.LastCopyOfArtifact`) (`self.BossCharacter`))
        (message `/Game/MagicTrigger/Blueprints/Interfaces/BPI_Damage.TransferDamage` (`self.BossCharacter`) 0.0 (`self.MultiplierOfDamage`))
        (`self.EndGame`)))))

(event `SpawnNewArtifact`
  ;[0 0.4155 0.4058] Создать новый артефакт
  (`KismetArrayLibrary.Array_Clear` (`self.ArrArtifactRef`))
  (`|SpawnActorFromClass` "/Game/MagicTrigger/Blueprints/Items/Artifact/BP_Artifact.BP_Artifact_C" (`KismetMathLibrary.MakeTransform` (`self.LocationForArtifact`) (`self.RotationForNewArtifact`) (`self.ScaleForNewArtefact`)) "Undefined" "OverrideRootScale" null null))

(event `EndGame`
  ;[0 0.2319 0.5894] End Game, показать заключительную надпись
  (`SceneComponent.SetHiddenInGame` (`/Game/MagicTrigger/Blueprints/Environment/BP_Castle.TextRender` (`self.Castle`)) false true))

(fn `CheckOnRightPlacing`
  (set `/Game/MagicTrigger/Blueprints/Items/Artifact/BP_Artifact.IsRightPlacing?` (== (`/Game/MagicTrigger/Blueprints/Items/Quest2/BP_CharacterPedestal_Quest2Parent.CountOfSpheres` (`/Game/MagicTrigger/Blueprints/Items/Artifact/BP_Artifact.BP_CharacterPedestal_Quest2` (`self.CurrentArtifactRef`))) (`/Game/MagicTrigger/Blueprints/Items/Artifact/BP_Artifact.Number` (`self.CurrentArtifactRef`))) (`self.CurrentArtifactRef`))
  (return))

(fn `CheckSumOfRightPlacings`
  (params (_ArrArtifactRef :type "Array of /Game/MagicTrigger/Blueprints/Items/Artifact/BP_Artifact Object Reference"))
  (returns (`_IsRightPlacing?` :type Boolean))
  (locals (SumOfRightPlacing :type Integer))
  (for _array_element _ArrArtifactRef
    (bind _bp_characterpedestal_quest2 (`/Game/MagicTrigger/Blueprints/Items/Artifact/BP_Artifact.BP_CharacterPedestal_Quest2` _array_element))
    (`/Engine/EditorBlueprintResources/StandardMacros.IsValid` _bp_characterpedestal_quest2
      (:`Is Valid`
        (if (== (`/Game/MagicTrigger/Blueprints/Items/Quest2/BP_CharacterPedestal_Quest2Parent.CountOfSpheres` _bp_characterpedestal_quest2) (`/Game/MagicTrigger/Blueprints/Items/Artifact/BP_Artifact.Number` _array_element))
          (`/Engine/EditorBlueprintResources/StandardMacros.IncrementInt` (`local.SumOfRightPlacing`))
          (else
            (break))))
      (:`Is Not Valid`
        (break))))
  (return (== (`KismetArrayLibrary.Array_Length` _ArrArtifactRef) (`local.SumOfRightPlacing`))))

(fn `EnablePedestal`
  (bind _currentartifactref (`self.CurrentArtifactRef`))
  (bind _overlappingactors (`self.GetOverlappingActors` (`self.CurrentArtifactRef`) "/Game/MagicTrigger/Blueprints/Items/Quest2/BP_CharacterPedestal_Quest2Parent.BP_CharacterPedestal_Quest2Parent_C"))
  (`/Engine/EditorBlueprintResources/StandardMacros.IsValid` (`self.CurrentArtifactRef`)
    (:`Is Valid`
      (if (> (`KismetArrayLibrary.Array_Length` _overlappingactors) 0)
        (bind _asbp_character_pedestal_quest_2parent (cast `/Game/MagicTrigger/Blueprints/Items/Quest2/BP_CharacterPedestal_Quest2Parent` (`|GetArrayItem` _overlappingactors))
          (:`then`
            (set `/Game/MagicTrigger/Blueprints/Items/Artifact/BP_Artifact.BP_CharacterPedestal_Quest2` _asbp_character_pedestal_quest_2parent _currentartifactref)
            (if (`/Game/MagicTrigger/Blueprints/Items/Quest2/BP_CharacterPedestal_Quest2Parent.isEnable?` (`/Game/MagicTrigger/Blueprints/Items/Artifact/BP_Artifact.BP_CharacterPedestal_Quest2` (`self.CurrentArtifactRef`)))
              (set `/Game/MagicTrigger/Blueprints/Items/Artifact/BP_Artifact.BP_CharacterPedestal_Quest2` null (`self.CurrentArtifactRef`))
              (return)
              (else
                (`/Game/MagicTrigger/Blueprints/Items/Quest2/BP_CharacterPedestal_Quest2Parent.EnablePedestal` (`/Game/MagicTrigger/Blueprints/Items/Artifact/BP_Artifact.BP_CharacterPedestal_Quest2` (`self.CurrentArtifactRef`)) (`self.K2_GetActorLocation` _currentartifactref))
                (`self.CheckOnRightPlacing`)
                (return))))
          (:`CastFailed`
            (return)))
        (else
          (return))))
    (:`Is Not Valid`
      (return))))

(fn `SpawnCopiesOfArtifact`
  (params (_ArtifactRef :type "/Game/MagicTrigger/Blueprints/Items/Artifact/BP_Artifact Object Reference"))
  (bind _kachujincharacterref (`self.KachujinCharacterRef`))
  (bind _kachujincharacterref_2 (`self.KachujinCharacterRef`))
  (bind (_returnvalue_location _returnvalue_rotation) (`KismetMathLibrary.BreakTransform` (`SceneComponent.GetSocketTransform` (`Character.Mesh` _kachujincharacterref_2) (`/Game/MagicTrigger/Blueprints/PlayerCharacter/BP_PlayerCharacter.ThrowableRightHand` _kachujincharacterref_2) "RTS_World")))
  (bind _returnvalue (`|SpawnActorFromClass` (`GameplayStatics.GetObjectClass` _ArtifactRef) (`KismetMathLibrary.MakeTransform` _returnvalue_location _returnvalue_rotation (`self.GetActorScale3D` _ArtifactRef)) "Undefined" "OverrideRootScale" null null))
  (bind _output_get (set `self.CurrentArtifactRef` _returnvalue))
  (bind _box (`/Game/MagicTrigger/Blueprints/Items/LiftingObjects/BP_LiftingObject.Box` _output_get))
  (`PrimitiveComponent.SetCollisionResponseToChannel` _box "ECC_Pawn" "ECR_Ignore")
  (`PrimitiveComponent.SetCollisionResponseToChannel` _box "ECC_GameTraceChannel6" "ECR_Ignore")
  (bind _returnvalue_2 (`KismetArrayLibrary.Array_Add` (`self.ArrArtifactRef`) (`self.CurrentArtifactRef`)))
  ;[0.3285 0.4928 0] Назначить порядковый номер копии в порядке их кастования
  (set `/Game/MagicTrigger/Blueprints/Items/Artifact/BP_Artifact.Number` (+ _returnvalue_2 1) (`self.CurrentArtifactRef`))
  (`self.EnablePedestal`)
  ;[0 0.02899 0.7923] Удалить Артефакт из руки перса, если скастовано макс. кол. копий Артефакта
  (if (not (< (`KismetArrayLibrary.Array_Length` (`self.ArrArtifactRef`)) (`self.MaxLengthArrArtifactRef`)))
    (`self.K2_DestroyActor` (`/Game/MagicTrigger/Blueprints/PlayerCharacter/BP_PlayerCharacter.LiftUpObject` _kachujincharacterref))
    (set `/Game/MagicTrigger/Blueprints/PlayerCharacter/BP_PlayerCharacter.LiftUpObject` null _kachujincharacterref))
  (return))

(fn `StartActivationPedestal`)

(fn `UserConstructionScript`)