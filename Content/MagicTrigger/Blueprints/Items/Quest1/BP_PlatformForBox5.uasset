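; Quest 1 platform that takes a box stone and serves as the trigger for shifting the large rock door in the cliff.
; On BeginPlay it registers itself with Quest1Manager through the reference aggregator, retrying every half second until the manager is valid.
; When a BP_BoxForPlatform_Parent actor overlaps Box1, it calls Platform5BeginOverlapBox with that actor; the rock movement itself is handled outside this Blueprint.
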(event `self.ReceiveActorBeginOverlap`
  (params (OtherActor :type "Actor Object Reference"))
  (`parent.ReceiveActorBeginOverlap` OtherActor))

(event `self.ReceiveTick`
  (params (DeltaSeconds :type "Float (single-precision)"))
  (`parent.ReceiveTick` DeltaSeconds))

(event `self.ReceiveBeginPlay`
  ;[0 0.6667 0.1546] EventBeginPlay. Платформа для сдвига скалы (большого камня в скале, двери).
  (`parent.ReceiveBeginPlay`)
  (bind _referenceaggregator (`/Game/MagicTrigger/Blueprints/FunctionLibraries/BPFL_ReferenceAggregator.GetReferenceAggregator`))
  (bind _quest1manager (`/Game/MagicTrigger/Blueprints/CoreClasses/BP_ReferenceAggregator.quest1Manager` _referenceaggregator))
  (`/Engine/EditorBlueprintResources/StandardMacros.IsValid` _quest1manager :!label _label
    (:`Is Valid`
      (set `/Game/MagicTrigger/Blueprints/Items/Quest1/BP_Quest1Manager.PlatformForBox5Ref` self _quest1manager))
    (:`Is Not Valid`
      (`KismetSystemLibrary.Delay` 0.5)
      (goto _label))))

(event `self.Box1.OnComponentBeginOverlap`
  (params (OverlappedComponent :type "PrimitiveComponent Object Reference") (OtherActor :type "Actor Object Reference") (OtherComp :type "PrimitiveComponent Object Reference") (OtherBodyIndex :type Integer) (bFromSweep :type Boolean) (SweepResult :type "HitResult Structure (by ref)"))
  ;[0 0.09662 0.7247] Если правильный камень ляжет на платформу для сдвига скалы
  (cast `/Game/MagicTrigger/Blueprints/Items/Quest1/BP_BoxForPlatform_Parent` OtherActor)
  (`self.Platform5BeginOverlapBox` OtherActor))

(fn `UserConstructionScript`
  (`parent.UserConstructionScript`))