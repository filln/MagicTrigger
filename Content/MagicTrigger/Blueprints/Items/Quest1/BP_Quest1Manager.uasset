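; Manager for Quest 1: a box-placement puzzle that unlocks a lift carrying the player between lower and upper levels.
; A looping timer waits for references, then binds lift and platform dispatchers and sorts platforms by Up/Down tags.
; Stepping on the lift compares box and platform tags for that level, moving the lift on success or resetting boxes on failure.
; Separately, the correct box on platform 5 slides the big wall open.
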(event `self.DoBeginPlay_IF`
  ;[0 0.802 0.01932] EventBeginPlay
  (`self.AssignDispatchers_IF`)
  (set `self.KachujinCharacterRef` (cast `/Game/MagicTrigger/Blueprints/PlayerCharacter/BP_PlayerCharacter` (`GameplayStatics.GetPlayerCharacter` 0) :!pure true))
  (for _array_element (`self.PlatformsForBox`)
    (if (`self.ActorHasTag` _array_element "Down")
      (`KismetArrayLibrary.Array_Add` (`self.PlatformsDown`) _array_element)
      (elif (`self.ActorHasTag` _array_element "Up")
        (`KismetArrayLibrary.Array_Add` (`self.PlatformsUp`) _array_element)))))

(event `self.ReceiveBeginPlay`
  ;[0 0.802 0.01932] EventBeginPlay
  (`self.StartBeginPlayTimer_IF`))

(event `self.BeforeBeginPlay_IF`
  ;[0 0.802 0.01932] EventBeginPlay
  (`/Engine/EditorBlueprintResources/StandardMacros.IsValid` (`GameplayStatics.GetGameMode`)
    (:`Is Valid`
      (message `/Game/MagicTrigger/Blueprints/Interfaces/BPI_GameMode.SetQuest1Manager_IF` (`GameplayStatics.GetGameMode`) self)
      (bind _bvalid (`self.CheckReferences_IF`))
      (if _bvalid
        (`KismetSystemLibrary.K2_ClearAndInvalidateTimerHandle` (`self.BeginPlayTimer`))
        (`self.DoBeginPlay_IF`)))))

(event `self.StartBeginPlayTimer_IF`
  ;[0 0.802 0.01932] EventBeginPlay
  (bind _returnvalue (`KismetSystemLibrary.K2_SetTimerDelegate` (delegate `self.BeforeBeginPlay_IF`) (`self.BeginPlayTimerTime`) true))
  (set `self.BeginPlayTimer` _returnvalue))

(event `PlatformBeginOverlapCharacter_Event_0`
  (params (OtherComp :type "PrimitiveComponent Object Reference") (CurrentPlatform :type "/Game/MagicTrigger/Blueprints/Items/Quest1/BP_PlatformForBox_Parent Object Reference"))
  ;[0 0.802 0.01932] EventBeginPlay
  (`self.PlatformBeginOverlapCharacter` OtherComp CurrentPlatform))

(event `PlatformEndOverlapCharacter_Event_0`
  (params (OtherComp :type "PrimitiveComponent Object Reference") (CurentPlatform :type "/Game/MagicTrigger/Blueprints/Items/Quest1/BP_PlatformForBox_Parent Object Reference"))
  ;[0 0.802 0.01932] EventBeginPlay
  (`self.PlatformEndOverlapCharacter` OtherComp CurentPlatform))

(event `self.AssignDispatchers_IF`
  ;[0 0.802 0.01932] EventBeginPlay
  (add `/Game/MagicTrigger/Blueprints/Items/Quest1/BP_Lift.BeginOverlapCharacter` (`self.LiftRef`) (delegate `BeginOverlapCharacter_Event_0`))
  (add `/Game/MagicTrigger/Blueprints/Items/Quest1/BP_Lift.EndOverlapCharacter` (`self.LiftRef`) (delegate `EndOverlapCharacter_Event_0`))
  (add `/Game/MagicTrigger/Blueprints/Items/Quest1/BP_PlatformForBox5.Platform5BeginOverlapBox` (`self.PlatformForBox5Ref`) (delegate `Platform5BeginOverlapBox_Event_0`))
  (for _array_element (`self.PlatformsForBox`)
    (add `/Game/MagicTrigger/Blueprints/Items/Quest1/BP_PlatformForBox_Parent.PlatformBeginOverlapCharacter` _array_element (delegate `PlatformBeginOverlapCharacter_Event_0`))
    (add `/Game/MagicTrigger/Blueprints/Items/Quest1/BP_PlatformForBox_Parent.PlatformEndOverlapCharacter` _array_element (delegate `PlatformEndOverlapCharacter_Event_0`))))

(event `BeginOverlapCharacter_Event_0`
  (params (OtherComp :type "PrimitiveComponent Object Reference"))
  ;[0 0.802 0.01932] EventBeginPlay
  (`self.LiftBeginOverlapCharacter` OtherComp))

(event `EndOverlapCharacter_Event_0`
  (params (OtherComp :type "PrimitiveComponent Object Reference"))
  ;[0 0.802 0.01932] EventBeginPlay
  (`self.LiftEndOverlapCharacter` OtherComp))

(event `Platform5BeginOverlapBox_Event_0`
  (params (OtherActor :type "Actor Object Reference"))
  ;[0 0.802 0.01932] EventBeginPlay
  (`self.Platform5BeginOverlapBox` OtherActor))

(event `LiftBeginOverlapCharacter`
  (params (OtherComp :type "PrimitiveComponent Object Reference"))
  ;[0.3768 0 0.4498] Когда перс заходит или сходит с лифта
  (if (and (== OtherComp (`Character.CapsuleComponent` (`self.KachujinCharacterRef`))) (not (`/Game/MagicTrigger/Blueprints/Items/Quest1/BP_Lift.IsOffOverlapCharacter?` (`self.LiftRef`))))
    (`self.BeginOverlapMoveDown`)
    (`KismetSystemLibrary.Delay` 1.0)
    (`self.CheckKey`)))

(event `LiftEndOverlapCharacter`
  (params (OtherComp :type "PrimitiveComponent Object Reference"))
  ;[0.3768 0 0.4498] Когда перс заходит или сходит с лифта
  (if (and (== OtherComp (`Character.CapsuleComponent` (`self.KachujinCharacterRef`))) (not (`/Game/MagicTrigger/Blueprints/Items/Quest1/BP_Lift.IsOffOverlapCharacter?` (`self.LiftRef`))))
    (`self.EndOverlapMoveUp`)))

(event `PlatformBeginOverlapCharacter`
  (params (OtherComp :type "PrimitiveComponent Object Reference") (CurrentPlatform :type "/Game/MagicTrigger/Blueprints/Items/Quest1/BP_PlatformForBox_Parent Object Reference"))
  (bind _kachujincharacterref (`self.KachujinCharacterRef`))
  ;[0.1739 0 0.6551] Если перс подойдет к платформе, то отдать ему ссылку на платформу. Если отойдет - обнулить.
  (`/Engine/EditorBlueprintResources/StandardMacros.IsValid` _kachujincharacterref
    (:`Is Valid`
      (if (== (`/Game/MagicTrigger/Blueprints/PlayerCharacter/BP_PlayerCharacter.InteractCollision` _kachujincharacterref) OtherComp)
        (set `/Game/MagicTrigger/Blueprints/PlayerCharacter/BP_PlayerCharacter.PlatformForBoxRef` CurrentPlatform (`self.KachujinCharacterRef`))))))

(event `BeginOverlapMoveDown`
  ;[0.3768 0 0.4498] Когда перс заходит или сходит с лифта
  (if (`/Game/MagicTrigger/Blueprints/Items/Quest1/BP_Lift.isLiftDown?` (`self.LiftRef`))
    (set `/Game/MagicTrigger/Blueprints/Items/Quest1/BP_Lift.CurrentLocation` (`/Game/MagicTrigger/Blueprints/Items/Quest1/BP_Lift.InitLocation` (`self.LiftRef`)) (`self.LiftRef`))
    (else
      (set `/Game/MagicTrigger/Blueprints/Items/Quest1/BP_Lift.CurrentLocation` (`/Game/MagicTrigger/Blueprints/Items/Quest1/BP_Lift.UpLocation` (`self.LiftRef`)) (`self.LiftRef`))))
  (`KismetSystemLibrary.MoveComponentTo` (`Actor.RootComponent` (`self.LiftRef`)) (`KismetMathLibrary.MakeVector` (.x (`/Game/MagicTrigger/Blueprints/Items/Quest1/BP_Lift.CurrentLocation` (`self.LiftRef`))) (.y (`/Game/MagicTrigger/Blueprints/Items/Quest1/BP_Lift.CurrentLocation` (`self.LiftRef`))) (- (.z (`/Game/MagicTrigger/Blueprints/Items/Quest1/BP_Lift.CurrentLocation` (`self.LiftRef`))) (* (.z (`.BoxExtent` (`KismetSystemLibrary.GetComponentBounds` (`/Game/MagicTrigger/Blueprints/Items/Quest1/BP_Lift.StaticMesh` (`self.LiftRef`))))) 2.0))) (`self.K2_GetActorRotation` (`self.LiftRef`)) true true 1.0))

(event `PlatformEndOverlapCharacter`
  (params (OtherComp :type "PrimitiveComponent Object Reference") (CurrentPlatform :type "/Game/MagicTrigger/Blueprints/Items/Quest1/BP_PlatformForBox_Parent Object Reference"))
  (bind _kachujincharacterref (`self.KachujinCharacterRef`))
  ;[0.1739 0 0.6551] Если перс подойдет к платформе, то отдать ему ссылку на платформу. Если отойдет - обнулить.
  (`/Engine/EditorBlueprintResources/StandardMacros.IsValid` _kachujincharacterref
    (:`Is Valid`
      (if (== (`/Game/MagicTrigger/Blueprints/PlayerCharacter/BP_PlayerCharacter.InteractCollision` _kachujincharacterref) OtherComp)
        (set `/Game/MagicTrigger/Blueprints/PlayerCharacter/BP_PlayerCharacter.PlatformForBoxRef` null (`self.KachujinCharacterRef`))))))

(event `EndOverlapMoveUp`
  ;[0.3768 0 0.4498] Когда перс заходит или сходит с лифта
  (if (`/Game/MagicTrigger/Blueprints/Items/Quest1/BP_Lift.isLiftDown?` (`self.LiftRef`))
    (set `/Game/MagicTrigger/Blueprints/Items/Quest1/BP_Lift.CurrentLocation` (`/Game/MagicTrigger/Blueprints/Items/Quest1/BP_Lift.InitLocation` (`self.LiftRef`)) (`self.LiftRef`))
    (else
      (set `/Game/MagicTrigger/Blueprints/Items/Quest1/BP_Lift.CurrentLocation` (`/Game/MagicTrigger/Blueprints/Items/Quest1/BP_Lift.UpLocation` (`self.LiftRef`)) (`self.LiftRef`))))
  (`KismetSystemLibrary.MoveComponentTo` (`Actor.RootComponent` (`self.LiftRef`)) (`/Game/MagicTrigger/Blueprints/Items/Quest1/BP_Lift.CurrentLocation` (`self.LiftRef`)) (`self.K2_GetActorRotation` (`self.LiftRef`)) true true 1.0))

(event `Platform5BeginOverlapBox`
  (params (OtherActor :type "Actor Object Reference"))
  ;[0.2222 0.5991 0] Если правильный камень ляжет на платформу для сдвига скалы
  (cast `/Game/MagicTrigger/Blueprints/Items/Quest1/BP_BoxForPlatform3And5` OtherActor)
  (`KismetSystemLibrary.Delay` 1.0)
  (`self.MoveBigWall`))

(event `MoveBigWall`
  (bind (_initiallocationdoor_x _initiallocationdoor_y _initiallocationdoor_z) (`KismetMathLibrary.BreakVector` (`/Game/MagicTrigger/Blueprints/Items/Quest1/BP_BigWall.InitialLocationDoor` (`self.BigWallRef`))))
  ;[0.2222 0.5991 0] Если правильный камень ляжет на платформу для сдвига скалы
  (`KismetSystemLibrary.PrintString` "OpenBigWall")
  (`KismetSystemLibrary.MoveComponentTo` (`/Game/MagicTrigger/Blueprints/Items/Quest1/BP_BigWall.DoorSphere` (`self.BigWallRef`)) (`KismetMathLibrary.MakeVector` _initiallocationdoor_x (+ _initiallocationdoor_y 70.0) _initiallocationdoor_z) (`SceneComponent.K2_GetComponentRotation` (`/Game/MagicTrigger/Blueprints/Items/Quest1/BP_BigWall.DoorSphere` (`self.BigWallRef`))) true true 5.0))

(event `CheckKey`
  ;[0 0.1159 0.7054] Проверить расстановку камней на платформах
  (if (`/Game/MagicTrigger/Blueprints/Items/Quest1/BP_Lift.isLiftDown?` (`self.LiftRef`))
    (bind _islockopen (`self.CheckSumOfRightPlacings` (`self.PlatformsDown`)))
    (if _islockopen
      (`self.LockIsOpen` :!label _label)
      (else
        (`self.LockIsClosed` :!label _label_2)))
    (else
      (bind _islockopen_2 (`self.CheckSumOfRightPlacings` (`self.PlatformsUp`)))
      (if _islockopen_2
        (goto _label)
        (else
          (goto _label_2))))))

(event `LockIsClosed`
  (`KismetSystemLibrary.PrintString` "Closed")
  ;[0.2222 0.5991 0] Если ключ неправильный, переместить все боксы на платформах к начальному положению
  (for _array_element (`self.PlatformsForBox`)
    (bind _currentboxref (`/Game/MagicTrigger/Blueprints/Items/Quest1/BP_PlatformForBox_Parent.CurrentBoxRef` _array_element))
    (`/Engine/EditorBlueprintResources/StandardMacros.IsValid` _currentboxref
      (:`Is Valid`
        (`/Game/MagicTrigger/Blueprints/Items/Quest1/BP_BoxForPlatform_Parent.MoveBoxToInitLocation` _currentboxref)))))

(event `LockIsOpen`
  ;[0.02899 0.7923 0] Когда ключ найден, можно двигать лифт
  (`KismetSystemLibrary.PrintString` "Open")
  (if (`/Game/MagicTrigger/Blueprints/Items/Quest1/BP_Lift.isLiftDown?` (`self.LiftRef`))
    (`self.MoveUp`)
    (else
      (`self.MoveDown`))))

(event `MoveUp`
  (bind (_returnvalue_roll _returnvalue_pitch _returnvalue_yaw) (`KismetMathLibrary.BreakRotator` (`self.K2_GetActorRotation`)))
  (bind _liftref (`self.LiftRef`))
  ;[0.02899 0.7923 0] Когда ключ найден, можно двигать лифт
  (`self.IsCharacterOnLift?` true)
  (`KismetSystemLibrary.MoveComponentTo` (`Actor.RootComponent` (`GameplayStatics.GetPlayerCharacter` 0)) (`SceneComponent.K2_GetComponentLocation` (`/Game/MagicTrigger/Blueprints/Items/Quest1/BP_Lift.Scene` (`self.LiftRef`))) (`self.K2_GetActorRotation` (`GameplayStatics.GetPlayerCharacter` 0)) true true 0.2 true)
  (`self.K2_AttachToComponent` (`GameplayStatics.GetPlayerCharacter` 0) (`/Game/MagicTrigger/Blueprints/Items/Quest1/BP_Lift.Scene` (`self.LiftRef`)) "None" "SnapToTarget" "KeepWorld" "KeepWorld" true)
  (`KismetSystemLibrary.MoveComponentTo` (`Actor.RootComponent` (`self.LiftRef`)) (`/Game/MagicTrigger/Blueprints/Items/Quest1/BP_Lift.UpLocation` (`self.LiftRef`)) (`KismetMathLibrary.MakeRotator` _returnvalue_roll _returnvalue_pitch (+ _returnvalue_yaw 180.0)) true true 4.0)
  (set `/Game/MagicTrigger/Blueprints/Items/Quest1/BP_Lift.IsLockOpen?` false _liftref)
  (set `/Game/MagicTrigger/Blueprints/Items/Quest1/BP_Lift.isLiftDown?` false _liftref)
  (`self.IsCharacterOnLift?` false)
  (`self.BeginOverlapMoveDown`))

(event `MoveDown`
  (bind (_returnvalue_roll _returnvalue_pitch _returnvalue_yaw) (`KismetMathLibrary.BreakRotator` (`self.K2_GetActorRotation`)))
  (bind _liftref (`self.LiftRef`))
  ;[0.02899 0.7923 0] Когда ключ найден, можно двигать лифт
  (`self.IsCharacterOnLift?` true)
  (`KismetSystemLibrary.MoveComponentTo` (`Actor.RootComponent` (`GameplayStatics.GetPlayerCharacter` 0)) (`SceneComponent.K2_GetComponentLocation` (`/Game/MagicTrigger/Blueprints/Items/Quest1/BP_Lift.Scene` (`self.LiftRef`))) (`self.K2_GetActorRotation` (`GameplayStatics.GetPlayerCharacter` 0)) true true)
  (`self.K2_AttachToComponent` (`GameplayStatics.GetPlayerCharacter` 0) (`/Game/MagicTrigger/Blueprints/Items/Quest1/BP_Lift.Scene` (`self.LiftRef`)) "None" "SnapToTarget" "KeepWorld" "KeepWorld" true)
  (`KismetSystemLibrary.MoveComponentTo` (`Actor.RootComponent` (`self.LiftRef`)) (`/Game/MagicTrigger/Blueprints/Items/Quest1/BP_Lift.InitLocation` (`self.LiftRef`)) (`KismetMathLibrary.MakeRotator` _returnvalue_roll _returnvalue_pitch (+ _returnvalue_yaw 180.0)) true true 4.0)
  (set `/Game/MagicTrigger/Blueprints/Items/Quest1/BP_Lift.IsLockOpen?` false _liftref)
  (set `/Game/MagicTrigger/Blueprints/Items/Quest1/BP_Lift.isLiftDown?` true _liftref)
  (`self.IsCharacterOnLift?` false)
  (`self.BeginOverlapMoveDown`))

(fn `CheckReferences_IF`
  (returns (bValid :type Boolean))
  (if (and (`KismetSystemLibrary.IsValid` (`GameplayStatics.GetPlayerCharacter` 0)) (`KismetSystemLibrary.IsValid` (`self.PlatformForBox5Ref`)) (`KismetSystemLibrary.IsValid` (`self.LiftRef`)))
    (cast `/Game/MagicTrigger/Blueprints/PlayerCharacter/BP_PlayerCharacter` (`GameplayStatics.GetPlayerCharacter` 0)
      (:`then`
        (if (< (`KismetArrayLibrary.Array_Length` (`self.PlatformsForBox`)) (`self.CountOfPlatforms`))
          (return false)
          (else
            (return true))))
      (:`CastFailed`
        (return false)))
    (else
      (return false))))

(fn `CheckSumOfRightPlacings`
  (params (_Array :type "Array of /Game/MagicTrigger/Blueprints/Items/Quest1/BP_PlatformForBox_Parent Object Reference"))
  (returns (IsLockOpen :type Boolean))
  (locals (SumOfRightPlacings :type Integer))
  (set `local.SumOfRightPlacings` 0)
  (for _array_element _Array
    (bind _currentboxref (`/Game/MagicTrigger/Blueprints/Items/Quest1/BP_PlatformForBox_Parent.CurrentBoxRef` _array_element))
    (`/Engine/EditorBlueprintResources/StandardMacros.IsValid` _currentboxref
      (:`Is Valid`
        (if (== (`|GetArrayItem` (`Actor.Tags` _array_element)) (`|GetArrayItem` (`Actor.Tags` _currentboxref)))
          (`/Engine/EditorBlueprintResources/StandardMacros.IncrementInt` (`local.SumOfRightPlacings`))
          (else
            (break))))
      (:`Is Not Valid`
        (break))))
  (return (== (`KismetArrayLibrary.Array_Length` _Array) (`local.SumOfRightPlacings`))))

(fn `IsCharacterOnLift?`
  (params (`_isOnLift?` :type Boolean))
  (if `_isOnLift?`
    (`self.DisableInput` (`GameplayStatics.GetPlayerCharacter` 0) (`GameplayStatics.GetPlayerController` 0))
    (message `/Game/MagicTrigger/Blueprints/Interfaces/BPI_OwnerTargetSelection.OffWatchingActors_IF` (`GameplayStatics.GetPlayerCharacter` 0))
    (`CharacterMovementComponent.DisableMovement` (`Character.CharacterMovement` (`GameplayStatics.GetPlayerCharacter` 0)))
    (set `/Game/MagicTrigger/Blueprints/Items/Quest1/BP_Lift.IsOffOverlapCharacter?` true (`self.LiftRef`))
    (`self.SetActorEnableCollision` (`GameplayStatics.GetPlayerCharacter` 0) false)
    (return)
    (else
      (`self.EnableInput` (`GameplayStatics.GetPlayerCharacter` 0) (`GameplayStatics.GetPlayerController` 0))
      (`CharacterMovementComponent.SetMovementMode` (`Character.CharacterMovement` (`GameplayStatics.GetPlayerCharacter` 0)) "MOVE_Walking" 0)
      ;[0.8213 0 0] Отсоединить от лифта (квест 1)
      (`self.K2_DetachFromActor` (`GameplayStatics.GetPlayerCharacter` 0) "KeepWorld" "KeepWorld" "KeepWorld")
      (`self.SetActorEnableCollision` (`GameplayStatics.GetPlayerCharacter` 0) true)
      (set `/Game/MagicTrigger/Blueprints/Items/Quest1/BP_Lift.IsOffOverlapCharacter?` false (`self.LiftRef`))
      (return))))

(fn `UserConstructionScript`)