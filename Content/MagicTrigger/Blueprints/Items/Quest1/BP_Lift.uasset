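; Lift actor for Quest 1 that reports when the player character steps on or off it, leaving the response to Quest1Manager.
; On BeginPlay it stores its initial location and registers itself with Quest1Manager through the reference aggregator, retrying on a short delay until the manager is valid.
; OverlapBox events filtered to the player character fire begin and end overlap dispatchers.
; Observable events toggle custom depth on the mesh to outline it.
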(event `self.ReceiveBeginPlay`
  ;[0.02899 0 0.8018] EventBeginPlay
  (set `self.InitLocation` (`self.K2_GetActorLocation`))
  (bind _referenceaggregator (`/Game/MagicTrigger/Blueprints/FunctionLibraries/BPFL_ReferenceAggregator.GetReferenceAggregator`))
  (bind _quest1manager (`/Game/MagicTrigger/Blueprints/CoreClasses/BP_ReferenceAggregator.quest1Manager` _referenceaggregator))
  (`/Engine/EditorBlueprintResources/StandardMacros.IsValid` _quest1manager :!label _label
    (:`Is Valid`
      (set `/Game/MagicTrigger/Blueprints/Items/Quest1/BP_Quest1Manager.LiftRef` self _quest1manager))
    (:`Is Not Valid`
      (`KismetSystemLibrary.Delay` 0.5)
      (goto _label))))

(event `self.OverlapBox.OnComponentBeginOverlap`
  (params (OverlappedComponent :type "PrimitiveComponent Object Reference") (OtherActor :type "Actor Object Reference") (OtherComp :type "PrimitiveComponent Object Reference") (OtherBodyIndex :type Integer) (bFromSweep :type Boolean) (SweepResult :type "HitResult Structure (by ref)"))
  ;[0.3285 0 0.4987] Когда перс заходит или сходит с лифта, вызвать логику в Quest1Manager
  (cast `/Game/MagicTrigger/Blueprints/PlayerCharacter/BP_PlayerCharacter` OtherActor)
  (`self.BeginOverlapCharacter` OtherComp))

(event `self.OverlapBox.OnComponentEndOverlap`
  (params (OverlappedComponent :type "PrimitiveComponent Object Reference") (OtherActor :type "Actor Object Reference") (OtherComp :type "PrimitiveComponent Object Reference") (OtherBodyIndex :type Integer))
  ;[0.3285 0 0.4987] Когда перс заходит или сходит с лифта, вызвать логику в Quest1Manager
  (cast `/Game/MagicTrigger/Blueprints/PlayerCharacter/BP_PlayerCharacter` OtherActor)
  (`self.EndOverlapCharacter` OtherComp))

(event `/Game/MagicTrigger/Blueprints/Interfaces/BPI_Observe.BecomeObservable`
  ;[0 0.4541 0.3672] Отрисовать рамку, если под наблюдением перса
  (`PrimitiveComponent.SetRenderCustomDepth` (`self.StaticMesh`) true))

(event `/Game/MagicTrigger/Blueprints/Interfaces/BPI_Observe.BecomeNotObservable`
  ;[0 0.4541 0.3672] Отрисовать рамку, если под наблюдением перса
  (`PrimitiveComponent.SetRenderCustomDepth` (`self.StaticMesh`) false))

(fn `UserConstructionScript`)