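; Base quest platform that sinks when a BP_BoxForPlatform_Parent stone rests on it and rises when that stone leaves.
; Box1 overlaps track a single stone by matching its Box component, triggering MoveDown on entry and a delayed MoveUp on exit.
; Two timelines lerp the platform between its initial location and twice its mesh's Z extent below; logic to move the stone itself is unconnected.
; Observation events toggle a custom-depth highlight on the mesh.
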(event `self.ReceiveBeginPlay`
  ;[0 0.3962 0.4251] EventBeginPlay
  (set `self.InitLocation` (`self.K2_GetActorLocation`)))

(event `TargetSelectionInterface.IsObserved`
  ;[0.04831 0 0.7822] Отрисовать рамку, если под наблюдением перса
  (`PrimitiveComponent.SetRenderCustomDepth` (`self.StaticMesh`) true))

(event `self.Box1.OnComponentBeginOverlap`
  (params (OverlappedComponent :type "PrimitiveComponent Object Reference") (OtherActor :type "Actor Object Reference") (OtherComp :type "PrimitiveComponent Object Reference") (OtherBodyIndex :type Integer) (bFromSweep :type Boolean) (SweepResult :type "HitResult Structure (by ref)"))
  ;[0 0.3768 0.4445] Если квестовый камень окажется на платформе, то запомнить ссылку на него и переместить его в точку на платформе, проиграть опускание платформы вместе с камнем. Если камень уйдет с платформы, то обнулить ссылку на него, проиграть поднимание платформы
  (`self.BeginOverlapBox1` OtherActor OtherComp))

(event `TargetSelectionInterface.IsNotObserved`
  ;[0.04831 0 0.7822] Отрисовать рамку, если под наблюдением перса
  (`PrimitiveComponent.SetRenderCustomDepth` (`self.StaticMesh`) false))

(event `self.Box1.OnComponentEndOverlap`
  (params (OverlappedComponent :type "PrimitiveComponent Object Reference") (OtherActor :type "Actor Object Reference") (OtherComp :type "PrimitiveComponent Object Reference") (OtherBodyIndex :type Integer))
  ;[0 0.3768 0.4445] Если квестовый камень окажется на платформе, то запомнить ссылку на него и переместить его в точку на платформе, проиграть опускание платформы вместе с камнем. Если камень уйдет с платформы, то обнулить ссылку на него, проиграть поднимание платформы
  (bind _asbp_box_for_platform_parent (cast `/Game/MagicTrigger/Blueprints/Items/Quest1/BP_BoxForPlatform_Parent` OtherActor))
  (if (== (`/Game/MagicTrigger/Blueprints/Items/LiftingObjects/BP_LiftingObject.Box` _asbp_box_for_platform_parent) OtherComp)
    (if (== (`self.CurrentBoxRef`) _asbp_box_for_platform_parent)
      (set `self.CurrentBoxRef` null)
      (`self.MoveUp`))))

(event `MoveDown`
  (bind _currentboxref (`self.CurrentBoxRef`))
  (bind _initlocation (`self.InitLocation`))
  ;[0 0.3768 0.4445] Если квестовый камень окажется на платформе, то запомнить ссылку на него и переместить его в точку на платформе, проиграть опускание платформы вместе с камнем. Если камень уйдет с платформы, то обнулить ссылку на него, проиграть поднимание платформы
  (set `/Game/MagicTrigger/Blueprints/Items/Quest1/BP_BoxForPlatform_Parent.CurrentLocation` (`self.K2_GetActorLocation` _currentboxref) _currentboxref)
  (bind (_direction _alpha) (`Timeline|Timeline_1` :!via `PlayFromStart`)
    (:`Update`
      (`self.K2_SetActorLocation` (`KismetMathLibrary.VLerp` _initlocation (`KismetMathLibrary.MakeVector` (.x _initlocation) (.y _initlocation) (- (.z _initlocation) (* (.z (`.BoxExtent` (`KismetSystemLibrary.GetComponentBounds` (`self.StaticMesh`)))) 2.0))) _alpha)))))

(event `MoveUp`
  (bind _initlocation (`self.InitLocation`))
  ;[0 0.3768 0.4445] Если квестовый камень окажется на платформе, то запомнить ссылку на него и переместить его в точку на платформе, проиграть опускание платформы вместе с камнем. Если камень уйдет с платформы, то обнулить ссылку на него, проиграть поднимание платформы
  (`KismetSystemLibrary.Delay` 1.0)
  (bind (_direction _alpha) (`Timeline|Timeline_0` :!via `ReverseFromEnd`)
    (:`Update`
      (`self.K2_SetActorLocation` (`KismetMathLibrary.VLerp` _initlocation (`KismetMathLibrary.MakeVector` (.x _initlocation) (.y _initlocation) (- (.z _initlocation) (* (.z (`.BoxExtent` (`KismetSystemLibrary.GetComponentBounds` (`self.StaticMesh`)))) 2.0))) _alpha)))))

(fn `BeginOverlapBox1`
  (params (OtherActor :type "Actor Object Reference") (OtherComponent :type "PrimitiveComponent Object Reference"))
  (`/Engine/EditorBlueprintResources/StandardMacros.IsValid` (`self.CurrentBoxRef`)
    (:`Is Valid`
      (return))
    (:`Is Not Valid`
      (bind _asbp_box_for_platform_parent (cast `/Game/MagicTrigger/Blueprints/Items/Quest1/BP_BoxForPlatform_Parent` OtherActor)
        (:`then`
          (if (== (`/Game/MagicTrigger/Blueprints/Items/LiftingObjects/BP_LiftingObject.Box` _asbp_box_for_platform_parent) OtherComponent)
            (set `self.CurrentBoxRef` _asbp_box_for_platform_parent)
            (`self.MoveDown`)
            (return)
            (else
              (return))))
        (:`CastFailed`
          (return))))))

(fn `GetInteractionText`
  (returns (InteractionText :type Text))
  (return ""))

(fn `UserConstructionScript`)