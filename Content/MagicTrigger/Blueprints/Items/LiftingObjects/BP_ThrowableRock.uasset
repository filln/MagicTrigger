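; BP_ThrowableRock is a throwable rock item that stuns and damages actors it touches.
; When its Box component begins an overlap, it sends a stun interface message to the other actor, then applies its Damage value, crediting the first player's controller as instigator.
; The graph does no target filtering and holds no throw logic; BeginPlay, Tick and actor overlap only forward to the parent class.
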(event `self.ReceiveBeginPlay`
  (`parent.ReceiveBeginPlay`))

(event `self.ReceiveActorBeginOverlap`
  (params (OtherActor :type "Actor Object Reference"))
  (`parent.ReceiveActorBeginOverlap` OtherActor))

(event `self.ReceiveTick`
  (params (DeltaSeconds :type "Float (single-precision)"))
  (`parent.ReceiveTick` DeltaSeconds))

(event `self.Box.OnComponentBeginOverlap`
  (params (OverlappedComponent :type "PrimitiveComponent Object Reference") (OtherActor :type "Actor Object Reference") (OtherComp :type "PrimitiveComponent Object Reference") (OtherBodyIndex :type Integer) (bFromSweep :type Boolean) (SweepResult :type "HitResult Structure (by ref)"))
  (message `/Game/MagicTrigger/Blueprints/Interfaces/BPI_TrowableRockResponse.Stunning_IF` OtherActor)
  (`GameplayStatics.ApplyDamage` OtherActor (`self.Damage`) (`Pawn.GetController` (`GameplayStatics.GetPlayerCharacter` 0)) self))

(fn `UserConstructionScript`)