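; BP_LiftingObject is an interactable item that the Kachujin character can lift up and put down.
; It caches a reference aggregator on BeginPlay to reach the character and course HUD.
; Observation events toggle the mesh's custom depth to draw an outline, and another event shows or hides the HUD prompt.
; Interact calls the character's LiftUpPutDown and flips IsLifted, but only when the course HUD is valid.
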(event `self.ReceiveBeginPlay`
  ;[0.7054 0.1159 0] EventBeginPlay
  (bind _referenceaggregator (`/Game/MagicTrigger/Blueprints/FunctionLibraries/BPFL_ReferenceAggregator.GetReferenceAggregator`))
  (set `self.referenceAggregator` _referenceaggregator))

(event `TargetSelectionInterface.IsObserved`
  ;[0.7247 0 0.09777] Отрисовать рамку, если под наблюдением перса
  (`PrimitiveComponent.SetRenderCustomDepth` (`self.StaticMesh`) true))

(event `TargetSelectionInterface.IsNotObserved`
  ;[0.7247 0 0.09777] Отрисовать рамку, если под наблюдением перса
  (`PrimitiveComponent.SetRenderCustomDepth` (`self.StaticMesh`) false))

(event `/Game/MagicTrigger/Blueprints/Interfaces/BPI_Interaction.Interact`
  ;[0.6474 0.1739 0] Поднять или опустить себя
  (`/Engine/EditorBlueprintResources/StandardMacros.IsValid` (`/Game/MagicTrigger/Blueprints/CoreClasses/BP_ReferenceAggregator.HUDCourse` (`self.referenceAggregator`))
    (:`Is Valid`
      (`/Game/MagicTrigger/Blueprints/PlayerCharacter/BP_PlayerCharacter.LiftUp/PutDown` (`/Game/MagicTrigger/Blueprints/CoreClasses/BP_ReferenceAggregator.kachujinCharacter` (`self.referenceAggregator`)))
      (set `self.isLifted?` (not (`self.isLifted?`))))))

(event `/Game/MagicTrigger/Blueprints/Interfaces/BPI_Interaction.ShowOrHideInteractionWidget`
  (params (Show :type Boolean))
  ;[0.7054 0.1159 0] Показать виджет с подсказкой
  (`/Engine/EditorBlueprintResources/StandardMacros.IsValid` (`/Game/MagicTrigger/Blueprints/CoreClasses/BP_ReferenceAggregator.HUDCourse` (`self.referenceAggregator`))
    (:`Is Valid`
      (`/Game/MagicTrigger/Blueprints/CoreClasses/BP_HUD.ShowOrHideInteractionWidget` (`/Game/MagicTrigger/Blueprints/CoreClasses/BP_ReferenceAggregator.HUDCourse` (`self.referenceAggregator`)) Show (`self.InteractionText`)))))

(fn `UserConstructionScript`)