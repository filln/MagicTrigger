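; BP_ThrowableObject is a throwable item among the lifting objects that customises the interaction prompt shown on the HUD.
; BeginPlay, Tick and overlap events just forward to the parent class.
; ShoworHideInteractionWidget checks the HUDCourse from ReferenceAggregator, then shows or hides the widget with InteractionText when not lifted.
; While lifted, it only swaps the HUD text to ThrowableText, ignoring the Show flag.
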(event `self.ReceiveBeginPlay`
  (`parent.ReceiveBeginPlay`))

(event `self.ReceiveActorBeginOverlap`
  (params (OtherActor :type "Actor Object Reference"))
  (`parent.ReceiveActorBeginOverlap` OtherActor))

(event `self.ReceiveTick`
  (params (DeltaSeconds :type "Float (single-precision)"))
  (`parent.ReceiveTick` DeltaSeconds))

(event `/Game/MagicTrigger/Blueprints/Interfaces/BPI_Interaction.ShowOrHideInteractionWidget`
  (params (Show :type Boolean))
  ;[0.7054 0.116 0] Показать виджет с подсказкой
  (`/Engine/EditorBlueprintResources/StandardMacros.IsValid` (`/Game/MagicTrigger/Blueprints/CoreClasses/BP_ReferenceAggregator.HUDCourse` (`self.referenceAggregator`))
    (:`Is Valid`
      (if (`self.isLifted?`)
        (set `/Game/MagicTrigger/Blueprints/CoreClasses/BP_HUD.InteractionText` (`self.ThrowableText`) (`/Game/MagicTrigger/Blueprints/CoreClasses/BP_ReferenceAggregator.HUDCourse` (`self.referenceAggregator`)))
        (else
          (`/Game/MagicTrigger/Blueprints/CoreClasses/BP_HUD.ShowOrHideInteractionWidget` (`/Game/MagicTrigger/Blueprints/CoreClasses/BP_ReferenceAggregator.HUDCourse` (`self.referenceAggregator`)) Show (`self.InteractionText`)))))))

(fn `UserConstructionScript`)