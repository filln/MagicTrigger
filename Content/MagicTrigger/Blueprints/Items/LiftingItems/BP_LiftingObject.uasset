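; BP_LiftingObject is an interactable item that, judging by its name, the player can lift.
; IsObserved and IsNotObserved events toggle custom depth rendering on its static mesh to show an outline while the character looks at it.
; Getter functions expose its attach socket and interaction text, while the overlap, tick and construction logic are empty.
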(event `self.ReceiveBeginPlay`
  ;[0.7054 0.1159 0] EventBeginPlay
)

(event `TargetSelectionInterface.IsObserved`
  ;[0.7247 0 0.09777] Отрисовать рамку, если под наблюдением перса
  (`PrimitiveComponent.SetRenderCustomDepth` (`self.StaticMesh`) true))

(event `TargetSelectionInterface.IsNotObserved`
  ;[0.7247 0 0.09777] Отрисовать рамку, если под наблюдением перса
  (`PrimitiveComponent.SetRenderCustomDepth` (`self.StaticMesh`) false))

(fn `GetAttachSocket_IF`
  (returns (AttachSocket :type Name))
  (return (`self.AttachSocket`)))

(fn `GetInteractionText`
  (returns (InteractionText :type Text))
  (return (`self.InteractionText`)))

(fn `UserConstructionScript`)