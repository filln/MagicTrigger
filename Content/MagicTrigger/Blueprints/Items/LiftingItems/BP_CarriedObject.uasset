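; BP_CarriedObject is a liftable item that the player carries with two hands.
; Interface events forward lift-up and put-down animation states to player character 0 as two-hand interface messages.
; A physics toggle sets simulation on the static mesh, then reattaches the box and interaction collision to the root, snapping location while keeping world rotation and scale.
; BeginPlay, overlap and Tick only call the parent class.
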(event `self.ReceiveBeginPlay`
  (`parent.ReceiveBeginPlay`))

(event `self.ReceiveActorBeginOverlap`
  (params (OtherActor :type "Actor Object Reference"))
  (`parent.ReceiveActorBeginOverlap` OtherActor))

(event `self.ReceiveTick`
  (params (DeltaSeconds :type "Float (single-precision)"))
  (`parent.ReceiveTick` DeltaSeconds))

(event `/Game/Developers/OLDFiles/Interfaces/BPI_LiftingObjects_OLD.SetPlayingAnimationLiftUp_IF`
  (params (bPlaying :type Boolean))
  (bind _returnvalue (`GameplayStatics.GetPlayerCharacter` 0))
  (`/Engine/EditorBlueprintResources/StandardMacros.IsValid` _returnvalue
    (:`Is Valid`
      (message `/Game/Developers/OLDFiles/Interfaces/BPI_AnimationManager_OLD.SetPlayingAnimationLiftUp2Hand_IF` _returnvalue bPlaying))))

(event `/Game/Developers/OLDFiles/Interfaces/BPI_LiftingObjects_OLD.SetPlayingAnimationPutDown_IF`
  (params (bPlaying :type Boolean))
  (bind _returnvalue (`GameplayStatics.GetPlayerCharacter` 0))
  (`/Engine/EditorBlueprintResources/StandardMacros.IsValid` _returnvalue
    (:`Is Valid`
      (message `/Game/Developers/OLDFiles/Interfaces/BPI_AnimationManager_OLD.SetPlayingAnimationPutDown2Hand_IF` _returnvalue bPlaying))))

(event `/Game/Developers/OLDFiles/Interfaces/BPI_LiftingObjects_OLD.SetSimulatePhysics_IF`
  (params (bSimulate :type Boolean))
  (`PrimitiveComponent.SetSimulatePhysics` (`self.StaticMesh`) bSimulate)
  (`SceneComponent.K2_AttachToComponent` (`self.Box`) (`self.RootComponent`) "None" "SnapToTarget" "KeepWorld" "KeepWorld" true)
  (`SceneComponent.K2_AttachToComponent` (`self.InteractCollision`) (`self.RootComponent`) "None" "SnapToTarget" "KeepWorld" "KeepWorld" true))

(fn `UserConstructionScript`)