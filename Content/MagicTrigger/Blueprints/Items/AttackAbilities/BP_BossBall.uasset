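; BP_BossBall is a boss attack projectile that grows and glows while attached to its owner's mesh socket, driven by a BossBallStruct.
; When launched, it detaches, enables collision and moves to the target's location captured at that moment.
; On arrival it scales again, damages overlapping non-owner characters through BPI_Damage, then destroys itself.
; Construction removes other still-held copies, sets a short lifespan and creates the dynamic emissive material.
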(event `Activate`
  (params (_BossBallStruct :type "/Game/MagicTrigger/Data/SBossBall Structure"))
  ;[0 0.09662 0.7247] Присоединить к владельцу
  (bind _output_get (set `self.BossBallStruct` _BossBallStruct))
  (`self.SetActorEnableCollision` false)
  (`self.K2_AttachToComponent` (`Character.Mesh` (`.OwnerCharacter_19_0D62516841770246BF8235BACF64E3F9` (break `/Game/MagicTrigger/Data/SBossBall` _output_get))) (`.BossBallSocket_10_F3E329DB451124B7A30C7998B0DDFECE` (break `/Game/MagicTrigger/Data/SBossBall` _output_get)) "KeepWorld" "KeepWorld" "KeepWorld")
  (`self.ScaleAndEmissive`))

(event `ScaleAndEmissive`
  (bind (_bossballstruct_bossball _bossballstruct_ownercharacter _bossballstruct_timeofscaleinownershand _bossballstruct_multiplierofscaleinownershand _bossballstruct_emissivemultiplier) (break `/Game/MagicTrigger/Data/SBossBall` (`self.BossBallStruct`)))
  (bind _initialscale (`self.InitialScale`))
  ;[0 0.009662 0.8116] Увеличить размер и яркость
  (set `self.InitialScale` (`self.GetActorScale3D`))
  (`TimelineComponent.SetPlayRate` (`self.Timeline_ScaleAndEmissive`) (/ 1.0 _bossballstruct_timeofscaleinownershand))
  (bind (_direction _alpha) (`Timeline|Timeline_ScaleAndEmissive` :!via `PlayFromStart`)
    (:`Update`
      (`self.SetActorScale3D` (`KismetMathLibrary.VLerp` _initialscale (* _initialscale _bossballstruct_multiplierofscaleinownershand) _alpha))
      (`MaterialInstanceDynamic.SetScalarParameterValue` (`self.MaterialInst`) "EmissiveMultiplier" (`KismetMathLibrary.Lerp` 0.0 _bossballstruct_emissivemultiplier _alpha)))))

(event `MoveBossBallToTarget`
  (params (_TargetCharacter :type "Character Object Reference"))
  (bind (_bossballstruct_bossball _bossballstruct_ownercharacter _bossballstruct_timeofscaleinownershand _bossballstruct_multiplierofscaleinownershand _bossballstruct_emissivemultiplier _bossballstruct_timeofmove) (break `/Game/MagicTrigger/Data/SBossBall` (`self.BossBallStruct`)))
  ;[0.3478 0.4735 0] Переместить к цели
  (set `self.TargetCharacter` _TargetCharacter)
  (`self.K2_DetachFromActor` "KeepWorld" "KeepWorld" "KeepWorld")
  (`self.SetActorEnableCollision` true)
  (`/Engine/EditorBlueprintResources/StandardMacros.IsValid` (`self.TargetCharacter`)
    (:`Is Valid`
      ;[0.8213 0 0] Не может быть удален при появлении новой копии (в constructionScript). После того, как покинул руки овнера.
      (set `self.сanBeDestroyed?` false)
      (`KismetSystemLibrary.MoveComponentTo` (`self.RootComponent`) (`self.K2_GetActorLocation` (`self.TargetCharacter`)) (`SceneComponent.RelativeRotation` (`self.RootComponent`)) false false _bossballstruct_timeofmove)
      (`|ExecutionSequence`
        (:`then_0`
          (`self.EffectsEreDestroy`))
        (:`then_1`
          (`self.TransferDamageAndDestroy`))))
    (:`Is Not Valid`
      (`self.K2_DestroyActor`))))

(event `EffectsEreDestroy`
  (bind (_bossballstruct_bossball _bossballstruct_ownercharacter _bossballstruct_timeofscaleinownershand _bossballstruct_multiplierofscaleinownershand _bossballstruct_emissivemultiplier _bossballstruct_timeofmove _bossballstruct_damage _bossballstruct_multiplierofdamage _bossballstruct_bossballsocket _bossballstruct_multiplierofscaleeredestroy _bossballstruct_timeofscaleeredestroy) (break `/Game/MagicTrigger/Data/SBossBall` (`self.BossBallStruct`)))
  ;[0 0.7827 0.03865] Эффекты перед дестроем
  (`self.Scale` _bossballstruct_timeofscaleeredestroy _bossballstruct_multiplierofscaleeredestroy))

(event `TransferDamageAndDestroy`
  (bind (_bossballstruct_bossball _bossballstruct_ownercharacter _bossballstruct_timeofscaleinownershand _bossballstruct_multiplierofscaleinownershand _bossballstruct_emissivemultiplier _bossballstruct_timeofmove _bossballstruct_damage) (break `/Game/MagicTrigger/Data/SBossBall` (`self.BossBallStruct`)))
  (bind (_bossballstruct_bossball_2 _bossballstruct_ownercharacter_2 _bossballstruct_timeofscaleinownershand_2 _bossballstruct_multiplierofscaleinownershand_2 _bossballstruct_emissivemultiplier_2 _bossballstruct_timeofmove_2 _bossballstruct_damage_2 _bossballstruct_multiplierofdamage _bossballstruct_bossballsocket _bossballstruct_multiplierofscaleeredestroy _bossballstruct_timeofscaleeredestroy) (break `/Game/MagicTrigger/Data/SBossBall` (`self.BossBallStruct`)))
  ;[0.3768 0 0.4498] Атаковать и удалиться
  (for _array_element (`PrimitiveComponent.GetOverlappingActors` (`self.Sphere`) "/Script/Engine.Character")
    (bind _ascharacter (cast `Character` _array_element))
    (if (and (!= _ascharacter _bossballstruct_ownercharacter_2) (`KismetSystemLibrary.DoesImplementInterface` _ascharacter "/Game/MagicTrigger/Blueprints/Interfaces/BPI_Damage.BPI_Damage_C"))
      (message `/Game/MagicTrigger/Blueprints/Interfaces/BPI_Damage.TransferDamage` _ascharacter _bossballstruct_damage _bossballstruct_multiplierofdamage)))
  (`KismetSystemLibrary.Delay` _bossballstruct_timeofscaleeredestroy)
  (`self.K2_DestroyActor`))

(event `Scale`
  (params (_TimeOfScale :type "Float (double-precision)") (_MultiplierOfScale :type "Float (double-precision)"))
  (bind _initialscale (`self.InitialScale`))
  ;[0 0.01932 0.802] Увеличиться
  (`TimelineComponent.SetPlayRate` (`self.Timeline_Scale`) (/ 1.0 _TimeOfScale))
  (set `self.InitialScale` (`self.GetActorScale3D`))
  (bind (_direction _alpha) (`Timeline|Timeline_Scale` :!via `PlayFromStart`)
    (:`Update`
      (`self.SetActorScale3D` (`KismetMathLibrary.VLerp` _initialscale (* _initialscale _MultiplierOfScale) _alpha)))))

(fn `UserConstructionScript`
  (`|ExecutionSequence`
    (:`then_0`
      ;[0 0.2222 0.5991] Удалить копии, если разрешено (не ушли от владельца)
      (bind _outactors (`GameplayStatics.GetAllActorsOfClass` "BP_BossBall_C"))
      (for _array_element _outactors
        (if (and (!= _array_element self) (`/Game/MagicTrigger/Blueprints/Items/AttackAbilities/BP_BossBall.сanBeDestroyed?` _array_element))
          (`self.K2_DestroyActor` _array_element)))
      (`self.SetLifeSpan` 3.0))
    (:`then_1`
      ;[0.4251 0.3962 0] Настроить материал
      (bind _returnvalue (`PrimitiveComponent.CreateDynamicMaterialInstance` (`self.StaticMesh`) 0 "/Game/MagicTrigger/Materials/M_Ability.M_Ability" "None"))
      (bind _output_get (set `self.MaterialInst` _returnvalue))
      (`MaterialInstanceDynamic.SetTextureParameterValue` _output_get "Texture" "/Game/MagicTrigger/Textures/T_BossBall_D.T_BossBall_D")
      (`MaterialInstanceDynamic.SetVectorParameterValue` (`self.MaterialInst`) "EmissiveColor" (struct :`R` 0.53 :`A` 1.0))
      (`MaterialInstanceDynamic.SetScalarParameterValue` (`self.MaterialInst`) "EmissiveMultiplier" 1.0))))