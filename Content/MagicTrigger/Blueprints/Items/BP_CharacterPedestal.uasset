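; BP_CharacterPedestal is a pedestal actor that supplies the world position of its PointForArtifact component to the game's artifact manager.
; On BeginPlay it starts a looping timer that retries until the manager can be fetched from the game mode through an interface and is valid.
; It then clears the timer and writes that position into the manager's LocationForArtifact.
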(event `self.ReceiveBeginPlay`
  (`self.StartBeginPlayTimer_IF`))

(event `self.DoBeginPlay_IF`
  (set `/Game/MagicTrigger/Blueprints/Items/Artifact/BP_ArtifactManager.LocationForArtifact` (`SceneComponent.K2_GetComponentLocation` (`self.PointForArtifact`)) (`self.BP_ArtifactManager`)))

(event `self.BeforeBeginPlay_IF`
  (bind _bvalid (`self.CheckReferences_IF`))
  (if _bvalid
    (`KismetSystemLibrary.K2_ClearAndInvalidateTimerHandle` (`self.BeginPlayTimer`))
    (`self.DoBeginPlay_IF`)))

(event `self.StartBeginPlayTimer_IF`
  (bind _returnvalue (`KismetSystemLibrary.K2_SetTimerDelegate` (delegate `self.BeforeBeginPlay_IF`) (`self.BeginPlayTimerTime`) true))
  (set `self.BeginPlayTimer` _returnvalue))

(fn `CheckReferences_IF`
  (returns (bValid :type Boolean))
  (`/Engine/EditorBlueprintResources/StandardMacros.IsValid` (`GameplayStatics.GetGameMode`)
    (:`Is Valid`
      (bind _bp_artifactmanager (message `/Game/Developers/OLDFiles/Interfaces/BPI_GameMode_OLD.GetArtifactManager_IF` (`GameplayStatics.GetGameMode`)))
      (bind _output_get (set `self.BP_ArtifactManager` _bp_artifactmanager))
      (`/Engine/EditorBlueprintResources/StandardMacros.IsValid` _output_get
        (:`Is Valid`
          (return true))
        (:`Is Not Valid`
          (return false))))
    (:`Is Not Valid`
      (return false))))

(fn `UserConstructionScript`)